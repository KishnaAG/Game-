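; Player controller for the main menu level, driving the front-end flow for new game, continue, load and quit.
; On begin play it sets the view to a menu camera, switches to UI-only input and shows the menu widget.
; Menu entries open a save slot picker in new or load mode, resume the continue slot, or open a quit confirmation modal.
; BP_StoreGameInstance starts, loads or deletes slots before the game level opens.
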(event `self.ReceiveBeginPlay`
  ;[1 1 1 0.8] Event begin play
  (bind _returnvalue (`GameplayStatics.GetActorOfClass` (`self.MenuCameraClass`)))
  (`self.SetViewTargetWithBlend` self _returnvalue 0.0 "VTBlend_Linear" 0.0 false)
  (`WidgetBlueprintLibrary.SetInputMode_UIOnlyEx` self null)
  (`self.ShowMainMenu`))

(fn `ConfirmQuit`
  ;[1 1 1 0.8] Confirm quit
  (bind _returnvalue (`|CreateWidget` (`self.ModalClass`) self))
  (set `/Game/GrandOpening/Blueprints/Widgets/Gameplay/BP_ModalWidget.Title` (`self.QuitTitle`) _returnvalue)
  (set `/Game/GrandOpening/Blueprints/Widgets/Gameplay/BP_ModalWidget.Message` (`self.QuitMessage`) _returnvalue)
  (add `/Game/GrandOpening/Blueprints/Widgets/Gameplay/BP_ModalWidget.OnConfirmed` _returnvalue (`|CreateDelegate` :!event `QuitToDesktop`))
  (`UserWidget.AddToViewport` _returnvalue 0))

(fn `ContinueGame`
  ;[1 1 1 0.8] Continue game
  (bind _asbp_store_game_instance (cast `/Game/GrandOpening/Blueprints/Misc/BP_StoreGameInstance` (`GameplayStatics.GetGameInstance`)))
  (bind _slotindex (`/Game/GrandOpening/Blueprints/Misc/BP_StoreGameInstance.ResolveContinueSlotIndex` _asbp_store_game_instance))
  (if (>= _slotindex 0)
    (`/Game/GrandOpening/Blueprints/Misc/BP_StoreGameInstance.RequestLoad` _asbp_store_game_instance _slotindex)
    (`GameplayStatics.OpenLevelBySoftObjectPtr` (`self.GameLevel`))))

(fn `HandleBack`
  ;[1 1 1 0.8] Handle back
  (`/Game/GrandOpening/Blueprints/Widgets/Menu/BP_SlotPickerWidget.Dismiss` (`self.SlotPicker`))
  (`self.ShowMainMenu`))

(fn `HandleDeleteRequested`
  (params (Index :type Integer))
  ;[1 1 1 0.8] Handle delete requested
  (bind _asbp_store_game_instance (cast `/Game/GrandOpening/Blueprints/Misc/BP_StoreGameInstance` (`GameplayStatics.GetGameInstance`)))
  (`/Game/GrandOpening/Blueprints/Misc/BP_StoreGameInstance.DeleteSlot` _asbp_store_game_instance Index)
  (`/Game/GrandOpening/Blueprints/Widgets/Menu/BP_SlotPickerWidget.ClearSlot` (`self.SlotPicker`) Index))

(fn `HandleEntry`
  (params (Id :type Name))
  ;[1 1 1 0.8] Handle entry
  (if (== Id "NewGame")
    (`self.OpenSlotPicker` "NewEnumerator0")
    (elif (== Id "Continue")
      (`self.ContinueGame`)
      (elif (== Id "LoadGame")
        (`self.OpenSlotPicker` "NewEnumerator1")
        (elif (== Id "Quit")
          (`self.ConfirmQuit`))))))

(fn `HandleSlotPicked`
  (params (Index :type Integer))
  ;[1 1 1 0.8] Handle slot picked
  (bind _asbp_store_game_instance (cast `/Game/GrandOpening/Blueprints/Misc/BP_StoreGameInstance` (`GameplayStatics.GetGameInstance`)))
  (if (`|EnumEquality` (`self.PickerMode`) "NewEnumerator0")
    (`/Game/GrandOpening/Blueprints/Misc/BP_StoreGameInstance.StartNewGame` _asbp_store_game_instance Index)
    (`GameplayStatics.OpenLevelBySoftObjectPtr` (`self.GameLevel`))
    (else
      (`/Game/GrandOpening/Blueprints/Misc/BP_StoreGameInstance.RequestLoad` _asbp_store_game_instance Index)
      (`GameplayStatics.OpenLevelBySoftObjectPtr` (`self.GameLevel`)))))

(fn `OpenSlotPicker`
  (params (Mode :type "/Game/GrandOpening/Blueprints/Enumerations/E_SlotPickerMode Enum" :default "NewEnumerator0"))
  ;[1 1 1 0.8] Open slot picker
  (set `self.PickerMode` Mode)
  (`/Game/GrandOpening/Blueprints/Widgets/Menu/BP_MainMenuWidget.Dismiss` (`self.MenuScreen`))
  (bind _returnvalue (`|CreateWidget` (`self.SlotPickerClass`) self))
  (set `self.SlotPicker` _returnvalue)
  (`/Game/GrandOpening/Blueprints/Widgets/Menu/BP_SlotPickerWidget.OpenAs` _returnvalue Mode)
  (add `/Game/GrandOpening/Blueprints/Widgets/Menu/BP_SlotPickerWidget.OnSlotPicked` _returnvalue (`|CreateDelegate` :!event `HandleSlotPicked`))
  (add `/Game/GrandOpening/Blueprints/Widgets/Menu/BP_SlotPickerWidget.OnDeleteRequested` _returnvalue (`|CreateDelegate` :!event `HandleDeleteRequested`))
  (add `/Game/GrandOpening/Blueprints/Widgets/Menu/BP_SlotPickerWidget.OnBack` _returnvalue (`|CreateDelegate` :!event `HandleBack`))
  (`UserWidget.AddToViewport` _returnvalue 0))

(fn `QuitToDesktop`
  ;[1 1 1 0.8] Quit to desktop
  (`KismetSystemLibrary.QuitGame` self "Quit"))

(fn `ShowMainMenu`
  ;[1 1 1 0.8] Show main menu
  (bind _returnvalue (`|CreateWidget` (`self.MenuScreenClass`) self))
  (set `self.MenuScreen` _returnvalue)
  (add `/Game/GrandOpening/Blueprints/Widgets/Menu/BP_MainMenuWidget.OnEntryChosen` _returnvalue (`|CreateDelegate` :!event `HandleEntry`))
  (`UserWidget.AddToViewport` _returnvalue 0))

(fn `UserConstructionScript`)
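; BP_MenuCamera is a menu camera actor that slowly sways around its starting orientation.
; BeginPlay stores the initial rotation as a base.
; Each Tick adds time-based sine offsets to that base, scaled by DriftDegrees and DriftSeconds, leaving roll unchanged.
; Pitch swings at half the frequency and about a third of the amplitude of yaw, producing a figure-eight style drift without a Timeline.
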(event `self.ReceiveBeginPlay`
  ;[1 1 1 0.8] Event begin play
  (set `self.BaseRotation` (`self.K2_GetActorRotation`)))

(event `self.ReceiveTick`
  (params (DeltaSeconds :type "Float (single-precision)"))
  (bind _baserotation (`self.BaseRotation`))
  (bind _driftdegrees (`self.DriftDegrees`))
  (bind _returnvalue (/ (* (`KismetSystemLibrary.GetGameTimeInSeconds`) 360.0) (`self.DriftSeconds`)))
  ;[1 1 1 0.8] Event tick
  (`self.K2_SetActorRotation` (`KismetMathLibrary.MakeRotator` (.roll _baserotation) (+ (.pitch _baserotation) (* (`KismetMathLibrary.DegSin` (* _returnvalue 0.5)) (* _driftdegrees 0.35))) (+ (.yaw _baserotation) (* (`KismetMathLibrary.DegSin` _returnvalue) _driftdegrees)))))

(fn `UserConstructionScript`)
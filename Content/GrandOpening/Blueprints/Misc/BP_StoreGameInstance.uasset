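; Game instance for the store game that manages numbered save slots, including new game, load, delete and finding the most recent slot to continue.
; Saving gathers state from the game state's managers and the game mode into a store save, plus a small header save for slot listings.
; A temporary scene capture at the player camera exports each slot's PNG thumbnail.
; Loading only stores the save as pending; this file does not apply it.
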(fn `CaptureThumbnail`
  (params (Index :type Integer))
  (bind _returnvalue (`GameplayStatics.GetPlayerCameraManager` 0))
  ;[1 1 1 0.8] Capture thumbnail
  (bind _returnvalue_2 (`KismetRenderingLibrary.CreateRenderTarget2D` (`self.ThumbnailWidth`) (`self.ThumbnailHeight`) "RTF_RGBA8"))
  (bind _returnvalue_3 (`|SpawnActorFromClass` "/Script/Engine.SceneCapture2D" (`KismetMathLibrary.MakeTransform` (`PlayerCameraManager.GetCameraLocation` _returnvalue) (`PlayerCameraManager.GetCameraRotation` _returnvalue)) "AlwaysSpawn" "MultiplyWithRoot" null null))
  (bind _capturecomponent2d (`SceneCapture2D.CaptureComponent2D` _returnvalue_3))
  (set `SceneCaptureComponent2D.TextureTarget` _returnvalue_2 _capturecomponent2d)
  (set `SceneCaptureComponent.CaptureSource` "SCS_FinalColorLDR" _capturecomponent2d)
  (`SceneCaptureComponent2D.CaptureScene` _capturecomponent2d)
  (bind _folder (`self.ThumbnailFolder`))
  (bind _filename (`self.ThumbnailFile` Index))
  (`KismetRenderingLibrary.ExportRenderTarget` _returnvalue_2 _folder _filename)
  (`Actor.K2_DestroyActor` _returnvalue_3))

(fn `DeleteSlot`
  (params (Index :type Integer))
  ;[1 1 1 0.8] Delete slot
  (bind _slotname (`self.MakeSlotName` Index))
  (`GameplayStatics.DeleteGameInSlot` _slotname)
  (bind _headername (`self.MakeHeaderName` Index))
  (`GameplayStatics.DeleteGameInSlot` _headername))

(fn `HasSlot`
  (params (Index :type Integer))
  (returns (Exists :type Boolean))
  ;[1 1 1 0.8] Has slot
  (bind _slotname (`self.MakeSlotName` Index))
  (bind _returnvalue (`GameplayStatics.DoesSaveGameExist` _slotname))
  (return _returnvalue))

(fn `MakeHeaderName`
  (params (Index :type Integer))
  (returns (HeaderName :type String))
  ;[1 1 1 0.8] Make header name
  (bind _slotname (`self.MakeSlotName` Index))
  (return (`KismetStringLibrary.Concat_StrStr` _slotname "Header")))

(fn `MakeSlotName`
  (params (Index :type Integer))
  (returns (SlotName :type String))
  ;[1 1 1 0.8] Make slot name
  (return (`KismetStringLibrary.Concat_StrStr` "Slot" (`KismetStringLibrary.Conv_IntToString` Index))))

(fn `ReadSlotInfo`
  (params (Index :type Integer))
  (returns (Info :type "/Game/GrandOpening/Blueprints/Structures/S_SaveSlotInfo Structure"))
  (locals (Slot :type "/Game/GrandOpening/Blueprints/Structures/S_SaveSlotInfo Structure"))
  ;[1 1 1 0.8] Read slot info
  (bind _headername (`self.MakeHeaderName` Index))
  (bind _returnvalue (`GameplayStatics.LoadGameFromSlot` _headername))
  (bind _assg_slot_header (cast `/Game/GrandOpening/Blueprints/Misc/SG_SlotHeader` _returnvalue))
  (`/Engine/EditorBlueprintResources/StandardMacros.IsValid` _assg_slot_header
    (:`Is Valid`
      (bind _folder (`self.ThumbnailFolder`))
      (bind _filename (`self.ThumbnailFile` Index))
      (bind _returnvalue_2 (`KismetRenderingLibrary.ImportFileAsTexture2D` (`KismetStringLibrary.Concat_StrStr` (`KismetStringLibrary.Concat_StrStr` _folder "/") _filename)))
      (set `local.Slot` (make `/Game/GrandOpening/Blueprints/Structures/S_SaveSlotInfo` (`/Game/GrandOpening/Blueprints/Misc/SG_SlotHeader.SlotDay` _assg_slot_header) (`/Game/GrandOpening/Blueprints/Misc/SG_SlotHeader.SlotBalance` _assg_slot_header) (`/Game/GrandOpening/Blueprints/Misc/SG_SlotHeader.SlotRating` _assg_slot_header) (`/Game/GrandOpening/Blueprints/Misc/SG_SlotHeader.SavedAt` _assg_slot_header) _returnvalue_2)))
    (:`Is Not Valid`
      _))
  (return (`local.Slot`)))

(fn `RequestLoad`
  (params (Index :type Integer))
  ;[1 1 1 0.8] Request load
  (set `self.CurrentSlotIndex` Index)
  (bind _slotname (`self.MakeSlotName` Index))
  (bind _returnvalue (`GameplayStatics.LoadGameFromSlot` _slotname))
  (bind _assg_store_save (cast `/Game/GrandOpening/Blueprints/Misc/SG_StoreSave` _returnvalue))
  (set `self.PendingSave` _assg_store_save))

(fn `ResolveContinueSlotIndex`
  (returns (SlotIndex :type Integer))
  (locals (Found :type Integer) (Latest :type "DateTime Structure"))
  ;[1 1 1 0.8] Resolve continue slot index
  (set `local.Found` -1)
  (for _index (range (`self.SlotCount`))
    (bind _headername (`self.MakeHeaderName` _index))
    (bind _returnvalue (`GameplayStatics.LoadGameFromSlot` _headername))
    (bind _assg_slot_header (cast `/Game/GrandOpening/Blueprints/Misc/SG_SlotHeader` _returnvalue))
    (`/Engine/EditorBlueprintResources/StandardMacros.IsValid` _assg_slot_header
      (:`Is Valid`
        (bind _savedat (`/Game/GrandOpening/Blueprints/Misc/SG_SlotHeader.SavedAt` _assg_slot_header))
        (if (or (< (`local.Found`) 0) (> _savedat (`local.Latest`)))
          (set `local.Found` _index)
          (set `local.Latest` _savedat)))))
  (return (`local.Found`)))

(fn `SaveToSlot`
  (params (Index :type Integer))
  ;[1 1 1 0.8] Save to slot
  (bind _returnvalue (`GameplayStatics.CreateSaveGameObject` "/Game/GrandOpening/Blueprints/Misc/SG_StoreSave.SG_StoreSave_C"))
  (bind _asbp_store_game_state (cast `/Game/GrandOpening/Blueprints/Misc/BP_StoreGameState` (`GameplayStatics.GetGameState`)))
  (`/Game/GrandOpening/Blueprints/ActorComponents/BP_StoreManager.CollectInto` (`/Game/GrandOpening/Blueprints/Misc/BP_StoreGameState.BP_StoreManager` _asbp_store_game_state) _returnvalue)
  (`/Game/GrandOpening/Blueprints/ActorComponents/BP_EconomyManager.CollectInto` (`/Game/GrandOpening/Blueprints/Misc/BP_StoreGameState.BP_EconomyManager` _asbp_store_game_state) _returnvalue)
  (`/Game/GrandOpening/Blueprints/ActorComponents/BP_DeliveryManager.CollectInto` (`/Game/GrandOpening/Blueprints/Misc/BP_StoreGameState.BP_DeliveryManager` _asbp_store_game_state) _returnvalue)
  (`/Game/GrandOpening/Blueprints/ActorComponents/BP_AdManager.CollectInto` (`/Game/GrandOpening/Blueprints/Misc/BP_StoreGameState.BP_AdManager` _asbp_store_game_state) _returnvalue)
  (`/Game/GrandOpening/Blueprints/ActorComponents/BP_ProgressionManager.CollectInto` (`/Game/GrandOpening/Blueprints/Misc/BP_StoreGameState.BP_ProgressionManager` _asbp_store_game_state) _returnvalue)
  (`/Game/GrandOpening/Blueprints/ActorComponents/BP_StaffManager.CollectInto` (`/Game/GrandOpening/Blueprints/Misc/BP_StoreGameState.BP_StaffManager` _asbp_store_game_state) _returnvalue)
  (bind _asbp_store_game_mode (cast `/Game/GrandOpening/Blueprints/PlayerCharacter/BP_StoreGameMode` (`GameplayStatics.GetGameMode`)))
  (`/Game/GrandOpening/Blueprints/PlayerCharacter/BP_StoreGameMode.CollectWorldInto` _asbp_store_game_mode _returnvalue)
  (bind _slotname (`self.MakeSlotName` Index))
  (`GameplayStatics.SaveGameToSlot` _returnvalue _slotname)
  (bind _returnvalue_2 (`GameplayStatics.CreateSaveGameObject` "/Game/GrandOpening/Blueprints/Misc/SG_SlotHeader.SG_SlotHeader_C"))
  (set `/Game/GrandOpening/Blueprints/Misc/SG_SlotHeader.SlotDay` (`/Game/GrandOpening/Blueprints/Misc/SG_StoreSave.StoreDay` _returnvalue) _returnvalue_2)
  (set `/Game/GrandOpening/Blueprints/Misc/SG_SlotHeader.SlotBalance` (`/Game/GrandOpening/Blueprints/Misc/SG_StoreSave.Balance` _returnvalue) _returnvalue_2)
  (set `/Game/GrandOpening/Blueprints/Misc/SG_SlotHeader.SlotRating` (`/Game/GrandOpening/Blueprints/Misc/SG_StoreSave.Rating` _returnvalue) _returnvalue_2)
  (set `/Game/GrandOpening/Blueprints/Misc/SG_SlotHeader.SavedAt` (`KismetMathLibrary.Now`) _returnvalue_2)
  (bind _headername (`self.MakeHeaderName` Index))
  (`GameplayStatics.SaveGameToSlot` _returnvalue_2 _headername)
  (`self.CaptureThumbnail` Index)
  (set `self.CurrentSlotIndex` Index))

(fn `StartNewGame`
  (params (Index :type Integer))
  ;[1 1 1 0.8] Start new game
  (`self.DeleteSlot` Index)
  (set `self.PendingSave` null)
  (set `self.CurrentSlotIndex` Index))

(fn `ThumbnailFile`
  (params (Index :type Integer))
  (returns (FileName :type String))
  ;[1 1 1 0.8] Thumbnail file
  (bind _slotname (`self.MakeSlotName` Index))
  (return (`KismetStringLibrary.Concat_StrStr` _slotname ".png")))

(fn `ThumbnailFolder`
  (returns (Folder :type String))
  ;[1 1 1 0.8] Thumbnail folder
  (return (`KismetStringLibrary.Concat_StrStr` (`KismetSystemLibrary.GetProjectSavedDirectory`) "SaveGames")))
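; BP_ProductFlight is a short-lived actor that animates a collision-free product mesh flying to a pose relative to a target component.
; Launch stores the start, target and clearances, then Tick re-resolves the target each frame, so moving targets are followed.
; Time-remapped lerps lift it above both ends, carry it across and lower it, while rotation blends throughout.
; It calls OnArrived and self-destructs on completion, or silently self-destructs if the target becomes invalid.
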(event `self.ReceiveTick`
  (params (DeltaSeconds :type "Float (single-precision)"))
  (bind _travelstartalpha (`self.TravelStartAlpha`))
  (bind _travelendalpha (`self.TravelEndAlpha`))
  (bind _startlocation (`self.StartLocation`))
  (bind _targetcomponent (`self.TargetComponent`))
  (bind _z (.z _startlocation))
  (bind _returnvalue (+ (`self.Elapsed`) DeltaSeconds))
  (bind _returnvalue_2 (`KismetMathLibrary.ComposeTransforms` (`self.TargetLocal`) (`SceneComponent.K2_GetComponentToWorld` _targetcomponent)))
  (bind _returnvalue_3 (`KismetMathLibrary.FClamp` (/ _returnvalue (`self.Duration`))))
  (bind _location (.location _returnvalue_2))
  (bind _z_2 (.z _location))
  ;[1 1 1 0.8] Event tick
  (`/Engine/EditorBlueprintResources/StandardMacros.IsValid` _targetcomponent
    (:`Is Valid`
      (`self.K2_SetActorLocation` self (`KismetMathLibrary.MakeVector` (.x (`KismetMathLibrary.VLerp` _startlocation _location (`KismetMathLibrary.MapRangeClamped` _returnvalue_3 _travelstartalpha _travelendalpha 0.0 1.0))) (.y (`KismetMathLibrary.VLerp` _startlocation _location (`KismetMathLibrary.MapRangeClamped` _returnvalue_3 _travelstartalpha _travelendalpha 0.0 1.0))) (`KismetMathLibrary.Lerp` (`KismetMathLibrary.Lerp` _z (`KismetMathLibrary.FMax` (`KismetMathLibrary.FMax` (+ _z (`self.StartClearanceCm`)) (+ _z_2 (`self.TargetClearanceCm`))) (+ (`KismetMathLibrary.FMax` _z _z_2) (`self.ArcHeightCm`))) (`KismetMathLibrary.MapRangeClamped` _returnvalue_3 0.0 _travelstartalpha 0.0 1.0)) _z_2 (`KismetMathLibrary.MapRangeClamped` _returnvalue_3 _travelendalpha 1.0 0.0 1.0))) false false)
      (`self.K2_SetActorRotation` self (`KismetMathLibrary.RLerp` (`self.StartRotation`) (.rotation _returnvalue_2) _returnvalue_3) false)
      (set `self.Elapsed` _returnvalue)
      (if (>= (`self.Elapsed`) (`self.Duration`))
        (`self.OnArrived`)
        (`self.K2_DestroyActor` self)))
    (:`Is Not Valid`
      (`self.K2_DestroyActor` self))))

(fn `Launch`
  (params (Mesh :type "StaticMesh Object Reference") (Target :type "SceneComponent Object Reference") (LocalPose :type "Transform Structure") (StartClearanceCm :type "Float (double-precision)") (TargetClearanceCm :type "Float (double-precision)"))
  ;[1 1 1 0.8] Launch
  (`StaticMeshComponent.SetStaticMesh` (`self.UnitMesh`) Mesh)
  (`PrimitiveComponent.SetCollisionEnabled` (`self.UnitMesh`) "NoCollision")
  (set `self.StartLocation` (`self.K2_GetActorLocation` self))
  (set `self.StartRotation` (`self.K2_GetActorRotation` self))
  (set `self.TargetComponent` Target)
  (set `self.TargetLocal` LocalPose)
  (set `self.StartClearanceCm` StartClearanceCm)
  (set `self.TargetClearanceCm` TargetClearanceCm)
  (set `self.Elapsed` 0.0)
  (`self.SetActorTickEnabled` self true))

(fn `UserConstructionScript`)
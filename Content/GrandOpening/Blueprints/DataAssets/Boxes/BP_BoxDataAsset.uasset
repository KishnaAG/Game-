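; Data asset describing a box type, with a function that works out how many units of a given product fit inside it.
; CapacityFor floors the interior size over the product footprint in X and Y for a grid count, then multiplies by the vertical stack count.
; Stack height is capped by the product's StackMax, and every axis is clamped to at least one, so capacity never drops to zero.
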(fn `CapacityFor`
  (params (Product :type "/Game/GrandOpening/Blueprints/DataAssets/Products/BP_ProductDataAsset Object Reference"))
  (returns (Capacity :type Integer))
  (bind (_x _y) (`KismetMathLibrary.BreakVector2D` (`/Game/GrandOpening/Blueprints/DataAssets/Products/BP_ProductDataAsset.FootprintCm` Product)))
  ;[1 1 1 0.8] Capacity for
  (return (* (* (`KismetMathLibrary.Max` 1 (`KismetMathLibrary.FFloor` (/ (.x (`self.InteriorSizeCm`)) _x))) (`KismetMathLibrary.Max` 1 (`KismetMathLibrary.FFloor` (/ (.y (`self.InteriorSizeCm`)) _y)))) (`KismetMathLibrary.Max` 1 (`KismetMathLibrary.Min` (`/Game/GrandOpening/Blueprints/DataAssets/Products/BP_ProductDataAsset.StackMax` Product) (`KismetMathLibrary.FFloor` (/ (.z (`self.InteriorSizeCm`)) (`/Game/GrandOpening/Blueprints/DataAssets/Products/BP_ProductDataAsset.StackHeightCm` Product))))))))
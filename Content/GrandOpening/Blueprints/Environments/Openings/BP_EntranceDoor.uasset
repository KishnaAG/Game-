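; BP_EntranceDoor is an entrance door that plays a bell on trigger overlap and arbitrates agents passing between outdoors and indoors.
; RequestPassage always grants agents beyond the approach radius or not changing sides, using a right-vector dot product to tell indoors from outdoors.
; Crossing agents share the doorway in one flow direction while nobody waits; others queue first-come, first-served until occupants are released explicitly or by distance.
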(event `self.BellTrigger.OnComponentBeginOverlap`
  (params (OverlappedComponent :type "PrimitiveComponent Object Reference") (OtherActor :type "Actor Object Reference") (OtherComp :type "PrimitiveComponent Object Reference") (OtherBodyIndex :type Integer) (bFromSweep :type Boolean) (SweepResult :type "HitResult Structure (by ref)"))
  ;[1 1 1 0.8] On component begin overlap
  (`GameplayStatics.SpawnSoundAttached` (`self.BellSound`) (`self.Threshold`) "None" (0.0 0.0 200.0) (struct) "KeepRelativeOffset" false 1.0 1.0 0.0 null null))

(fn `IsIndoors`
  (params (Point :type "Vector Structure"))
  (returns (ReturnValue :type Boolean))
  ;[1 1 1 0.8] Is indoors
  (return (> (`KismetMathLibrary.Dot_VectorVector` (- Point (`self.K2_GetActorLocation`)) (`self.GetActorRightVector`)) 0.0)))

(fn `ReleasePassage`
  (params (Agent :type "Actor Object Reference"))
  ;[1 1 1 0.8] Release passage
  (`KismetArrayLibrary.Array_RemoveItem` (`self.Occupants`) Agent)
  (`KismetArrayLibrary.Array_RemoveItem` (`self.Waiting`) Agent))

(fn `RequestPassage`
  (params (Agent :type "Actor Object Reference") (Destination :type "Vector Structure"))
  (returns (ReturnValue :type Boolean))
  (locals (Granted :type Boolean))
  (bind _returnvalue (`self.K2_GetActorLocation` Agent))
  (bind _granted (`local.Granted`))
  (bind _returnvalue_2 (<= (`KismetMathLibrary.Vector_Distance2D` _returnvalue (`SceneComponent.K2_GetComponentLocation` (`self.Threshold`))) (`self.ApproachRadiusCm`)))
  ;[1 1 1 0.8] Request passage
  (bind _returnvalue_3 (`self.IsIndoors` Destination))
  (bind _returnvalue_4 (`self.IsIndoors` _returnvalue))
  (if (not _returnvalue_2)
    (`self.ReleasePassage` Agent))
  (set `local.Granted` (or (or (not _returnvalue_2) (== _returnvalue_3 _returnvalue_4)) (`KismetArrayLibrary.Array_Contains` (`self.Occupants`) Agent)))
  (if (not _granted)
    (if (or (and (== (`KismetArrayLibrary.Array_Length` (`self.Occupants`)) 0) (or (== (`KismetArrayLibrary.Array_Length` (`self.Waiting`)) 0) (== (`|GetArrayItem` (`self.Waiting`)) Agent))) (and (and (> (`KismetArrayLibrary.Array_Length` (`self.Occupants`)) 0) (== (`KismetArrayLibrary.Array_Length` (`self.Waiting`)) 0)) (== (`self.FlowIndoors`) _returnvalue_3)))
      (`KismetArrayLibrary.Array_Add` (`self.Occupants`) Agent)
      (`KismetArrayLibrary.Array_RemoveItem` (`self.Waiting`) Agent)
      (set `self.FlowIndoors` _returnvalue_3)
      (set `local.Granted` true)
      (else
        (`KismetArrayLibrary.Array_AddUnique` (`self.Waiting`) Agent)
        (set `local.Granted` false))))
  (return _granted))

(fn `UserConstructionScript`)
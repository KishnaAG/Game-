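; BP_ScreenBase is a base interactable in-world screen that shows a widget and can be switched on or off.
; On begin play it sets the widget's host to itself or its parent actor.
; Interacting releases the carried item, focuses the player's view on the read pose, hides the crosshair and calls the empty BeginRead hook, or clears focus if already focused.
; SetPowered toggles display visibility and interactability.
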(event `self.ReceiveBeginPlay`
  (bind _returnvalue (`self.GetParentActor`))
  ;[1 1 1 0.8] Event begin play
  (bind _asbp_screen_base_widget (cast `/Game/GrandOpening/Blueprints/Widgets/World/BP_ScreenBaseWidget` (`WidgetComponent.GetWidget` (`self.DisplayWidget`))))
  (if (`self.HostIsSelf`)
    (`/Game/GrandOpening/Blueprints/Widgets/World/BP_ScreenBaseWidget.SetHost` _asbp_screen_base_widget self :!label _label)
    (else
      (`/Engine/EditorBlueprintResources/StandardMacros.IsValid` _returnvalue
        (:`Is Valid`
          (`/Game/GrandOpening/Blueprints/Widgets/World/BP_ScreenBaseWidget.SetHost` _asbp_screen_base_widget _returnvalue))
        (:`Is Not Valid`
          (goto _label))))))

(event `self.BP_InteractableComponent.OnInteracted`
  (params (Interactor :type "Actor Object Reference"))
  (bind _readposescene (`self.ReadPoseScene`))
  ;[1 1 1 0.8] On interacted
  ;;[1 1 1 0.8] Setup focus and setup
  (bind _asbp_store_character (cast `/Game/GrandOpening/Blueprints/PlayerCharacter/BP_StoreCharacter` Interactor))
  (bind _returnvalue (`self.GetComponentByClass` _asbp_store_character "/Game/GrandOpening/Blueprints/ActorComponents/BP_ViewMotionComponent.BP_ViewMotionComponent_C"))
  (if (`/Game/GrandOpening/Blueprints/ActorComponents/BP_ViewMotionComponent.Focusing` _returnvalue)
    (`/Game/GrandOpening/Blueprints/ActorComponents/BP_ViewMotionComponent.ClearFocus` _returnvalue)
    (bind _returnvalue_2 (`self.GetComponentByClass` _asbp_store_character "/Game/GrandOpening/Blueprints/ActorComponents/BP_InteractionComponent.BP_InteractionComponent_C"))
    (`/Game/GrandOpening/Blueprints/ActorComponents/BP_InteractionComponent.ShowCrosshair` _returnvalue_2)
    (else
      (`/Game/GrandOpening/Blueprints/ActorComponents/BP_CarryComponent.ReleaseActor` (`self.GetComponentByClass` _asbp_store_character "/Game/GrandOpening/Blueprints/ActorComponents/BP_CarryComponent.BP_CarryComponent_C"))
      (`/Game/GrandOpening/Blueprints/ActorComponents/BP_ViewMotionComponent.FocusOn` _returnvalue (`SceneComponent.K2_GetComponentLocation` _readposescene) (`SceneComponent.K2_GetComponentRotation` _readposescene))
      (`/Game/GrandOpening/Blueprints/ActorComponents/BP_InteractionComponent.HideCrosshair` _returnvalue_2)
      (`self.BeginRead` Interactor))))

(fn `BeginRead`
  (params (Reader :type "Actor Object Reference"))
  ;[1 1 1 0.8] Begin read
)

(fn `SetPowered`
  (params (Powered :type Boolean))
  ;[1 1 1 0.8] Set powered
  (`SceneComponent.SetHiddenInGame` (`self.DisplayWidget`) (not Powered) false)
  (`/Game/GrandOpening/Blueprints/ActorComponents/BP_InteractableComponent.SetInteractable` (`self.BP_InteractableComponent`) Powered))

(fn `UserConstructionScript`)
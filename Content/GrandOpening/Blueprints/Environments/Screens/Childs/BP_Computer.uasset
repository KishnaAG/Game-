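; BP_Computer is an in-world computer screen that a store character can read and operate with the mouse through its BP_ComputerWidget.
; BeginRead shows the cursor, switches to game-and-UI input, refreshes the current app, has BP_ProgressionManager evaluate, then refreshes the desktop.
; It binds to the reader's BP_ViewMotionComponent focus-ended event, whose handler hides the cursor, restores game-only input and unbinds itself.
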(event `self.BeginRead`
  (params (Reader :type "Actor Object Reference"))
  (bind _reader (`self.Reader`))
  ;[1 1 1 0.8] Event begin read
  ;;[1 1 1 0.8] Event begin read
  (bind _asbp_store_character (cast `/Game/GrandOpening/Blueprints/PlayerCharacter/BP_StoreCharacter` Reader))
  (set `self.Reader` _asbp_store_character)
  (bind _asbp_computer_widget (cast `/Game/GrandOpening/Blueprints/Widgets/World/BP_ComputerWidget` (`WidgetComponent.GetWidget` (`self.DisplayWidget`))))
  (set `self.ComputerWidget` _asbp_computer_widget)
  (bind _asplayer_controller (cast `PlayerController` (`Pawn.GetController` _reader)))
  (set `PlayerController.bShowMouseCursor` true _asplayer_controller)
  (`WidgetBlueprintLibrary.SetInputMode_GameAndUIEx` _asplayer_controller null "DoNotLock" false)
  (add `/Game/GrandOpening/Blueprints/ActorComponents/BP_ViewMotionComponent.OnFocusEnded` (`self.GetComponentByClass` _reader "/Game/GrandOpening/Blueprints/ActorComponents/BP_ViewMotionComponent.BP_ViewMotionComponent_C") (delegate `HandleFocusEnded`))
  (`/Game/GrandOpening/Blueprints/Widgets/World/BP_ComputerWidget.RefreshCurrentApp` (`self.ComputerWidget`))
  (`/Game/GrandOpening/Blueprints/ActorComponents/BP_ProgressionManager.Evaluate` (`self.GetComponentByClass` (`GameplayStatics.GetGameState`) "/Game/GrandOpening/Blueprints/ActorComponents/BP_ProgressionManager.BP_ProgressionManager_C"))
  (`/Game/GrandOpening/Blueprints/Widgets/World/BP_ComputerWidget.RefreshDesktop` (`self.ComputerWidget`)))

(event `HandleFocusEnded`
  (bind _reader (`self.Reader`))
  ;[1 1 1 0.8] Event begin read
  ;;[1 1 1 0.8] Handle focus ended
  (bind _asplayer_controller (cast `PlayerController` (`Pawn.GetController` _reader)))
  (set `PlayerController.bShowMouseCursor` false _asplayer_controller)
  (`WidgetBlueprintLibrary.SetInputMode_GameOnly` _asplayer_controller)
  (remove `/Game/GrandOpening/Blueprints/ActorComponents/BP_ViewMotionComponent.OnFocusEnded` (`self.GetComponentByClass` _reader "/Game/GrandOpening/Blueprints/ActorComponents/BP_ViewMotionComponent.BP_ViewMotionComponent_C") (delegate `HandleFocusEnded`)))

(fn `UserConstructionScript`
  (`parent.UserConstructionScript`))
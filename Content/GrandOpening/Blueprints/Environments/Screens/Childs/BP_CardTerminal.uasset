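; Card terminal screen actor for a checkout, where a reader completes a card payment through an on-screen widget.
; BeginRead gives the player a mouse cursor with game-and-UI input, and PowerOn shows the card and hands the terminal to its widget.
; InsertCard launches a spawned flight actor carrying the card mesh to the slot.
; Approve finishes the sale on the parent checkout, powers off and restores focus and crosshair.
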(event `self.BeginRead`
  (params (Reader :type "Actor Object Reference"))
  ;[1 1 1 0.8] Event begin read
  (bind _aspawn (cast `Pawn` Reader))
  (bind _asplayer_controller (cast `PlayerController` (`Pawn.GetController` _aspawn)))
  (set `self.Reader` Reader)
  (set `PlayerController.bShowMouseCursor` true _asplayer_controller)
  (`WidgetBlueprintLibrary.SetInputMode_GameAndUIEx` _asplayer_controller null "DoNotLock" false))

(fn `Approve`
  (params (Amount :type "Float (double-precision)"))
  ;[1 1 1 0.8] Approve
  (bind _asbp_checkout_base (cast `/Game/GrandOpening/Blueprints/Environments/Checkout/BP_CheckoutBase` (`self.GetParentActor`)))
  (`/Game/GrandOpening/Blueprints/Environments/Checkout/BP_CheckoutBase.FinishSale` _asbp_checkout_base Amount)
  (`self.PowerOff` self)
  (`self.Close` self))

(fn `Close`
  (bind _reader (`self.Reader`))
  ;[1 1 1 0.8] Close
  (`/Game/GrandOpening/Blueprints/ActorComponents/BP_ViewMotionComponent.ClearFocus` (`self.GetComponentByClass` _reader "/Game/GrandOpening/Blueprints/ActorComponents/BP_ViewMotionComponent.BP_ViewMotionComponent_C"))
  (`/Game/GrandOpening/Blueprints/ActorComponents/BP_InteractionComponent.ShowCrosshair` (`self.GetComponentByClass` _reader "/Game/GrandOpening/Blueprints/ActorComponents/BP_InteractionComponent.BP_InteractionComponent_C")))

(fn `InsertCard`
  (params (Start :type "Transform Structure"))
  (bind _card (`self.Card`))
  ;[1 1 1 0.8] Insert card
  (bind _returnvalue (`|SpawnActorFromClass` (`self.FlightClass`) Start "Undefined" "MultiplyWithRoot" null null))
  (add `/Game/GrandOpening/Blueprints/Misc/BP_ProductFlight.OnArrived` _returnvalue (`|CreateDelegate` :!event `PowerOn`))
  (`/Game/GrandOpening/Blueprints/Misc/BP_ProductFlight.Launch` _returnvalue (`StaticMeshComponent.StaticMesh` _card) _card (`KismetMathLibrary.MakeTransform` (0.0 0.0 0.0)) 0.0 0.0))

(fn `PowerOff`
  ;[1 1 1 0.8] Power off
  (`self.SetPowered` false)
  (`SceneComponent.SetHiddenInGame` (`self.Card`) true false))

(fn `PowerOn`
  ;[1 1 1 0.8] Power on
  (`self.SetPowered` true)
  (`SceneComponent.SetHiddenInGame` (`self.Card`) false false)
  (bind _asbp_card_terminal_widget (cast `/Game/GrandOpening/Blueprints/Widgets/World/BP_CardTerminalWidget` (`WidgetComponent.GetWidget` (`self.DisplayWidget`))))
  (`/Game/GrandOpening/Blueprints/Widgets/World/BP_CardTerminalWidget.SetTerminal` _asbp_card_terminal_widget self))

(fn `UserConstructionScript`
  (`parent.UserConstructionScript`))
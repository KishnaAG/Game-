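; Customer spawner that sends shoppers into the store while it is serving customers.
; A self-rescheduling timer derives its delay from DayConfig's hourly rate, scaled by day difficulty and ad traffic, and resets on StoreManager hour or serving changes.
; Each tick picks a weighted-random archetype, spawning it only if shelves stock something it wants and a checkout can serve.
; The archetype is then passed to the new customer's BP_CustomerBrain for initialization.
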(event `self.ReceiveBeginPlay`
  ;[1 1 1 0.8] Event begin play
  (set `self.StoreManager` (`self.GetComponentByClass` (`GameplayStatics.GetGameState`) "/Game/GrandOpening/Blueprints/ActorComponents/BP_StoreManager.BP_StoreManager_C"))
  (`/Engine/EditorBlueprintResources/StandardMacros.IsValid` (`self.StoreManager`)
    (:`Is Valid`
      (add `/Game/GrandOpening/Blueprints/ActorComponents/BP_StoreManager.OnHourChanged` (`self.StoreManager`) (`|CreateDelegate` :!event `HandleHourChanged`))
      (add `/Game/GrandOpening/Blueprints/ActorComponents/BP_StoreManager.OnServingChanged` (`self.StoreManager`) (`|CreateDelegate` :!event `HandleServingChanged`))
      (`self.ScheduleNextCustomer`))))

(fn `GetCustomerRate`
  (returns (Rate :type "Float (double-precision)"))
  (bind _dayconfig (`self.DayConfig`))
  (bind _storemanager (`self.StoreManager`))
  (bind _returnvalue (`self.GetComponentByClass` (`GameplayStatics.GetGameState`) "/Game/GrandOpening/Blueprints/ActorComponents/BP_AdManager.BP_AdManager_C"))
  (bind _returnvalue_2 (* (`|GetArrayItem` (`/Game/GrandOpening/Blueprints/DataAssets/Day/BP_DayConfigDataAsset.CustomersPerHour` _dayconfig) (`/Game/GrandOpening/Blueprints/ActorComponents/BP_StoreManager.CurrentHour` _storemanager)) (+ 1.0 (* (`/Game/GrandOpening/Blueprints/DataAssets/Day/BP_DayConfigDataAsset.DifficultyPerDay` _dayconfig) (`KismetMathLibrary.Conv_IntToDouble` (- (`/Game/GrandOpening/Blueprints/ActorComponents/BP_StoreManager.CurrentDay` _storemanager) 1))))))
  ;[1 1 1 0.8] Get customer rate
  (`/Engine/EditorBlueprintResources/StandardMacros.IsValid` _returnvalue
    (:`Is Valid`
      (bind _multiplier (`/Game/GrandOpening/Blueprints/ActorComponents/BP_AdManager.TrafficMultiplier` _returnvalue))
      (return (* _returnvalue_2 _multiplier)))
    (:`Is Not Valid`
      (return _returnvalue_2))))

(fn `HandleHourChanged`
  (params (Day :type Integer) (Hour :type Integer))
  ;[1 1 1 0.8] Handle hour changed
  (`self.ScheduleNextCustomer`))

(fn `HandleServingChanged`
  (params (Serving :type Boolean))
  ;[1 1 1 0.8] Handle serving changed
  (if Serving
    (`self.ScheduleNextCustomer` self)
    (else
      (`KismetSystemLibrary.K2_ClearAndInvalidateTimerHandle` (`self.SpawnTimer`)))))

(fn `PickArchetype`
  (returns (Archetype :type "/Game/GrandOpening/Blueprints/DataAssets/Customers/BP_CustomerArchetypeDataAsset Object Reference"))
  (locals (Total :type "Float (double-precision)") (Roll :type "Float (double-precision)") (Picked :type "/Game/GrandOpening/Blueprints/DataAssets/Customers/BP_CustomerArchetypeDataAsset Object Reference"))
  (bind _archetypemix (`/Game/GrandOpening/Blueprints/DataAssets/Day/BP_DayConfigDataAsset.ArchetypeMix` (`self.DayConfig`)))
  ;[1 1 1 0.8] Pick archetype
  (for _array_element _archetypemix
    (set `local.Total` (+ (`local.Total`) (`.Weight_5_82E12D83496D24324B03239799BA596C` (break `/Game/GrandOpening/Blueprints/Structures/S_ArchetypeMix` _array_element)))))
  (set `local.Roll` (`KismetMathLibrary.RandomFloatInRange` 0.0 (`local.Total`)))
  (for _array_element_2 _archetypemix
    (if (>= (`local.Roll`) 0.0)
      (bind (_archetype _weight) (break `/Game/GrandOpening/Blueprints/Structures/S_ArchetypeMix` _array_element_2))
      (set `local.Picked` _archetype))
    (set `local.Roll` (- (`local.Roll`) _weight)))
  (return (`local.Picked`)))

(fn `ScheduleNextCustomer`
  (locals (Delay :type "Float (double-precision)"))
  (bind _hourdurationseconds (`/Game/GrandOpening/Blueprints/DataAssets/Store/BP_StoreConfigDataAsset.HourDurationSeconds` (`/Game/GrandOpening/Blueprints/ActorComponents/BP_StoreManager.StoreConfig` (`self.StoreManager`))))
  ;[1 1 1 0.8] Schedule next customer
  (`KismetSystemLibrary.K2_ClearAndInvalidateTimerHandle` (`self.SpawnTimer`))
  (if (`/Game/GrandOpening/Blueprints/ActorComponents/BP_StoreManager.ServingCustomers` (`self.StoreManager`))
    (bind _rate (`self.GetCustomerRate` self))
    (if (> _rate 0.0)
      (set `local.Delay` (/ _hourdurationseconds _rate))
      (else
        (set `local.Delay` _hourdurationseconds)))
    (bind _returnvalue (`KismetSystemLibrary.K2_SetTimer` self "SpawnCustomer" (`local.Delay`)))
    (set `self.SpawnTimer` _returnvalue)))

(fn `SpawnCustomer`
  ;[1 1 1 0.8] Spawn customer
  (`self.ScheduleNextCustomer` self)
  (bind _archetype (`self.PickArchetype` self))
  (`/Engine/EditorBlueprintResources/StandardMacros.IsValid` _archetype
    (:`Is Valid`
      (bind _something (`self.StoreHasSomethingFor` self _archetype))
      (bind _returnvalue (`self.StoreHasOpenCheckout`))
      (if (and _something _returnvalue)
        (bind _returnvalue_2 (`|SpawnActorFromClass` (`self.CustomerClass`) (`KismetMathLibrary.MakeTransform` (`SceneComponent.K2_GetComponentLocation` (`self.SpawnPoint`))) "AdjustIfPossibleButAlwaysSpawn" "MultiplyWithRoot" null null))
        (`/Engine/EditorBlueprintResources/StandardMacros.IsValid` _returnvalue_2
          (:`Is Valid`
            (bind _returnvalue_3 (`self.GetComponentByClass` _returnvalue_2 "/Game/GrandOpening/Blueprints/ActorComponents/BP_CustomerBrain.BP_CustomerBrain_C"))
            (set `/Game/GrandOpening/Blueprints/ActorComponents/BP_CustomerBrain.Archetype` _archetype _returnvalue_3)
            (`/Game/GrandOpening/Blueprints/ActorComponents/BP_CustomerBrain.InitializeCustomer` _returnvalue_3)))))))

(fn `StoreHasOpenCheckout`
  (returns (ReturnValue :type Boolean))
  (locals (Found :type Boolean))
  ;[1 1 1 0.8] Store has open checkout
  (set `local.Found` false)
  (bind _outactors (`GameplayStatics.GetAllActorsOfClass` "/Game/GrandOpening/Blueprints/Environments/Checkout/BP_CheckoutBase.BP_CheckoutBase_C"))
  (for _array_element _outactors
    (bind _returnvalue (`/Game/GrandOpening/Blueprints/Environments/Checkout/BP_CheckoutBase.CanServe` _array_element))
    (if _returnvalue
      (set `local.Found` true)
      (break)))
  (return (`local.Found`)))

(fn `StoreHasSomethingFor`
  (params (Archetype :type "/Game/GrandOpening/Blueprints/DataAssets/Customers/BP_CustomerArchetypeDataAsset Object Reference"))
  (returns (Something :type Boolean))
  ;[1 1 1 0.8] Store has something for
  (bind _outactors (`GameplayStatics.GetAllActorsOfClass` "/Game/GrandOpening/Blueprints/Environments/Shelves/BP_ShelfBase.BP_ShelfBase_C"))
  (for _array_element _outactors
    (bind _products (`/Game/GrandOpening/Blueprints/Environments/Shelves/BP_ShelfBase.StockedProducts` _array_element))
    (for _array_element_2 _products
      (bind _wanted (`/Game/GrandOpening/Blueprints/DataAssets/Customers/BP_CustomerArchetypeDataAsset.GetWants` Archetype _array_element_2 (`/Game/GrandOpening/Blueprints/DataAssets/Customers/BP_CustomerArchetypeDataAsset.BudgetMax` Archetype)))
      (if _wanted
        (return true))))
  (return false))

(fn `UserConstructionScript`)
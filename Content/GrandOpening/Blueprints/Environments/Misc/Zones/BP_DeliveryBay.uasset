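; BP_DeliveryBay is a delivery zone actor that hands out drop positions for incoming deliveries.
; On begin play it registers itself with the BP_DeliveryManager component on the game state, if present.
; TakeNextSlot cycles round-robin through a row-and-column grid and returns a world transform at drop height, aligned to the bay's location and rotation.
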(event `self.ReceiveBeginPlay`
  (bind _returnvalue (`self.GetComponentByClass` (`GameplayStatics.GetGameState`) "/Game/GrandOpening/Blueprints/ActorComponents/BP_DeliveryManager.BP_DeliveryManager_C"))
  ;[1 1 1 0.8] Event begin play
  (`/Engine/EditorBlueprintResources/StandardMacros.IsValid` _returnvalue
    (:`Is Valid`
      (`/Game/GrandOpening/Blueprints/ActorComponents/BP_DeliveryManager.RegisterBay` _returnvalue self))))

(fn `TakeNextSlot`
  (returns (SlotTransform :type "Transform Structure"))
  (locals (Slot :type Integer))
  (bind _returnvalue (`self.GetTransform`))
  (bind _slotsperrow (`self.SlotsPerRow`))
  (bind _slotpitchcm (`self.SlotPitchCm`))
  ;[1 1 1 0.8] Take next slot
  (set `local.Slot` (mod (`self.NextSlotIndex`) (* _slotsperrow (`self.SlotRows`))))
  (set `self.NextSlotIndex` (+ (`local.Slot`) 1))
  (return (`KismetMathLibrary.MakeTransform` (`KismetMathLibrary.TransformLocation` _returnvalue (`KismetMathLibrary.MakeVector` (* (/ (`local.Slot`) _slotsperrow) _slotpitchcm) (* (mod (`local.Slot`) _slotsperrow) _slotpitchcm) (`self.DropHeightCm`))) (.rotation _returnvalue))))

(fn `UserConstructionScript`)
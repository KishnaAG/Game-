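; BP_AdPanel is an advertising panel prop that displays the poster of an ad campaign.
; On BeginPlay it creates a dynamic material for the body mesh's poster slot and registers with the game state's ad manager component, unregistering on EndPlay.
; ShowCampaign sets the base color texture to the campaign's poster, falling back to a blank poster when the campaign or its poster is missing.
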(event `self.ReceiveBeginPlay`
  (bind _bodymesh (`self.BodyMesh`))
  (bind _returnvalue (`self.GetComponentByClass` (`GameplayStatics.GetGameState`) "/Game/GrandOpening/Blueprints/ActorComponents/BP_AdManager.BP_AdManager_C"))
  ;[1 1 1 0.8] Event begin play
  (bind _returnvalue_2 (`PrimitiveComponent.CreateDynamicMaterialInstance` _bodymesh (`PrimitiveComponent.GetMaterialIndex` _bodymesh "M_AdPoster") null "None"))
  (set `self.PosterMaterial` _returnvalue_2)
  (set `self.AdManager` _returnvalue)
  (`/Engine/EditorBlueprintResources/StandardMacros.IsValid` _returnvalue
    (:`Is Valid`
      (`/Game/GrandOpening/Blueprints/ActorComponents/BP_AdManager.RegisterPanel` _returnvalue self))))

(event `self.ReceiveEndPlay`
  (params (EndPlayReason :type "EEndPlayReason Enum" :default "Destroyed"))
  (bind _admanager (`self.AdManager`))
  ;[1 1 1 0.8] Event end play
  (`/Engine/EditorBlueprintResources/StandardMacros.IsValid` _admanager
    (:`Is Valid`
      (`/Game/GrandOpening/Blueprints/ActorComponents/BP_AdManager.UnregisterPanel` _admanager self))))

(fn `PosterFor`
  (params (Campaign :type "/Game/GrandOpening/Blueprints/DataAssets/Ads/BP_AdCampaignDataAsset Object Reference"))
  (returns (Poster :type "Texture2D Object Reference"))
  (bind _poster (`/Game/GrandOpening/Blueprints/DataAssets/Ads/BP_AdCampaignDataAsset.Poster` Campaign))
  ;[1 1 1 0.8] Poster for
  (`/Engine/EditorBlueprintResources/StandardMacros.IsValid` Campaign
    (:`Is Valid`
      (`/Engine/EditorBlueprintResources/StandardMacros.IsValid` _poster
        (:`Is Valid`
          (return _poster))
        (:`Is Not Valid`
          (return (`self.BlankPoster`)))))
    (:`Is Not Valid`
      (return (`self.BlankPoster`)))))

(fn `ShowCampaign`
  (params (Campaign :type "/Game/GrandOpening/Blueprints/DataAssets/Ads/BP_AdCampaignDataAsset Object Reference"))
  (bind _postermaterial (`self.PosterMaterial`))
  ;[1 1 1 0.8] Show campaign
  (`/Engine/EditorBlueprintResources/StandardMacros.IsValid` _postermaterial
    (:`Is Valid`
      (bind _poster (`self.PosterFor` Campaign))
      (`MaterialInstanceDynamic.SetTextureParameterValue` _postermaterial "BaseColorTex" _poster))))

(fn `UserConstructionScript`)
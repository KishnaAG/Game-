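; BP_OpenSign is the store's open sign, which a player interacts with to request closing the store.
; A looping timer starts at BeginPlay, alongside an initial RefreshEnabled check.
; RefreshEnabled scans all BP_Customer actors and makes the sign interactable only if each customer's brain is in one of two specific states.
; Interaction casts to the store character and its player controller, then calls RequestCloseStore.
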(event `self.ReceiveBeginPlay`
  ;[1 1 1 0.8] Event begin play
  (`self.RefreshEnabled`)
  (`KismetSystemLibrary.K2_SetTimerDelegate` (`|CreateDelegate` :!event `RefreshEnabled`) (`self.RefreshSeconds`) true))

(event `self.BP_InteractableComponent.OnInteracted`
  (params (Interactor :type "Actor Object Reference"))
  ;[1 1 1 0.8] On interacted
  (bind _asbp_store_character (cast `/Game/GrandOpening/Blueprints/PlayerCharacter/BP_StoreCharacter` Interactor))
  (bind _asbp_store_player_controller (cast `/Game/GrandOpening/Blueprints/PlayerCharacter/BP_StorePlayerController` (`Pawn.GetController` _asbp_store_character)))
  (`/Game/GrandOpening/Blueprints/PlayerCharacter/BP_StorePlayerController.RequestCloseStore` _asbp_store_player_controller))

(fn `RefreshEnabled`
  (bind _bp_interactablecomponent (`self.BP_InteractableComponent`))
  ;[1 1 1 0.8] Refresh enabled
  (`/Game/GrandOpening/Blueprints/ActorComponents/BP_InteractableComponent.SetInteractable` _bp_interactablecomponent true)
  (bind _outactors (`GameplayStatics.GetAllActorsOfClass` "/Game/GrandOpening/Blueprints/AI/Customer/BP_Customer.BP_Customer_C"))
  (for _array_element _outactors
    (bind _state (`/Game/GrandOpening/Blueprints/ActorComponents/BP_CustomerBrain.State` (`/Game/GrandOpening/Blueprints/AI/Customer/BP_Customer.BP_CustomerBrain` _array_element)))
    (if (and (`|EnumInequality` _state "NewEnumerator6") (`|EnumInequality` _state "NewEnumerator7"))
      (`/Game/GrandOpening/Blueprints/ActorComponents/BP_InteractableComponent.SetInteractable` _bp_interactablecomponent false))))

(fn `UserConstructionScript`)
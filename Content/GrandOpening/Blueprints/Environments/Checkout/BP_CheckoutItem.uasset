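; BP_CheckoutItem is a product at a checkout that the player scans by interacting with it, passing itself to its Checkout.
; ConfigureItem sets the product mesh, owning checkout and lateral offset, then refreshes the scan prompt.
; The item is interactable only while the player carries that checkout's paired scanner and the checkout is unmanned.
; BeginPlay binds to the player carry component's carry-changed event.
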(event `self.BP_InteractableComponent.OnInteracted`
  (params (Interactor :type "Actor Object Reference"))
  ;[1 1 1 0.8] On interacted
  (`/Game/GrandOpening/Blueprints/Environments/Checkout/BP_CheckoutBase.ScanItem` (`self.Checkout`) self))

(event `self.ReceiveBeginPlay`
  ;[1 1 1 0.8] Event begin play
  (add `/Game/GrandOpening/Blueprints/ActorComponents/BP_CarryComponent.OnCarryChanged` (`self.GetComponentByClass` (`GameplayStatics.GetPlayerCharacter` 0) "/Game/GrandOpening/Blueprints/ActorComponents/BP_CarryComponent.BP_CarryComponent_C") (`|CreateDelegate` :!event `RefreshScanPrompt`)))

(fn `ConfigureItem`
  (params (Product :type "/Game/GrandOpening/Blueprints/DataAssets/Products/BP_ProductDataAsset Object Reference") (Checkout :type "/Game/GrandOpening/Blueprints/Environments/Checkout/BP_CheckoutBase Object Reference") (LateralOffsetCm :type "Float (double-precision)"))
  ;[1 1 1 0.8] Configure item
  (set `self.Product` Product)
  (set `self.Checkout` Checkout)
  (set `self.LateralOffsetCm` LateralOffsetCm)
  (`StaticMeshComponent.SetStaticMesh` (`self.Mesh`) (`/Game/GrandOpening/Blueprints/DataAssets/Products/BP_ProductDataAsset.Mesh` Product))
  (`self.RefreshScanPrompt`))

(fn `RefreshScanPrompt`
  (bind _checkout (`self.Checkout`))
  ;[1 1 1 0.8] Refresh scan prompt - only interactable if the scanner is in hand and it's the right scanner of the current checkout
  (bind _manned (`/Game/GrandOpening/Blueprints/Environments/Checkout/BP_CheckoutBase.IsManned` _checkout))
  (`/Game/GrandOpening/Blueprints/ActorComponents/BP_InteractableComponent.SetInteractable` (`self.BP_InteractableComponent`) (and (== (`/Game/GrandOpening/Blueprints/ActorComponents/BP_CarryComponent.CarriedActor` (`self.GetComponentByClass` (`GameplayStatics.GetPlayerCharacter` 0) "/Game/GrandOpening/Blueprints/ActorComponents/BP_CarryComponent.BP_CarryComponent_C")) (`/Game/GrandOpening/Blueprints/Environments/Checkout/BP_CheckoutBase.PairedScanner` _checkout)) (not _manned))))

(fn `UserConstructionScript`)
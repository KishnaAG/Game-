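; BP_DrawerMoney is a money piece in the checkout cash drawer, representing a single denomination.
; Its construction script applies the configured mesh and sets the interactable's label to the denomination formatted as a dollar amount.
; When the interactable component is used, it broadcasts OnTaken with itself, leaving the handling to listeners.
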(event `self.BP_InteractableComponent.OnInteracted`
  (params (Interactor :type "Actor Object Reference"))
  ;[1 1 1 0.8] On interacted
  (`self.OnTaken` self))

(fn `UserConstructionScript`
  ;[1 1 1 0.8] Construction script
  (`StaticMeshComponent.SetStaticMesh` (`self.MoneyMesh`) (`self.Mesh`))
  (set `/Game/GrandOpening/Blueprints/ActorComponents/BP_InteractableComponent.Label` (`|FormatText` "${Amount}" (`KismetTextLibrary.Conv_DoubleToText` (`self.Denomination`) "HalfToEven" false true 1 324 2 2)) (`self.BP_InteractableComponent`)))
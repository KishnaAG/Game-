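; Checkout counter pile of one money denomination that grows as units arrive and hands them back to the drawer when interacted with.
; Configure sets the mesh, material and value; units travel as spawned BP_ProductFlight actors and stack vertically as mesh instances.
; Count changes when a flight launches, updating the prompt label, and interaction passes the pile to the owning BP_CheckoutBase, staying enabled only while units remain.
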(event `self.BP_InteractableComponent.OnInteracted`
  (params (Interactor :type "Actor Object Reference"))
  ;[1 1 1 0.8] On interacted
  (bind _asbp_checkout_base (cast `/Game/GrandOpening/Blueprints/Environments/Checkout/BP_CheckoutBase` (`self.GetOwner`)))
  (`/Game/GrandOpening/Blueprints/Environments/Checkout/BP_CheckoutBase.ReturnToDrawer` _asbp_checkout_base self)
  (`/Game/GrandOpening/Blueprints/ActorComponents/BP_InteractableComponent.SetInteractable` (`self.BP_InteractableComponent`) (> (`self.Count`) 0))
  (`/Game/GrandOpening/Blueprints/ActorComponents/BP_InteractionComponent.RefreshPrompt` (`self.GetComponentByClass` Interactor "/Game/GrandOpening/Blueprints/ActorComponents/BP_InteractionComponent.BP_InteractionComponent_C")))

(fn `AddUnit`
  (bind _moneystack (`self.MoneyStack`))
  (bind (_min _max) (`StaticMeshComponent.GetLocalBounds` _moneystack))
  ;[1 1 1 0.8] Add unit
  (`InstancedStaticMeshComponent.AddInstance` _moneystack (`KismetMathLibrary.MakeTransform` (`KismetMathLibrary.MakeVector` 0.0 0.0 (* (`InstancedStaticMeshComponent.GetInstanceCount` _moneystack) (.z (- _max _min))))) false))

(fn `Configure`
  (params (UnitMesh :type "StaticMesh Object Reference") (UnitMaterial :type "MaterialInterface Object Reference") (Value :type "Float (double-precision)"))
  (bind _moneystack (`self.MoneyStack`))
  ;[1 1 1 0.8] Configure
  (`StaticMeshComponent.SetStaticMesh` _moneystack UnitMesh)
  (`PrimitiveComponent.SetMaterial` _moneystack 0 UnitMaterial)
  (set `self.Denomination` Value))

(fn `ReceiveUnit`
  (params (From :type "SceneComponent Object Reference"))
  (bind _moneystack (`self.MoneyStack`))
  (bind (_min _max) (`StaticMeshComponent.GetLocalBounds` _moneystack))
  ;[1 1 1 0.8] Receive unit
  (bind _returnvalue (`|SpawnActorFromClass` "/Game/GrandOpening/Blueprints/Misc/BP_ProductFlight.BP_ProductFlight_C" (`SceneComponent.K2_GetComponentToWorld` From) "Undefined" "MultiplyWithRoot" self null))
  (add `/Game/GrandOpening/Blueprints/Misc/BP_ProductFlight.OnArrived` _returnvalue (`|CreateDelegate` :!event `AddUnit`))
  (`/Game/GrandOpening/Blueprints/Misc/BP_ProductFlight.Launch` _returnvalue (`StaticMeshComponent.StaticMesh` _moneystack) _moneystack (`KismetMathLibrary.MakeTransform` (`KismetMathLibrary.MakeVector` 0.0 0.0 (* (`self.Count`) (.z (- _max _min))))) 0.0 0.0)
  (`PrimitiveComponent.SetMaterial` (`/Game/GrandOpening/Blueprints/Misc/BP_ProductFlight.UnitMesh` _returnvalue) 0 (`PrimitiveComponent.GetMaterial` _moneystack 0))
  (set `self.Count` (+ (`self.Count`) 1))
  (`self.RefreshLabel`)
  (`/Game/GrandOpening/Blueprints/ActorComponents/BP_InteractableComponent.SetInteractable` (`self.BP_InteractableComponent`) true))

(fn `RefreshLabel`
  ;[1 1 1 0.8] Refresh label
  (set `/Game/GrandOpening/Blueprints/ActorComponents/BP_InteractableComponent.Label` (`|FormatText` "${Amount} x{Count}" (`KismetTextLibrary.Conv_DoubleToText` (`self.Denomination`) "HalfToEven" false true 1 324 2 2) (`KismetTextLibrary.Conv_IntToText` (`self.Count`))) (`self.BP_InteractableComponent`)))

(fn `ReturnUnit`
  (params (To :type "SceneComponent Object Reference"))
  (bind _moneystack (`self.MoneyStack`))
  (bind _returnvalue (- (`InstancedStaticMeshComponent.GetInstanceCount` _moneystack) 1))
  ;[1 1 1 0.8] Return unit
  (bind _returnvalue_2 (`|SpawnActorFromClass` "/Game/GrandOpening/Blueprints/Misc/BP_ProductFlight.BP_ProductFlight_C" (`InstancedStaticMeshComponent.GetInstanceTransform` _moneystack _returnvalue true) "Undefined" "MultiplyWithRoot" self null))
  (`/Game/GrandOpening/Blueprints/Misc/BP_ProductFlight.Launch` _returnvalue_2 (`StaticMeshComponent.StaticMesh` _moneystack) To (`KismetMathLibrary.MakeTransform` (0.0 0.0 0.0)) 0.0 0.0)
  (`PrimitiveComponent.SetMaterial` (`/Game/GrandOpening/Blueprints/Misc/BP_ProductFlight.UnitMesh` _returnvalue_2) 0 (`PrimitiveComponent.GetMaterial` _moneystack 0))
  (`InstancedStaticMeshComponent.RemoveInstance` _moneystack _returnvalue)
  (set `self.Count` (- (`self.Count`) 1))
  (`self.RefreshLabel`))

(fn `UserConstructionScript`)
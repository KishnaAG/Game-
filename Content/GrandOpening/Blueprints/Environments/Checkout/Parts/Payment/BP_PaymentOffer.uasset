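; BP_PaymentOffer is the card or cash payment that appears at the checkout for the player to take.
; It starts withdrawn, meaning hidden, without collision and non-interactable.
; OfferCard and OfferCash call MakeOffer, which swaps the body mesh, material and interaction label, then reveals and enables the actor.
; Interacting fires OnTaken but leaves the offer visible until Withdraw is called.
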(event `self.ReceiveBeginPlay`
  ;[1 1 1 0.8] Event begin play
  (`self.Withdraw` self))

(event `self.BP_InteractableComponent.OnInteracted`
  (params (Interactor :type "Actor Object Reference"))
  ;[1 1 1 0.8] On interacted
  (`self.OnTaken`))

(fn `MakeOffer`
  (params (Mesh :type "StaticMesh Object Reference") (Material :type "MaterialInterface Object Reference") (Label :type Text))
  (bind _bodymesh (`self.BodyMesh`))
  ;[1 1 1 0.8] Make offer
  (`StaticMeshComponent.SetStaticMesh` _bodymesh Mesh)
  (`PrimitiveComponent.SetMaterial` _bodymesh 0 Material)
  (set `/Game/GrandOpening/Blueprints/ActorComponents/BP_InteractableComponent.Label` Label (`self.BP_InteractableComponent`))
  (`self.SetActorHiddenInGame` self false)
  (`self.SetActorEnableCollision` self true)
  (`/Game/GrandOpening/Blueprints/ActorComponents/BP_InteractableComponent.SetInteractable` (`self.BP_InteractableComponent`) true))

(fn `OfferCard`
  ;[1 1 1 0.8] Offer card
  (`self.MakeOffer` self (`self.CardMesh`) (`self.CardMaterial`) (`self.CardLabel`)))

(fn `OfferCash`
  ;[1 1 1 0.8] Offer cash
  (`self.MakeOffer` self (`self.CashMesh`) (`self.CashMaterial`) (`self.CashLabel`)))

(fn `UserConstructionScript`)

(fn `Withdraw`
  ;[1 1 1 0.8] Withdraw
  (`self.SetActorHiddenInGame` self true)
  (`self.SetActorEnableCollision` self false)
  (`/Game/GrandOpening/Blueprints/ActorComponents/BP_InteractableComponent.SetInteractable` (`self.BP_InteractableComponent`) false))
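; Base delivery box that holds units of one product for stocking shelves, and can be carried, opened, racked or binned.
; A size asset drives meshes and the interior storage row, and a timeline swings the flaps.
; While open, it trades single units with shelves through a spawned flight actor, one transfer at a time.
; It publishes a stock task to the store manager on begin play and hour changes unless empty or player-carried.
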(event `self.ReceiveEndPlay`
  (params (EndPlayReason :type "EEndPlayReason Enum" :default "Destroyed"))
  (bind _returnvalue (`self.GetComponentByClass` (`GameplayStatics.GetGameState`) "/Game/GrandOpening/Blueprints/ActorComponents/BP_StoreManager.BP_StoreManager_C"))
  ;[1 1 1 0.8] Event end play
  (`/Engine/EditorBlueprintResources/StandardMacros.IsValid` _returnvalue
    (:`Is Valid`
      (`/Game/GrandOpening/Blueprints/ActorComponents/BP_StoreManager.WithdrawTask` _returnvalue self))))

(event `self.ReceiveBeginPlay`
  (bind _returnvalue (`self.GetComponentByClass` (`GameplayStatics.GetGameState`) "/Game/GrandOpening/Blueprints/ActorComponents/BP_StoreManager.BP_StoreManager_C"))
  ;[1 1 1 0.8] Event begin play
  (`self.ConfigureContents` self)
  (`self.RefreshLabel` self)
  (`/Engine/EditorBlueprintResources/StandardMacros.IsValid` _returnvalue
    (:`Is Valid`
      (add `/Game/GrandOpening/Blueprints/ActorComponents/BP_StoreManager.OnHourChanged` _returnvalue (`|CreateDelegate` :!event `OnStoreHourChanged`))
      (`self.PublishStockTask`))))

(event `self.BP_InteractableComponent.OnInteracted`
  (params (Interactor :type "Actor Object Reference"))
  ;[1 1 1 0.8] On interacted
  (`self.PickUp` self Interactor))

(event `TransferArrived`
  (bind _product (`self.Product`))
  ;[1 1 1 0.8] Transfer arrived
  (if (`self.PendingIntoBox`)
    (`/Game/GrandOpening/Blueprints/ActorComponents/BP_StorageComponent.AddUnit` (`self.StorageComponent`) _product)
    (else
      (bind _asbp_shelf_base (cast `/Game/GrandOpening/Blueprints/Environments/Shelves/BP_ShelfBase` (`self.PendingTarget`)))
      (`/Game/GrandOpening/Blueprints/Environments/Shelves/BP_ShelfBase.PlaceProduct` _asbp_shelf_base _product 1)))
  (set `self.PendingTarget` null)
  (bind _asbp_store_character (cast `/Game/GrandOpening/Blueprints/PlayerCharacter/BP_StoreCharacter` (`GameplayStatics.GetPlayerCharacter` 0)))
  (`/Game/GrandOpening/Blueprints/PlayerCharacter/BP_StoreCharacter.RefreshCarriedActions` _asbp_store_character))

(event `ToggleOpen`
  (bind _open (`self.Open`))
  ;[1 1 1 0.8] Toggle open
  (set `self.Open` (not _open))
  (if _open
    (bind (_direction _open_2) (`Timeline|OpenClose` :!label _label)
      (:`Update`
        (`self.ApplyFlapAngle` _open_2)))
    (else
      (goto _label :!via `Reverse`))))

(fn `AddActionsTo`
  (params (Panel :type "/Game/GrandOpening/Blueprints/Widgets/Gameplay/BP_ActionsWidget Object Reference"))
  (bind _focustarget (`self.FocusTarget`))
  ;[1 1 1 0.8] Add actions to
  (`/Game/GrandOpening/Blueprints/Widgets/Gameplay/BP_ActionsWidget.SetProductIcon` Panel (`/Game/GrandOpening/Blueprints/DataAssets/Products/BP_ProductDataAsset.Icon` (`self.Product`)))
  (`/Game/GrandOpening/Blueprints/Widgets/Gameplay/BP_ActionsWidget.AddAction` Panel (`self.ToggleAction`) (`KismetMathLibrary.SelectText` (`self.CloseLabel`) (`self.OpenLabel`) (`self.Open`)))
  (bind _result (`self.CanUnloadInto` self _focustarget))
  (if _result
    (`/Game/GrandOpening/Blueprints/Widgets/Gameplay/BP_ActionsWidget.AddAction` Panel (`self.PlaceAction`) (`self.StockLabel`)))
  (bind _result_2 (`self.CanLoadFrom` self _focustarget))
  (if _result_2
    (`/Game/GrandOpening/Blueprints/Widgets/Gameplay/BP_ActionsWidget.AddAction` Panel (`self.TakeAction`) (`self.TakeLabel`)))
  (bind _candisposeinto (`self.CanDisposeInto` self _focustarget))
  (if _candisposeinto
    (`/Game/GrandOpening/Blueprints/Widgets/Gameplay/BP_ActionsWidget.AddAction` Panel (`self.DisposeAction`) (`self.DisposeLabel`)))
  (bind _canstore (`self.CanStoreInto` self (`self.FocusTarget`)))
  (if _canstore
    (`/Game/GrandOpening/Blueprints/Widgets/Gameplay/BP_ActionsWidget.AddAction` Panel (`self.StoreAction`) (`self.StoreLabel`))))

(fn `ApplyFlapAngle`
  (params (Alpha :type "Float (double-precision)"))
  (bind _returnvalue (* Alpha (`self.OpenDegrees`)))
  ;[1 1 1 0.8] Apply flap angle
  (`SceneComponent.K2_SetRelativeRotation` (`self.FlapFrontMesh`) (`KismetMathLibrary.MakeRotator` _returnvalue 0.0 180.0) false false)
  (`SceneComponent.K2_SetRelativeRotation` (`self.FlapBackMesh`) (`KismetMathLibrary.MakeRotator` _returnvalue) false false)
  (`self.ApplyOpenState` self Alpha))

(fn `ApplyOpenState`
  (params (Alpha :type "Float (double-precision)"))
  ;[1 1 1 0.8] Apply open state
  (`SceneComponent.SetVisibility` (`self.StorageComponent`) (> Alpha 0.0) true))

(fn `AttachBoxTo`
  (params (Carrier :type "SceneComponent Object Reference") (Socket :type Name) (HandOffsetCm :type "Vector Structure"))
  (bind _bodymesh (`self.BodyMesh`))
  (bind (_min _max) (`StaticMeshComponent.GetLocalBounds` _bodymesh))
  ;[1 1 1 0.8] Attach box to
  (`PrimitiveComponent.SetSimulatePhysics` _bodymesh false)
  (`self.SetActorEnableCollision` false)
  (`/Game/GrandOpening/Blueprints/ActorComponents/BP_InteractableComponent.SetInteractable` (`self.BP_InteractableComponent`) false)
  (`self.K2_AttachToComponent` Carrier Socket "SnapToTarget" "SnapToTarget" "KeepWorld")
  (`self.K2_SetActorRelativeLocation` (`KismetMathLibrary.NegateVector` (`KismetMathLibrary.MakeVector` (+ (.x _min) (.x HandOffsetCm)) (+ (.y _max) (.y HandOffsetCm)) (.z HandOffsetCm)))))

(fn `CanDisposeInto`
  (params (Target :type "Actor Object Reference"))
  (returns (CanDisposeInto :type Boolean))
  ;[1 1 1 0.8] Can dispose into
  (cast `/Game/GrandOpening/Blueprints/Environments/Misc/BP_TrashBin` Target
    (:`then`
      (return true))
    (:`CastFailed`
      (return false))))

(fn `CanLoadFrom`
  (params (Target :type "Actor Object Reference"))
  (returns (Result :type Boolean))
  (bind _product (`self.Product`))
  ;[1 1 1 0.8] Can load from
  (`/Engine/EditorBlueprintResources/StandardMacros.IsValid` _product
    (:`Is Valid`
      (bind _asbp_shelf_base (cast `/Game/GrandOpening/Blueprints/Environments/Shelves/BP_ShelfBase` Target)
        (:`then`
          (bind _hasunit (`/Game/GrandOpening/Blueprints/Environments/Shelves/BP_ShelfBase.HasUnitOf` _asbp_shelf_base _product))
          (bind _result (`self.HasRoom` self))
          (bind _accessible (`/Game/GrandOpening/Blueprints/Environments/Shelves/BP_ShelfBase.IsAccessible` _asbp_shelf_base))
          (return (and (`self.Open`) (and _hasunit _result) _accessible)))
        (:`CastFailed`
          (return false))))
    (:`Is Not Valid`
      (return false))))

(fn `CanStoreInto`
  (params (Target :type "Actor Object Reference"))
  (returns (CanStore :type Boolean))
  ;[1 1 1 0.8] Can store into
  (bind _asbp_storage_rack (cast `/Game/GrandOpening/Blueprints/Environments/Shelves/BP_StorageRack` Target)
    (:`then`
      (bind (_slot _found) (`/Game/GrandOpening/Blueprints/Environments/Shelves/BP_StorageRack.FindFreeSlotFor` _asbp_storage_rack self))
      (return _found))
    (:`CastFailed`
      (return false))))

(fn `CanUnloadInto`
  (params (Target :type "Actor Object Reference"))
  (returns (Result :type Boolean))
  (bind _product (`self.Product`))
  ;[1 1 1 0.8] Can unload into
  (`/Engine/EditorBlueprintResources/StandardMacros.IsValid` _product
    (:`Is Valid`
      (bind _asbp_shelf_base (cast `/Game/GrandOpening/Blueprints/Environments/Shelves/BP_ShelfBase` Target)
        (:`then`
          (bind _hasroom (`/Game/GrandOpening/Blueprints/Environments/Shelves/BP_ShelfBase.HasRoomFor` _asbp_shelf_base _product))
          (bind _result (`self.HasUnit` self))
          (bind _accessible (`/Game/GrandOpening/Blueprints/Environments/Shelves/BP_ShelfBase.IsAccessible` _asbp_shelf_base))
          (return (and (`self.Open`) (and _hasroom _result) _accessible)))
        (:`CastFailed`
          (return false))))
    (:`Is Not Valid`
      (return false))))

(fn `ConfigureContents`
  (bind _size (`self.Size`))
  (bind _product (`self.Product`))
  (bind _storagecomponent (`self.StorageComponent`))
  (bind _row_interior (`self.Row_Interior`))
  (bind _x (.x (`/Game/GrandOpening/Blueprints/DataAssets/Boxes/BP_BoxDataAsset.InteriorMinCm` _size)))
  (bind _y (.y (`/Game/GrandOpening/Blueprints/DataAssets/Boxes/BP_BoxDataAsset.InteriorMinCm` _size)))
  (bind _z (.z (`/Game/GrandOpening/Blueprints/DataAssets/Boxes/BP_BoxDataAsset.InteriorMinCm` _size)))
  ;[1 1 1 0.8] Configure contents
  (`/Engine/EditorBlueprintResources/StandardMacros.IsValid` _size
    (:`Is Valid`
      (set `/Game/GrandOpening/Blueprints/ActorComponents/BP_StorageRow.DepthCm` (.y (`/Game/GrandOpening/Blueprints/DataAssets/Boxes/BP_BoxDataAsset.InteriorSizeCm` _size)) _row_interior)
      (set `/Game/GrandOpening/Blueprints/ActorComponents/BP_StorageRow.ClearanceCm` (.z (`/Game/GrandOpening/Blueprints/DataAssets/Boxes/BP_BoxDataAsset.InteriorSizeCm` _size)) _row_interior)
      (`SplineComponent.ClearSplinePoints` _row_interior false)
      (`SplineComponent.AddSplinePoint` _row_interior (`KismetMathLibrary.MakeVector` _x _y _z) "Local" false)
      (`SplineComponent.AddSplinePoint` _row_interior (`KismetMathLibrary.MakeVector` (+ _x (.x (`/Game/GrandOpening/Blueprints/DataAssets/Boxes/BP_BoxDataAsset.InteriorSizeCm` _size))) _y _z) "Local" true)
      (`/Game/GrandOpening/Blueprints/ActorComponents/BP_StorageComponent.CollectRows` _storagecomponent)
      (`/Engine/EditorBlueprintResources/StandardMacros.IsValid` _product
        (:`Is Valid`
          (for _ (range (`self.InitialUnits`))
            (`/Game/GrandOpening/Blueprints/ActorComponents/BP_StorageComponent.AddUnit` _storagecomponent _product))
          (`self.ApplyOpenState` self 0.0))
        (:`Is Not Valid`
          (`self.ApplyOpenState` self 0.0))))))

(fn `DetachBoxFromCarrier`
  ;[1 1 1 0.8] Detach box from carrier
  (`self.K2_DetachFromActor` "KeepWorld" "KeepWorld" "KeepWorld")
  (`self.SetActorEnableCollision` true)
  (`PrimitiveComponent.SetSimulatePhysics` (`self.BodyMesh`) true)
  (`/Game/GrandOpening/Blueprints/ActorComponents/BP_InteractableComponent.SetInteractable` (`self.BP_InteractableComponent`) true))

(fn `FillDebugPanel`
  (params (Panel :type "/Game/GrandOpening/Blueprints/Widgets/Gameplay/BP_DebugPanelWidget Object Reference"))
  (returns (Filled :type Boolean))
  (bind _product (`self.Product`))
  ;[1 1 1 0.8] Fill debug panel
  (bind _units (`/Game/GrandOpening/Blueprints/ActorComponents/BP_StorageComponent.CountOf` (`self.StorageComponent`) _product))
  (`/Game/GrandOpening/Blueprints/Widgets/Gameplay/BP_DebugPanelWidget.AddRow` Panel "Product" (`KismetTextLibrary.Conv_StringToText` (`KismetSystemLibrary.GetDisplayName` _product)))
  (`/Game/GrandOpening/Blueprints/Widgets/Gameplay/BP_DebugPanelWidget.AddRow` Panel "Size" (`KismetTextLibrary.Conv_StringToText` (`KismetSystemLibrary.GetDisplayName` (`self.Size`))))
  (`/Game/GrandOpening/Blueprints/Widgets/Gameplay/BP_DebugPanelWidget.AddRow` Panel "Units" (`KismetTextLibrary.Conv_IntToText` _units))
  (`/Game/GrandOpening/Blueprints/Widgets/Gameplay/BP_DebugPanelWidget.AddRow` Panel "Open" (`KismetTextLibrary.Conv_BoolToText` (`self.Open`)))
  (`/Game/GrandOpening/Blueprints/Widgets/Gameplay/BP_DebugPanelWidget.AddRow` Panel "Pending target" (`KismetTextLibrary.Conv_StringToText` (`KismetSystemLibrary.GetDisplayName` (`self.PendingTarget`))))
  (return true))

(fn `GetCarryBody`
  (returns (Body :type "StaticMeshComponent Object Reference"))
  ;[1 1 1 0.8] Get carry body
  (return (`self.BodyMesh`)))

(fn `GetCarryOffset`
  (returns (Transform :type "Transform Structure"))
  ;[1 1 1 0.8] Get carry offset
  (return (`self.CarryOffset`)))

(fn `HasRoom`
  (returns (Result :type Boolean))
  ;[1 1 1 0.8] Has room
  (bind _hasroom (`/Game/GrandOpening/Blueprints/ActorComponents/BP_StorageComponent.HasRoomFor` (`self.StorageComponent`) (`self.Product`)))
  (return _hasroom))

(fn `HasUnit`
  (returns (Result :type Boolean))
  ;[1 1 1 0.8] Has unit
  (bind _hasunit (`/Game/GrandOpening/Blueprints/ActorComponents/BP_StorageComponent.HasUnitOf` (`self.StorageComponent`) (`self.Product`)))
  (return _hasunit))

(fn `IsBoxOpen`
  (returns (Open :type Boolean))
  ;[1 1 1 0.8] Is box open
  (return (`self.Open`)))

(fn `IsCarriedByPlayer`
  (returns (Carried :type Boolean))
  ;[1 1 1 0.8] Is carried by player
  (return (== (`/Game/GrandOpening/Blueprints/ActorComponents/BP_CarryComponent.CarriedActor` (`self.GetComponentByClass` (`GameplayStatics.GetPlayerCharacter` 0) "/Game/GrandOpening/Blueprints/ActorComponents/BP_CarryComponent.BP_CarryComponent_C")) self)))

(fn `IsTransferring`
  (returns (ReturnValue :type Boolean))
  ;[1 1 1 0.8] Is transferring
  (`/Engine/EditorBlueprintResources/StandardMacros.IsValid` (`self.PendingTarget`)
    (:`Is Valid`
      (return true))
    (:`Is Not Valid`
      (return false))))

(fn `LaunchFlight`
  (params (Start :type "Transform Structure") (TargetRoot :type "SceneComponent Object Reference") (TargetLocal :type "Transform Structure") (StartClearanceCm :type "Float (double-precision)") (TargetClearanceCm :type "Float (double-precision)"))
  ;[1 1 1 0.8] Launch flight
  (bind _returnvalue (`|SpawnActorFromClass` (`self.FlightClass`) Start "Undefined" "MultiplyWithRoot" null null))
  (add `/Game/GrandOpening/Blueprints/Misc/BP_ProductFlight.OnArrived` _returnvalue (`|CreateDelegate` :!event `TransferArrived`))
  (`/Game/GrandOpening/Blueprints/Misc/BP_ProductFlight.Launch` _returnvalue (`/Game/GrandOpening/Blueprints/DataAssets/Products/BP_ProductDataAsset.Mesh` (`self.Product`)) TargetRoot TargetLocal StartClearanceCm TargetClearanceCm))

(fn `LeftGripPoint`
  (params (HandOffsetCm :type "Vector Structure"))
  (returns (Point :type "Vector Structure"))
  (bind _bodymesh (`self.BodyMesh`))
  (bind (_min _max) (`StaticMeshComponent.GetLocalBounds` _bodymesh))
  ;[1 1 1 0.8] Left grip point
  (return (`KismetMathLibrary.TransformLocation` (`SceneComponent.K2_GetComponentToWorld` _bodymesh) (`KismetMathLibrary.MakeVector` (+ (.x _min) (.x HandOffsetCm)) (- 0.0 (+ (.y _max) (.y HandOffsetCm))) (.z HandOffsetCm)))))

(fn `LoadOneFrom`
  (params (Target :type "Actor Object Reference"))
  (returns (Result :type Boolean))
  (bind _product (`self.Product`))
  (bind _storagecomponent (`self.StorageComponent`))
  ;[1 1 1 0.8] Load one from
  (bind _result (`self.CanLoadFrom` self Target))
  (bind _returnvalue (`self.IsTransferring` self))
  (if (or (not _result) _returnvalue)
    (return false)
    (else
      (bind _asbp_shelf_base (cast `/Game/GrandOpening/Blueprints/Environments/Shelves/BP_ShelfBase` Target)
        (:`then`
          (bind _placement (`/Game/GrandOpening/Blueprints/Environments/Shelves/BP_ShelfBase.TopUnitTransform` _asbp_shelf_base _product))
          (bind _placement_2 (`self.NextUnitTransform` self))
          (`/Game/GrandOpening/Blueprints/Environments/Shelves/BP_ShelfBase.TakeOneOf` _asbp_shelf_base _product)
          (set `self.PendingTarget` Target)
          (set `self.PendingIntoBox` true)
          (`self.LaunchFlight` self _placement _storagecomponent (`KismetMathLibrary.MakeRelativeTransform` _placement_2 (`SceneComponent.K2_GetComponentToWorld` _storagecomponent)) 0.0 (.z (`/Game/GrandOpening/Blueprints/DataAssets/Boxes/BP_BoxDataAsset.InteriorSizeCm` (`self.Size`))))
          (return true))
        (:`CastFailed`
          (return false))))))

(fn `NextUnitTransform`
  (returns (Placement :type "Transform Structure"))
  ;[1 1 1 0.8] Next unit transform
  (bind _placement (`/Game/GrandOpening/Blueprints/ActorComponents/BP_StorageComponent.NextUnitTransform` (`self.StorageComponent`) (`self.Product`)))
  (return _placement))

(fn `OnStoreHourChanged`
  (params (Day :type Integer) (Hour :type Integer))
  ;[1 1 1 0.8] On store hour changed
  (`self.PublishStockTask`))

(fn `PickUp`
  (params (Interactor :type "Actor Object Reference"))
  ;[1 1 1 0.8] Pick up
  (bind _asbp_store_character (cast `/Game/GrandOpening/Blueprints/PlayerCharacter/BP_StoreCharacter` Interactor))
  (`/Game/GrandOpening/Blueprints/PlayerCharacter/BP_StoreCharacter.CarryObject` _asbp_store_character self))

(fn `PlaceBoxInSlot`
  (params (Slot :type "Transform Structure"))
  ;[1 1 1 0.8] Place box in slot
  (`self.K2_DetachFromActor` "KeepWorld" "KeepWorld" "KeepWorld")
  (`self.K2_SetActorLocation` (.location Slot))
  (`self.K2_SetActorRotation` (.rotation Slot) true)
  (`self.SetActorEnableCollision` true)
  (`PrimitiveComponent.SetSimulatePhysics` (`self.BodyMesh`) false)
  (`/Game/GrandOpening/Blueprints/ActorComponents/BP_InteractableComponent.SetInteractable` (`self.BP_InteractableComponent`) true))

(fn `PublishStockTask`
  ;[1 1 1 0.8] Publish stock task
  (bind _carried (`self.IsCarriedByPlayer`))
  (bind _result (`self.HasUnit` self))
  (if (and _result (not _carried))
    (`/Game/GrandOpening/Blueprints/ActorComponents/BP_StoreManager.PublishTask` (`self.GetComponentByClass` (`GameplayStatics.GetGameState`) "/Game/GrandOpening/Blueprints/ActorComponents/BP_StoreManager.BP_StoreManager_C") "NewEnumerator4" self 5)))

(fn `RefreshLabel`
  (bind _product (`self.Product`))
  (bind _returnvalue (`WidgetComponent.GetUserWidgetObject` (`self.LabelScene`)))
  ;[1 1 1 0.8] Refresh label
  (`/Engine/EditorBlueprintResources/StandardMacros.IsValid` _returnvalue
    (:`Is Valid`
      (`/Engine/EditorBlueprintResources/StandardMacros.IsValid` _product
        (:`Is Valid`
          (bind _asbp_box_label_widget (cast `/Game/GrandOpening/Blueprints/Widgets/World/BP_BoxLabelWidget` _returnvalue))
          (`/Game/GrandOpening/Blueprints/Widgets/World/BP_BoxLabelWidget.SetProductIcon` _asbp_box_label_widget (`/Game/GrandOpening/Blueprints/DataAssets/Products/BP_ProductDataAsset.Icon` _product)))))))

(fn `SetFocusTarget`
  (params (Target :type "Actor Object Reference"))
  ;[1 1 1 0.8] Set focus target
  (set `self.FocusTarget` Target))

(fn `TopUnitTransform`
  (returns (Placement :type "Transform Structure"))
  ;[1 1 1 0.8] Top unit transform
  (bind _placement (`/Game/GrandOpening/Blueprints/ActorComponents/BP_StorageComponent.TopUnitTransform` (`self.StorageComponent`) (`self.Product`)))
  (return _placement))

(fn `UnloadOneInto`
  (params (Target :type "Actor Object Reference"))
  (returns (Result :type Boolean))
  (bind _product (`self.Product`))
  ;[1 1 1 0.8] Unload one into
  (bind _result (`self.CanUnloadInto` self Target))
  (bind _returnvalue (`self.IsTransferring` self))
  (if (or (not _result) _returnvalue)
    (return false)
    (else
      (bind _asbp_shelf_base (cast `/Game/GrandOpening/Blueprints/Environments/Shelves/BP_ShelfBase` Target)
        (:`then`
          (bind _placement (`self.TopUnitTransform` self))
          (bind _placement_2 (`/Game/GrandOpening/Blueprints/Environments/Shelves/BP_ShelfBase.NextUnitTransform` _asbp_shelf_base _product))
          (`/Game/GrandOpening/Blueprints/ActorComponents/BP_StorageComponent.RemoveUnit` (`self.StorageComponent`) _product)
          (set `self.PendingTarget` Target)
          (set `self.PendingIntoBox` false)
          (bind _storagecomponent (`/Game/GrandOpening/Blueprints/Environments/Shelves/BP_ShelfBase.StorageComponent` _asbp_shelf_base))
          (`self.LaunchFlight` self _placement _storagecomponent (`KismetMathLibrary.MakeRelativeTransform` _placement_2 (`SceneComponent.K2_GetComponentToWorld` _storagecomponent)) (.z (`/Game/GrandOpening/Blueprints/DataAssets/Boxes/BP_BoxDataAsset.InteriorSizeCm` (`self.Size`))) 0.0)
          (return true))
        (:`CastFailed`
          (return false))))))

(fn `UserConstructionScript`
  (bind _size (`self.Size`))
  (bind _flapfrontmesh (`self.FlapFrontMesh`))
  (bind _flapbackmesh (`self.FlapBackMesh`))
  (bind _flaphingeycm (`/Game/GrandOpening/Blueprints/DataAssets/Boxes/BP_BoxDataAsset.FlapHingeYCm` _size))
  (bind _flaphingezcm (`/Game/GrandOpening/Blueprints/DataAssets/Boxes/BP_BoxDataAsset.FlapHingeZCm` _size))
  ;[1 1 1 0.8] Construction script
  (`/Engine/EditorBlueprintResources/StandardMacros.IsValid` _size
    (:`Is Valid`
      (`StaticMeshComponent.SetStaticMesh` (`self.BodyMesh`) (`/Game/GrandOpening/Blueprints/DataAssets/Boxes/BP_BoxDataAsset.BodyMesh` _size))
      (`StaticMeshComponent.SetStaticMesh` _flapfrontmesh (`/Game/GrandOpening/Blueprints/DataAssets/Boxes/BP_BoxDataAsset.FlapLabelMesh` _size))
      (`StaticMeshComponent.SetStaticMesh` _flapbackmesh (`/Game/GrandOpening/Blueprints/DataAssets/Boxes/BP_BoxDataAsset.FlapMesh` _size))
      (`SceneComponent.K2_SetRelativeLocation` _flapfrontmesh (`KismetMathLibrary.MakeVector` 0.0 (- 0.0 _flaphingeycm) _flaphingezcm) false false)
      (`SceneComponent.K2_SetRelativeLocation` _flapbackmesh (`KismetMathLibrary.MakeVector` 0.0 _flaphingeycm _flaphingezcm) false false))))
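; BP_StreetLamp is an environment street lamp that switches itself on at night and off by day, following the store's in-game clock.
; On begin play it gets BP_StoreManager from the game state, applies the current hour and binds to its hour-changed event.
; A night window spanning midnight drives SetOn, which toggles the light and the mesh's emissive material parameter.
; The construction script also calls SetOn to apply the IsOn state.
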(event `self.ReceiveBeginPlay`
  ;[1 1 1 0.8] Event begin play
  (set `self.StoreManager` (`self.GetComponentByClass` (`GameplayStatics.GetGameState`) "/Game/GrandOpening/Blueprints/ActorComponents/BP_StoreManager.BP_StoreManager_C"))
  (`/Engine/EditorBlueprintResources/StandardMacros.IsValid` (`self.StoreManager`)
    (:`Is Valid`
      (add `/Game/GrandOpening/Blueprints/ActorComponents/BP_StoreManager.OnHourChanged` (`self.StoreManager`) (`|CreateDelegate` :!event `OnHourChanged`))
      (`self.ApplyClock` (`/Game/GrandOpening/Blueprints/ActorComponents/BP_StoreManager.CurrentHour` (`self.StoreManager`))))))

(fn `ApplyClock`
  (params (Hour :type Integer))
  ;[1 1 1 0.8] Apply clock
  (`self.SetOn` (or (>= Hour (`self.NightStartHour`)) (< Hour (`self.NightEndHour`)))))

(fn `OnHourChanged`
  (params (Day :type Integer) (Hour :type Integer))
  ;[1 1 1 0.8] On hour changed
  (`self.ApplyClock` Hour))

(fn `SetOn`
  (params (NewOn :type Boolean))
  ;[1 1 1 0.8] Set on
  (set `self.IsOn` NewOn)
  (`SceneComponent.SetVisibility` (`self.LampLight`) NewOn false)
  (`MeshComponent.SetScalarParameterValueOnMaterials` (`self.LampMesh`) "EmissiveStrength" (select `bool` NewOn :`true` (`self.EmissiveOn`)))
  (`LightComponent.SetIntensity` (`self.LampLight`) (`self.LightIntensity`)))

(fn `UserConstructionScript`
  ;[1 1 1 0.8] Construction script
  (`self.SetOn` (`self.IsOn`)))
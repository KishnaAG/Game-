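; BP_CeilingDiffuser is a ceiling light fixture that can be switched on or off.
; A SetOn function stores the state, toggles the light component's visibility, applies the configured intensity, and sets the diffuser mesh's EmissiveStrength material parameter to match.
; The construction script calls SetOn with the IsOn variable, so the fixture reflects that setting in the editor.
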(fn `SetOn`
  (params (NewOn :type Boolean))
  ;[1 1 1 0.8] Set on
  (set `self.IsOn` NewOn)
  (`SceneComponent.SetVisibility` (`self.DiffuserLight`) NewOn false)
  (`MeshComponent.SetScalarParameterValueOnMaterials` (`self.DiffuserMesh`) "EmissiveStrength" (select `bool` NewOn :`true` (`self.EmissiveOn`)))
  (`LightComponent.SetIntensity` (`self.DiffuserLight`) (`self.LightIntensity`)))

(fn `UserConstructionScript`
  ;[1 1 1 0.8] Set on
  (`self.SetOn` (`self.IsOn`)))
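; BP_LightSwitch is an interactable wall switch that turns a set of linked lights on and off.
; Interaction through its BP_InteractableComponent toggles the state and plays an attached toggle sound.
; SetState stores the state, tilts the toggle mesh either way and calls SetOn on each valid light in the Lights array.
; The construction script applies the initial IsOn value, so mesh and lights match in the editor.
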(event `self.BP_InteractableComponent.OnInteracted`
  (params (Interactor :type "Actor Object Reference"))
  ;[1 1 1 0.8] On interacted
  (`self.Toggle`)
  (`GameplayStatics.SpawnSoundAttached` (`self.ToggleSound`) (`self.ToggleMesh`) "None" (0.0 0.0 0.0) (struct) "KeepRelativeOffset" false 0.5 1.0 0.0 null null))

(fn `SetState`
  (params (NewOn :type Boolean))
  (bind _toggletilt (`self.ToggleTilt`))
  ;[1 1 1 0.8] Set state
  (set `self.IsOn` NewOn)
  (`SceneComponent.K2_SetRelativeRotation` (`self.ToggleMesh`) (`KismetMathLibrary.MakeRotator` 0.0 (select `bool` NewOn :`false` (- 0.0 _toggletilt) :`true` _toggletilt)) false false)
  (for _array_element (`self.Lights`)
    (`/Engine/EditorBlueprintResources/StandardMacros.IsValid` _array_element
      (:`Is Valid`
        (`/Game/GrandOpening/Blueprints/Environments/Lights/BP_CeilingDiffuser.SetOn` _array_element NewOn)))))

(fn `Toggle`
  ;[1 1 1 0.8] Toggle
  (`self.SetState` (not (`self.IsOn`))))

(fn `UserConstructionScript`
  ;[1 1 1 0.8] Construction script
  (`self.SetState` (`self.IsOn`)))
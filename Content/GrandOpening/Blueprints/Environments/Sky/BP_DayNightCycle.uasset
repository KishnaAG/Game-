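; Day/night cycle actor that rotates referenced Sun and Moon actors to match the store's clock.
; BeginPlay fetches BP_StoreManager from the GameState and enables Tick once it, Sun and Moon are valid.
; Each Tick, ApplyTimeOfDay maps clock hours linearly across sunrise to sunset into pitch with fixed yaws, scaling the offset moon arc by peak elevation.
; The actor itself copies the Moon's rotation.
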(event `self.ReceiveBeginPlay`
  (bind _returnvalue (`self.GetComponentByClass` (`GameplayStatics.GetGameState`) "/Game/GrandOpening/Blueprints/ActorComponents/BP_StoreManager.BP_StoreManager_C"))
  ;[1 1 1 0.8] Event begin play
  (set `self.StoreManager` _returnvalue)
  (`/Engine/EditorBlueprintResources/StandardMacros.IsValid` _returnvalue
    (:`Is Valid`
      (`/Engine/EditorBlueprintResources/StandardMacros.IsValid` (`self.Sun`)
        (:`Is Valid`
          (`/Engine/EditorBlueprintResources/StandardMacros.IsValid` (`self.Moon`)
            (:`Is Valid`
              (`self.SetActorTickEnabled` self true))))))))

(event `self.ReceiveTick`
  (params (DeltaSeconds :type "Float (single-precision)"))
  ;[1 1 1 0.8] Event tick
  (bind _hours (`/Game/GrandOpening/Blueprints/ActorComponents/BP_StoreManager.GetClockHours` (`self.StoreManager`)))
  (`self.ApplyTimeOfDay` _hours))

(fn `ApplyTimeOfDay`
  (params (Hours :type "Float (double-precision)"))
  (bind _sunrisehour (`self.SunriseHour`))
  (bind _returnvalue (* 180.0 (`KismetMathLibrary.SafeDivide` (- Hours _sunrisehour) (- (`self.SunsetHour`) _sunrisehour))))
  (bind _returnvalue_2 (`KismetMathLibrary.MakeRotator` 0.0 (* (- 180.0 _returnvalue) (`KismetMathLibrary.SafeDivide` (`self.MoonPeakElevation`) 90.0)) (`self.MoonYaw`)))
  ;[1 1 1 0.8] Apply time of day
  (`self.K2_SetActorRotation` (`self.Sun`) (`KismetMathLibrary.MakeRotator` 0.0 (- 0.0 _returnvalue) (`self.SunYaw`)) false)
  (`self.K2_SetActorRotation` (`self.Moon`) _returnvalue_2 false)
  (`self.K2_SetActorRotation` self _returnvalue_2 false))

(fn `UserConstructionScript`)
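; BP_BarcodeScanner is a physical handheld barcode scanner tool that a store character picks up through interaction and that docks in a cradle.
; DockTo stores the cradle transform, and ReturnToCradle zeroes velocity and teleports the scanner back there.
; AttachToHand releases it from the player's carry component, then snaps it to a socket with physics and collision off; ReleaseFromHand restores both and re-docks.
; It also supplies a camera-pitched carry offset and an attached beep sound.
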(event `self.BP_InteractableComponent.OnInteracted`
  (params (Interactor :type "Actor Object Reference"))
  ;[1 1 1 0.8] On interacted
  (`self.PickUp` self Interactor))

(fn `AttachToHand`
  (params (Hand :type "SceneComponent Object Reference") (Socket :type Name))
  (bind _returnvalue (`self.GetComponentByClass` (`GameplayStatics.GetPlayerCharacter` 0) "/Game/GrandOpening/Blueprints/ActorComponents/BP_CarryComponent.BP_CarryComponent_C"))
  ;[1 1 1 0.8] Attach to hand
  (if (== (`/Game/GrandOpening/Blueprints/ActorComponents/BP_CarryComponent.CarriedActor` _returnvalue) self)
    (`/Game/GrandOpening/Blueprints/ActorComponents/BP_CarryComponent.ReleaseActor` _returnvalue))
  (`PrimitiveComponent.SetSimulatePhysics` (`self.BodyMesh`) false)
  (`self.SetActorEnableCollision` false)
  (`self.K2_AttachToComponent` self Hand Socket "SnapToTarget" "SnapToTarget" "KeepWorld" true))

(fn `DockTo`
  (params (Cradle :type "Transform Structure"))
  ;[1 1 1 0.8] Dock to
  (set `self.CradleTransform` Cradle)
  (`self.ReturnToCradle` self))

(fn `GetCarryBody`
  (returns (Body :type "StaticMeshComponent Object Reference"))
  ;[1 1 1 0.8] Get carry body
  (return (`self.BodyMesh`)))

(fn `GetCarryOffset`
  (returns (Transform :type "Transform Structure"))
  ;[1 1 1 0.8] Get carry offset
  (return (`KismetMathLibrary.MakeTransform` (`self.CarryOffsetCm`) (`KismetMathLibrary.MakeRotator` 0.0 (.pitch (`PlayerCameraManager.GetCameraRotation` (`GameplayStatics.GetPlayerCameraManager` 0)))))))

(fn `PickUp`
  (params (Interactor :type "Actor Object Reference"))
  ;[1 1 1 0.8] Pick up
  (bind _asbp_store_character (cast `/Game/GrandOpening/Blueprints/PlayerCharacter/BP_StoreCharacter` Interactor))
  (`/Game/GrandOpening/Blueprints/PlayerCharacter/BP_StoreCharacter.CarryObject` _asbp_store_character self))

(fn `PlayBeepSound`
  ;[1 1 1 0.8] Play beep sound
  (`GameplayStatics.SpawnSoundAttached` (`self.ScanSound`) (`self.BodyMesh`) "None" (0.0 0.0 0.0) (struct) "KeepRelativeOffset" false 1.0 1.0 0.0 null null))

(fn `ReleaseFromHand`
  ;[1 1 1 0.8] Release from hand
  (`self.K2_DetachFromActor` self "KeepWorld" "KeepWorld" "KeepWorld")
  (`self.SetActorEnableCollision` true)
  (`PrimitiveComponent.SetSimulatePhysics` (`self.BodyMesh`) true)
  (`self.ReturnToCradle` self))

(fn `ReturnToCradle`
  (bind _bodymesh (`self.BodyMesh`))
  ;[1 1 1 0.8] Return to cradle
  (`PrimitiveComponent.SetPhysicsLinearVelocity` _bodymesh (0.0 0.0 0.0) false "None")
  (`PrimitiveComponent.SetPhysicsAngularVelocityInDegrees` _bodymesh (0.0 0.0 0.0) false "None")
  (`self.K2_SetActorTransform` self (`self.CradleTransform`) false true))

(fn `UserConstructionScript`)
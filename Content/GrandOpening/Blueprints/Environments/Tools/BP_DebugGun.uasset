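; BP_DebugGun is a carryable tool that points a laser and shows debug info for the actor under the player's aim.
; Interacting hands it to BP_StoreCharacter to carry, which enables tick and the beam, with carry pitch following the camera.
; Each tick traces from the camera, then stretches the beam from muzzle to aim point.
; Hit actors fill the readout panel through FillDebugPanelMessage, whose return value sets its visibility.
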(event `self.ReceiveBeginPlay`
  ;[1 1 1 0.8] Event begin play
  (bind _returnvalue (`PrimitiveComponent.CreateDynamicMaterialInstance` (`self.BeamMesh`) 0 null "None"))
  (`MaterialInstanceDynamic.SetVectorParameterValue` _returnvalue "Color" (`self.LaserColor`)))

(event `self.ReceiveTick`
  (params (DeltaSeconds :type "Float (single-precision)"))
  ;[1 1 1 0.8] Event tick
  (`self.AdvanceLaser` self))

(event `self.BP_InteractableComponent.OnInteracted`
  (params (Interactor :type "Actor Object Reference"))
  ;[1 1 1 0.8] On interacted
  (`self.PickUp` self Interactor))

(event `/Game/GrandOpening/Blueprints/Interfaces/BPI_Carryable.OnCarriedChanged`
  (params (Carried :type Boolean))
  ;[1 1 1 0.8] Event on carried changed
  (`self.SetActorTickEnabled` self Carried)
  (`SceneComponent.SetVisibility` (`self.ReadoutWidget`) false false)
  (`SceneComponent.SetVisibility` (`self.BeamMesh`) Carried false))

(fn `AdvanceLaser`
  (bind _returnvalue (`GameplayStatics.GetPlayerCameraManager` 0))
  (bind _laserrangecm (`self.LaserRangeCm`))
  (bind _beammesh (`self.BeamMesh`))
  (bind _laserthicknesscm (`self.LaserThicknessCm`))
  (bind _readoutwidget (`self.ReadoutWidget`))
  (bind _returnvalue_2 (`PlayerCameraManager.GetCameraLocation` _returnvalue))
  (bind _returnvalue_3 (`SceneComponent.K2_GetComponentLocation` (`self.MuzzleScene`)))
  (bind _returnvalue_4 (`KismetMathLibrary.GetForwardVector` (`PlayerCameraManager.GetCameraRotation` _returnvalue)))
  ;[1 1 1 0.8] Advance laser
  (bind _outhit (`KismetSystemLibrary.LineTraceSingle` _returnvalue_2 (+ _returnvalue_2 (* _returnvalue_4 _laserrangecm)) "TraceTypeQuery2" false (`|MakeArray` (`GameplayStatics.GetPlayerPawn` 0) :!type "Actor Object Reference")))
  (bind (_bblockinghit _binitialoverlap _time _distance _location _impactpoint _normal _impactnormal _physmat _hitactor) (`GameplayStatics.BreakHitResult` _outhit))
  (bind _returnvalue_5 (+ _returnvalue_2 (* _returnvalue_4 (`KismetMathLibrary.SelectFloat` _distance _laserrangecm _bblockinghit))))
  (`SceneComponent.K2_SetWorldRotation` _beammesh (`KismetMathLibrary.FindLookAtRotation` _returnvalue_3 _returnvalue_5) false false)
  (`SceneComponent.SetRelativeScale3D` _beammesh (`KismetMathLibrary.MakeVector` (`KismetMathLibrary.Vector_Distance` _returnvalue_3 _returnvalue_5) _laserthicknesscm _laserthicknesscm))
  (bind _asbp_debug_panel_widget (cast `/Game/GrandOpening/Blueprints/Widgets/Gameplay/BP_DebugPanelWidget` (`WidgetComponent.GetUserWidgetObject` _readoutwidget)))
  (`/Engine/EditorBlueprintResources/StandardMacros.IsValid` _hitactor
    (:`Is Valid`
      (`/Game/GrandOpening/Blueprints/Widgets/Gameplay/BP_DebugPanelWidget.ClearRows` _asbp_debug_panel_widget)
      (`/Game/GrandOpening/Blueprints/Widgets/Gameplay/BP_DebugPanelWidget.SetTitle` _asbp_debug_panel_widget (`KismetTextLibrary.Conv_StringToText` (`KismetSystemLibrary.GetDisplayName` _hitactor)))
      (bind _filled (message `/Game/GrandOpening/Blueprints/Interfaces/BPI_DebugInspect.FillDebugPanel` _hitactor _asbp_debug_panel_widget))
      (`SceneComponent.SetVisibility` (`self.ReadoutWidget`) _filled false))
    (:`Is Not Valid`
      (`SceneComponent.SetVisibility` _readoutwidget false false))))

(fn `GetCarryBody`
  (returns (Body :type "StaticMeshComponent Object Reference"))
  ;[1 1 1 0.8] Get carry body
  (return (`self.BodyMesh`)))

(fn `GetCarryOffset`
  (returns (Transform :type "Transform Structure"))
  ;[1 1 1 0.8] Get carry offset
  (return (`KismetMathLibrary.MakeTransform` (`self.CarryOffsetCm`) (`KismetMathLibrary.MakeRotator` 0.0 (.pitch (`PlayerCameraManager.GetCameraRotation` (`GameplayStatics.GetPlayerCameraManager` 0)))))))

(fn `PickUp`
  (params (Interactor :type "Actor Object Reference"))
  ;[1 1 1 0.8] Pick up
  (bind _asbp_store_character (cast `/Game/GrandOpening/Blueprints/PlayerCharacter/BP_StoreCharacter` Interactor))
  (`/Game/GrandOpening/Blueprints/PlayerCharacter/BP_StoreCharacter.CarryObject` _asbp_store_character self))

(fn `UserConstructionScript`)
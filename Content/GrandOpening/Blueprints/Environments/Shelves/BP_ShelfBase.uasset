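; Base shelf actor that stores products and limits them to the categories its shelf type accepts.
; A storage component holds the rows and handles room checks, unit transforms, adding and removing; the shelf wraps it with a category filter and place and take functions.
; On BeginPlay it collects the rows and stocks an optional initial product.
; It also fills a debug panel with shelf type, row contents and accepted categories.
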(event `self.ReceiveBeginPlay`
  ;[1 1 1 0.8] Event begin play
  (`/Game/GrandOpening/Blueprints/ActorComponents/BP_StorageComponent.CollectRows` (`self.StorageComponent`))
  (`self.StockInitialProduct` self))

(fn `AcceptsProduct`
  (params (Product :type "/Game/GrandOpening/Blueprints/DataAssets/Products/BP_ProductDataAsset Object Reference"))
  (returns (Accepted :type Boolean))
  ;[1 1 1 0.8] Accepts product
  (return (`KismetArrayLibrary.Array_Contains` (`/Game/GrandOpening/Blueprints/DataAssets/Shelves/BP_ShelfTypeDataAsset.AcceptedCategories` (`self.ShelfType`)) (`/Game/GrandOpening/Blueprints/DataAssets/Products/BP_ProductDataAsset.Category` Product))))

(fn `FillDebugPanel`
  (params (Panel :type "/Game/GrandOpening/Blueprints/Widgets/Gameplay/BP_DebugPanelWidget Object Reference"))
  (returns (Filled :type Boolean))
  (bind _shelftype (`self.ShelfType`))
  (`/Game/GrandOpening/Blueprints/Widgets/Gameplay/BP_DebugPanelWidget.AddRow` Panel "Shelf type" (`KismetTextLibrary.Conv_StringToText` (`KismetSystemLibrary.GetDisplayName` _shelftype)))
  (for _array_element (`/Game/GrandOpening/Blueprints/ActorComponents/BP_StorageComponent.Rows` (`self.StorageComponent`))
    (bind _product (`/Game/GrandOpening/Blueprints/ActorComponents/BP_StorageRow.Product` _array_element))
    (`/Engine/EditorBlueprintResources/StandardMacros.IsValid` _product
      (:`Is Valid`
        (bind _returnvalue (`KismetTextLibrary.Conv_IntToText` (`/Game/GrandOpening/Blueprints/ActorComponents/BP_StorageRow.Count` _array_element)))
        (`/Game/GrandOpening/Blueprints/Widgets/Gameplay/BP_DebugPanelWidget.AddRow` Panel (`KismetTextLibrary.Conv_StringToText` (`KismetSystemLibrary.GetDisplayName` _product)) _returnvalue))
      (:`Is Not Valid`
        (`/Game/GrandOpening/Blueprints/Widgets/Gameplay/BP_DebugPanelWidget.AddRow` Panel "Empty row" _returnvalue))))
  (`/Engine/EditorBlueprintResources/StandardMacros.IsValid` _shelftype
    (:`Is Valid`
      (for _array_element_2 (`/Game/GrandOpening/Blueprints/DataAssets/Shelves/BP_ShelfTypeDataAsset.AcceptedCategories` _shelftype)
        (`/Game/GrandOpening/Blueprints/Widgets/Gameplay/BP_DebugPanelWidget.AddRow` Panel "Accepts" (`KismetTextLibrary.Conv_StringToText` (`|GetEnumeratorNameAsString` _array_element_2)))))
    (:`Is Not Valid`
      _))
  (return true))

(fn `HasRoomFor`
  (params (Product :type "/Game/GrandOpening/Blueprints/DataAssets/Products/BP_ProductDataAsset Object Reference"))
  (returns (HasRoom :type Boolean))
  ;[1 1 1 0.8] Has room for
  (bind _accepted (`self.AcceptsProduct` self Product))
  (if (not _accepted)
    (return false)
    (else
      (bind _hasroom (`/Game/GrandOpening/Blueprints/ActorComponents/BP_StorageComponent.HasRoomFor` (`self.StorageComponent`) Product))
      (return _hasroom))))

(fn `HasUnitOf`
  (params (Product :type "/Game/GrandOpening/Blueprints/DataAssets/Products/BP_ProductDataAsset Object Reference"))
  (returns (HasUnit :type Boolean))
  ;[1 1 1 0.8] Has unit of
  (bind _hasunit (`/Game/GrandOpening/Blueprints/ActorComponents/BP_StorageComponent.HasUnitOf` (`self.StorageComponent`) Product))
  (return _hasunit))

(fn `IsAccessible`
  (returns (Accessible :type Boolean))
  ;[1 1 1 0.8] Is accessible
  (return true))

(fn `NextUnitTransform`
  (params (Product :type "/Game/GrandOpening/Blueprints/DataAssets/Products/BP_ProductDataAsset Object Reference"))
  (returns (Placement :type "Transform Structure"))
  ;[1 1 1 0.8] Next unit transform
  (bind _placement (`/Game/GrandOpening/Blueprints/ActorComponents/BP_StorageComponent.NextUnitTransform` (`self.StorageComponent`) Product))
  (return _placement))

(fn `PlaceProduct`
  (params (Product :type "/Game/GrandOpening/Blueprints/DataAssets/Products/BP_ProductDataAsset Object Reference") (Count :type Integer))
  (returns (Placed :type Boolean))
  ;[1 1 1 0.8] Place product
  (for _ (range Count)
    (bind _hasroom (`self.HasRoomFor` self Product))
    (if (not _hasroom)
      (return false)
      (else
        (`/Game/GrandOpening/Blueprints/ActorComponents/BP_StorageComponent.AddUnit` (`self.StorageComponent`) Product))))
  (return true))

(fn `StockedProducts`
  (returns (Products :type "Array of /Game/GrandOpening/Blueprints/DataAssets/Products/BP_ProductDataAsset Object Reference"))
  ;[1 1 1 0.8] Stocked products
  (bind _products (`/Game/GrandOpening/Blueprints/ActorComponents/BP_StorageComponent.StockedProducts` (`self.StorageComponent`)))
  (return _products))

(fn `StockInitialProduct`
  (bind _initialproduct (`self.InitialProduct`))
  ;[1 1 1 0.8] Stock initial product
  (`/Engine/EditorBlueprintResources/StandardMacros.IsValid` _initialproduct
    (:`Is Valid`
      (`self.PlaceProduct` self _initialproduct (`self.InitialCount`)))))

(fn `TakeOneOf`
  (params (Product :type "/Game/GrandOpening/Blueprints/DataAssets/Products/BP_ProductDataAsset Object Reference"))
  (returns (Taken :type Boolean))
  (bind _storagecomponent (`self.StorageComponent`))
  ;[1 1 1 0.8] Has unit of
  (bind _hasunit (`/Game/GrandOpening/Blueprints/ActorComponents/BP_StorageComponent.HasUnitOf` _storagecomponent Product))
  (if (not _hasunit)
    (return false)
    (else
      (`/Game/GrandOpening/Blueprints/ActorComponents/BP_StorageComponent.RemoveUnit` _storagecomponent Product)
      (return true))))

(fn `TopUnitTransform`
  (params (Product :type "/Game/GrandOpening/Blueprints/DataAssets/Products/BP_ProductDataAsset Object Reference"))
  (returns (Placement :type "Transform Structure"))
  ;[1 1 1 0.8] Top unit transform
  (bind _placement (`/Game/GrandOpening/Blueprints/ActorComponents/BP_StorageComponent.TopUnitTransform` (`self.StorageComponent`) Product))
  (return _placement))

(fn `UserConstructionScript`
  ;[1 1 1 0.8] Construction script
  (`StaticMeshComponent.SetStaticMesh` (`self.Mesh`) (`self.ShelfMesh`)))
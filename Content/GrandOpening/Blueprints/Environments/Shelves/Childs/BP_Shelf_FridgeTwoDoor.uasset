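; BP_Shelf_FridgeTwoDoor is a shelf child Blueprint for a two-door fridge that the player opens and closes by interacting with it.
; Interaction flips DoorsOpen and eases both door components to mirrored yaw angles over a set time.
; Each toggle also swaps the open/close prompt label and refreshes the store character's carried-item actions.
; An IsAccessible function returns DoorsOpen, so the shelf reports as accessible only while the doors are open.
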(event `ToggleDoors`
  (bind _doorleft (`self.DoorLeft`))
  (bind _doorright (`self.DoorRight`))
  (bind _doorseconds (`self.DoorSeconds`))
  ;[1 1 1 0.8] Toggle doors
  (bind _output_get (set `self.DoorsOpen` (not (`self.DoorsOpen`))))
  (`self.RefreshDoorPrompt` self)
  (`|ExecutionSequence`
    (:`then_0`
      (bind _returnvalue (select `bool` _output_get :`true` (`self.OpenAngleDeg`)))
      (`KismetSystemLibrary.MoveComponentTo` _doorleft (`SceneComponent.RelativeLocation` _doorleft) (`KismetMathLibrary.MakeRotator` 0.0 0.0 (- 0.0 _returnvalue)) true true _doorseconds))
    (:`then_1`
      (`KismetSystemLibrary.MoveComponentTo` _doorright (`SceneComponent.RelativeLocation` _doorright) (`KismetMathLibrary.MakeRotator` 0.0 0.0 (+ 180.0 _returnvalue)) true true _doorseconds))))

(event `self.BP_InteractableComponent.OnInteracted`
  (params (Interactor :type "Actor Object Reference"))
  ;[1 1 1 0.8] On interacted
  (`self.ToggleDoors`))

(fn `IsAccessible`
  (returns (Accessible :type Boolean))
  ;[1 1 1 0.8] Is accessible
  (return (`self.DoorsOpen`)))

(fn `RefreshDoorPrompt`
  ;[1 1 1 0.8] Refresh door prompt
  (set `/Game/GrandOpening/Blueprints/ActorComponents/BP_InteractableComponent.Label` (`KismetMathLibrary.SelectText` (`self.CloseLabel`) (`self.OpenLabel`) (`self.DoorsOpen`)) (`self.BP_InteractableComponent`))
  (bind _asbp_store_character (cast `/Game/GrandOpening/Blueprints/PlayerCharacter/BP_StoreCharacter` (`GameplayStatics.GetPlayerCharacter` 0)))
  (`/Engine/EditorBlueprintResources/StandardMacros.IsValid` _asbp_store_character
    (:`Is Valid`
      (`/Game/GrandOpening/Blueprints/PlayerCharacter/BP_StoreCharacter.RefreshCarriedActions` _asbp_store_character))))

(fn `UserConstructionScript`
  (`parent.UserConstructionScript`))
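; BP_Shelf_Round is a round, tiered shelf whose storage rows are circular splines.
; Its construction script applies the shelf mesh, then has StorageComponent collect its row splines.
; Each row is rebuilt as an eight-point closed loop in local space, using that tier's radius and height.
; Only as many rows are rebuilt as both tier arrays have entries for.
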(fn `UserConstructionScript`
  (bind _storagecomponent (`self.StorageComponent`))
  (bind _tierradiuscm (`self.TierRadiusCm`))
  (bind _tierheightcm (`self.TierHeightCm`))
  (bind _rows (`/Game/GrandOpening/Blueprints/ActorComponents/BP_StorageComponent.Rows` _storagecomponent))
  ;[1 1 1 0.8] Construction script
  (`StaticMeshComponent.SetStaticMesh` (`self.Mesh`) (`self.ShelfMesh`))
  (`/Game/GrandOpening/Blueprints/ActorComponents/BP_StorageComponent.CollectRows` _storagecomponent)
  (for _index (range (`KismetMathLibrary.Min` (`KismetArrayLibrary.Array_Length` _rows) (`KismetMathLibrary.Min` (`KismetArrayLibrary.Array_Length` _tierradiuscm) (`KismetArrayLibrary.Array_Length` _tierheightcm))))
    (bind _output (`|GetArrayItem` _rows _index))
    (`SplineComponent.ClearSplinePoints` _output false)
    (for _index_2 (range 8)
      (bind _output_2 (`|GetArrayItem` _tierradiuscm _index))
      (bind _returnvalue (* 45.0 (`KismetMathLibrary.Conv_IntToDouble` _index_2)))
      (`SplineComponent.AddSplinePoint` _output (`KismetMathLibrary.MakeVector` (* _output_2 (`KismetMathLibrary.DegCos` _returnvalue)) (* _output_2 (`KismetMathLibrary.DegSin` _returnvalue)) (`|GetArrayItem` _tierheightcm _index)) "Local" false))
    (`SplineComponent.SetClosedLoop` _output true true)))
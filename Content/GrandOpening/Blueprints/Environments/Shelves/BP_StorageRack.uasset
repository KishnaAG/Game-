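; Storage rack that stores a carried delivery box in its first free slot when a store character interacts with it.
; Slot transforms form rows centered on the actor, computed from slots per level, pitch and level heights.
; A sphere overlap for other delivery boxes tests occupancy, so no slot bookkeeping is needed.
; The character places the box, then the rack aligns its rotation and turns off physics on its carry body.
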(event `self.BP_InteractableComponent.OnInteracted`
  (params (Interactor :type "Actor Object Reference"))
  ;[1 1 1 0.8] On interacted
  (bind _asbp_store_character (cast `/Game/GrandOpening/Blueprints/PlayerCharacter/BP_StoreCharacter` Interactor))
  (bind _box (`/Game/GrandOpening/Blueprints/PlayerCharacter/BP_StoreCharacter.GetCarriedBox` _asbp_store_character))
  (`/Engine/EditorBlueprintResources/StandardMacros.IsValid` _box
    (:`Is Valid`
      (bind (_slot _found) (`self.FindFreeSlotFor` self _box))
      (if _found
        (`/Game/GrandOpening/Blueprints/PlayerCharacter/BP_StoreCharacter.PlaceObject` _asbp_store_character (.location _slot))
        (`self.K2_SetActorRotation` _box (.rotation _slot) true)
        (bind _body (`/Game/GrandOpening/Blueprints/Interfaces/BPI_Carryable.GetCarryBody` _box))
        (`PrimitiveComponent.SetSimulatePhysics` _body false)))))

(fn `FindFreeSlotFor`
  (params (Box :type "/Game/GrandOpening/Blueprints/Environments/Boxes/BP_DeliveryBoxBase Object Reference"))
  (returns (Slot :type "Transform Structure") (Found :type Boolean))
  (locals (FreeSlot :type "Transform Structure") (SlotFound :type Boolean))
  ;[1 1 1 0.8] Find free slot for
  (for _index (range (* (`self.SlotsPerLevel`) (`KismetArrayLibrary.Array_Length` (`self.LevelHeightsCm`))))
    (bind _slot (`self.SlotTransform` self _index))
    (bind _free (`self.IsSlotFree` self _slot Box))
    (if _free
      (set `local.FreeSlot` _slot)
      (set `local.SlotFound` true)
      (break)))
  (return (`local.FreeSlot`) (`local.SlotFound`)))

(fn `IsSlotFree`
  (params (Slot :type "Transform Structure") (Box :type "/Game/GrandOpening/Blueprints/Environments/Boxes/BP_DeliveryBoxBase Object Reference"))
  (returns (Free :type Boolean))
  ;[1 1 1 0.8] Is slot free
  (bind (_outactors _returnvalue) (`KismetSystemLibrary.SphereOverlapActors` (.location Slot) (`self.SlotProbeCm`) (`|MakeArray` "ObjectTypeQuery4" :!type "EObjectTypeQuery Enum") "/Game/GrandOpening/Blueprints/Environments/Boxes/BP_DeliveryBoxBase.BP_DeliveryBoxBase_C" (`|MakeArray` Box :!type "Actor Object Reference")))
  (return (not _returnvalue)))

(fn `SlotTransform`
  (params (Index :type Integer))
  (returns (Slot :type "Transform Structure"))
  (bind _slotsperlevel (`self.SlotsPerLevel`))
  ;[1 1 1 0.8] Slot transform
  (return (`KismetMathLibrary.ComposeTransforms` (`KismetMathLibrary.MakeTransform` (`KismetMathLibrary.MakeVector` (* (- (`KismetMathLibrary.Conv_IntToDouble` (mod Index _slotsperlevel)) (* (`KismetMathLibrary.Conv_IntToDouble` (- _slotsperlevel 1)) 0.5)) (`self.SlotPitchCm`)) 0.0 (`|GetArrayItem` (`self.LevelHeightsCm`) (/ Index _slotsperlevel)))) (`self.GetTransform` self))))

(fn `UserConstructionScript`)
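; BP_Employee is the store employee actor, with its AI state held in BPEmployeeBrain.
; The only logic here fills a debug panel with the brain's candidate, task flag, manned checkout, target location and roam timer.
; It also shows the candidate's roles label, falling back to "None" when no valid candidate is set.
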(fn `FillDebugPanel`
  (params (Panel :type "/Game/GrandOpening/Blueprints/Widgets/Gameplay/BP_DebugPanelWidget Object Reference"))
  (returns (Filled :type Boolean))
  (bind _bp_employeebrain (`self.BP_EmployeeBrain`))
  (bind _candidate (`/Game/GrandOpening/Blueprints/ActorComponents/BP_EmployeeBrain.Candidate` _bp_employeebrain))
  ;[1 1 1 0.8] Fill debug panel
  (`/Game/GrandOpening/Blueprints/Widgets/Gameplay/BP_DebugPanelWidget.AddRow` Panel "Candidate" (`KismetTextLibrary.Conv_StringToText` (`KismetSystemLibrary.GetDisplayName` _candidate)))
  (`/Game/GrandOpening/Blueprints/Widgets/Gameplay/BP_DebugPanelWidget.AddRow` Panel "Has task" (`KismetTextLibrary.Conv_BoolToText` (`/Game/GrandOpening/Blueprints/ActorComponents/BP_EmployeeBrain.HasTask` _bp_employeebrain)))
  (`/Game/GrandOpening/Blueprints/Widgets/Gameplay/BP_DebugPanelWidget.AddRow` Panel "Manned checkout" (`KismetTextLibrary.Conv_StringToText` (`KismetSystemLibrary.GetDisplayName` (`/Game/GrandOpening/Blueprints/ActorComponents/BP_EmployeeBrain.MannedCheckout` _bp_employeebrain))))
  (`/Game/GrandOpening/Blueprints/Widgets/Gameplay/BP_DebugPanelWidget.AddRow` Panel "Target location" (`KismetTextLibrary.Conv_VectorToText` (`/Game/GrandOpening/Blueprints/ActorComponents/BP_EmployeeBrain.TargetLocation` _bp_employeebrain)))
  (`/Game/GrandOpening/Blueprints/Widgets/Gameplay/BP_DebugPanelWidget.AddRow` Panel "Roam until" (`KismetTextLibrary.Conv_DoubleToText` (`/Game/GrandOpening/Blueprints/ActorComponents/BP_EmployeeBrain.RoamUntil` _bp_employeebrain) "HalfToEven"))
  (`/Engine/EditorBlueprintResources/StandardMacros.IsValid` _candidate
    (:`Is Valid`
      (bind _label (`/Game/GrandOpening/Blueprints/DataAssets/Employees/BP_EmployeeCandidateDataAsset.RolesLabel` _candidate))
      (`/Game/GrandOpening/Blueprints/Widgets/Gameplay/BP_DebugPanelWidget.AddRow` Panel "Role" _label))
    (:`Is Not Valid`
      (`/Game/GrandOpening/Blueprints/Widgets/Gameplay/BP_DebugPanelWidget.AddRow` Panel "Role" "None")))
  (return true))

(fn `UserConstructionScript`)
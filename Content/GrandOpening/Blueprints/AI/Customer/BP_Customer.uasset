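; BP_Customer is the AI shopper Blueprint, with its shopping state held in BPCustomerBrain.
; Its construction script is empty; the only logic here fills a debug panel supplied by the caller.
; FillDebugPanel reads the brain's state, archetype, budget, basket count, patience and shelf and browsing targets into labelled rows, then returns true.
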(fn `FillDebugPanel`
  (params (Panel :type "/Game/GrandOpening/Blueprints/Widgets/Gameplay/BP_DebugPanelWidget Object Reference"))
  (returns (Filled :type Boolean))
  (bind _bp_customerbrain (`self.BP_CustomerBrain`))
  ;[1 1 1 0.8] Fill debug panel
  (`/Game/GrandOpening/Blueprints/Widgets/Gameplay/BP_DebugPanelWidget.AddRow` Panel "State" (`KismetTextLibrary.Conv_StringToText` (`|GetEnumeratorNameAsString` (`/Game/GrandOpening/Blueprints/ActorComponents/BP_CustomerBrain.State` _bp_customerbrain))))
  (`/Game/GrandOpening/Blueprints/Widgets/Gameplay/BP_DebugPanelWidget.AddRow` Panel "Archetype" (`KismetTextLibrary.Conv_StringToText` (`KismetSystemLibrary.GetDisplayName` (`/Game/GrandOpening/Blueprints/ActorComponents/BP_CustomerBrain.Archetype` _bp_customerbrain))))
  (`/Game/GrandOpening/Blueprints/Widgets/Gameplay/BP_DebugPanelWidget.AddRow` Panel "Budget" (`KismetTextLibrary.Conv_DoubleToText` (`/Game/GrandOpening/Blueprints/ActorComponents/BP_CustomerBrain.BudgetValue` _bp_customerbrain) "HalfToEven"))
  (`/Game/GrandOpening/Blueprints/Widgets/Gameplay/BP_DebugPanelWidget.AddRow` Panel "Target items" (`KismetTextLibrary.Conv_IntToText` (`/Game/GrandOpening/Blueprints/ActorComponents/BP_CustomerBrain.TargetItems` _bp_customerbrain)))
  (`/Game/GrandOpening/Blueprints/Widgets/Gameplay/BP_DebugPanelWidget.AddRow` Panel "Basket" (`KismetTextLibrary.Conv_IntToText` (`KismetArrayLibrary.Array_Length` (`/Game/GrandOpening/Blueprints/ActorComponents/BP_CustomerBrain.Basket` _bp_customerbrain))))
  (`/Game/GrandOpening/Blueprints/Widgets/Gameplay/BP_DebugPanelWidget.AddRow` Panel "Patience left" (`KismetTextLibrary.Conv_DoubleToText` (`/Game/GrandOpening/Blueprints/ActorComponents/BP_CustomerBrain.PatienceLeft` _bp_customerbrain) "HalfToEven"))
  (`/Game/GrandOpening/Blueprints/Widgets/Gameplay/BP_DebugPanelWidget.AddRow` Panel "Target shelf" (`KismetTextLibrary.Conv_StringToText` (`KismetSystemLibrary.GetDisplayName` (`/Game/GrandOpening/Blueprints/ActorComponents/BP_CustomerBrain.TargetShelf` _bp_customerbrain))))
  (`/Game/GrandOpening/Blueprints/Widgets/Gameplay/BP_DebugPanelWidget.AddRow` Panel "Target location" (`KismetTextLibrary.Conv_VectorToText` (`/Game/GrandOpening/Blueprints/ActorComponents/BP_CustomerBrain.TargetLocation` _bp_customerbrain)))
  (`/Game/GrandOpening/Blueprints/Widgets/Gameplay/BP_DebugPanelWidget.AddRow` Panel "Browse until" (`KismetTextLibrary.Conv_DoubleToText` (`/Game/GrandOpening/Blueprints/ActorComponents/BP_CustomerBrain.BrowseUntil` _bp_customerbrain) "HalfToEven"))
  (return true))

(fn `UserConstructionScript`)
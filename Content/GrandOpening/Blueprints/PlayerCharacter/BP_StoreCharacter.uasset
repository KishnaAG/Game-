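; Player character for a store game: moves, interacts, carries and throws objects, moves units between a carried delivery box and the focused actor, and forwards build input.
; Enhanced Input events delegate to interaction, carry, view motion and placement components.
; Carry and focus changes rebuild the action prompt widget; carrying also scales walk and sprint speed.
; View focus locks move and look input, blocks jump and crouch, and landing or crouching feeds camera motion.
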(event `self.BP_ViewMotionComponent.OnFocusBegan`
  ;[1 1 1 0.8] On focus began
  (`self.SetViewLocked` self true))

(event `self.BP_ViewMotionComponent.OnFocusEnded`
  ;[1 1 1 0.8] On focus ended
  (`self.SetViewLocked` self false))

(event `self.BP_InteractionComponent.OnFocusChanged`
  ;[1 1 1 0.8] On focus changed
  (`self.RefreshCarriedActions`))

(event `self.ReceiveBeginPlay`
  ;[1 1 1 0.8] Event begin play
  (bind _asplayer_controller (cast `PlayerController` (`self.GetController` self)))
  (`EnhancedInputSubsystemInterface.AddMappingContext` (pcsubsystem `EnhancedInputLocalPlayerSubsystem` _asplayer_controller) (`self.GameplayContext`) 0 (struct))
  (`self.RefreshWalkSpeed`))

(event `StopCrouching`
  ;[1 1 1 0.8] Stop crouching
  (`self.UnCrouch`))

(event `self.OnLanded`
  (params (Hit :type "HitResult Structure (by ref)"))
  ;[1 1 1 0.8] Event on landed
  (`/Game/GrandOpening/Blueprints/ActorComponents/BP_ViewMotionComponent.ApplyLandImpact` (`self.BP_ViewMotionComponent`) (.z (`self.GetVelocity` self))))

(event `self.K2_OnStartCrouch`
  (params (HalfHeightAdjust :type "Float (single-precision)") (ScaledHalfHeightAdjust :type "Float (single-precision)"))
  ;[1 1 1 0.8] Event on start crouch
  (`/Game/GrandOpening/Blueprints/ActorComponents/BP_ViewMotionComponent.AddCrouchTransition` (`self.BP_ViewMotionComponent`) ScaledHalfHeightAdjust))

(event `self.K2_OnEndCrouch`
  (params (HalfHeightAdjust :type "Float (single-precision)") (ScaledHalfHeightAdjust :type "Float (single-precision)"))
  ;[1 1 1 0.8] Event on end crouch
  (`/Game/GrandOpening/Blueprints/ActorComponents/BP_ViewMotionComponent.AddCrouchTransition` (`self.BP_ViewMotionComponent`) (- 0.0 ScaledHalfHeightAdjust)))

(event `self.BP_CarryComponent.OnCarryChanged`
  ;[1 1 1 0.8] On carry changed
  (`self.RefreshWalkSpeed`)
  (`self.RefreshCarriedActions`)
  (`/Game/GrandOpening/Blueprints/ActorComponents/BP_InteractionComponent.SetIgnored` (`self.BP_InteractionComponent`) (`/Game/GrandOpening/Blueprints/ActorComponents/BP_CarryComponent.CarriedActor` (`self.BP_CarryComponent`))))

(event `EnhancedInput|/Game/GrandOpening/Inputs/Inputs/IA_Interact`
  (params (ActionValue :type Boolean) (ElapsedSeconds :type "Float (double-precision)") (TriggeredSeconds :type "Float (double-precision)") (InputAction :type "InputAction Object Reference" :default "/Game/GrandOpening/Inputs/Inputs/IA_Interact.IA_Interact"))
  ;[0.3958 0.07014 0.1822 0.8] Inputs
  ;;[1 1 1 0.8] IA_Interact
  (:`Started`
    (`self.HandleInteractPressed`))
  (:`Completed`
    (`/Game/GrandOpening/Blueprints/ActorComponents/BP_InteractionComponent.EndInteract` (`self.BP_InteractionComponent`))))

(event `EnhancedInput|/Game/GrandOpening/Inputs/Inputs/IA_Move`
  (params (ActionValue :type "Vector2D Structure") (ElapsedSeconds :type "Float (double-precision)") (TriggeredSeconds :type "Float (double-precision)") (InputAction :type "InputAction Object Reference" :default "/Game/GrandOpening/Inputs/Inputs/IA_Move.IA_Move"))
  ;[0.3958 0.07014 0.1822 0.8] Inputs
  ;;[1 1 1 0.8] IA_Move
  (:`Triggered`
    (`self.MoveFromInput` ActionValue)))

(event `EnhancedInput|/Game/GrandOpening/Inputs/Inputs/IA_Look`
  (params (ActionValue :type "Vector2D Structure") (ElapsedSeconds :type "Float (double-precision)") (TriggeredSeconds :type "Float (double-precision)") (InputAction :type "InputAction Object Reference" :default "/Game/GrandOpening/Inputs/Inputs/IA_Look.IA_Look"))
  ;[0.3958 0.07014 0.1822 0.8] Inputs
  ;;[1 1 1 0.8] IA_Look
  (:`Triggered`
    (`self.LookFromInput` ActionValue)))

(event `EnhancedInput|/Game/GrandOpening/Inputs/Inputs/IA_Sprint`
  (params (ActionValue :type Boolean) (ElapsedSeconds :type "Float (double-precision)") (TriggeredSeconds :type "Float (double-precision)") (InputAction :type "InputAction Object Reference" :default "/Game/GrandOpening/Inputs/Inputs/IA_Sprint.IA_Sprint"))
  ;[0.3958 0.07014 0.1822 0.8] Inputs
  ;;[1 1 1 0.8] IA_Sprint
  (:`Started`
    (`self.ApplySprint` true))
  (:`Completed`
    (`self.ApplySprint` false)))

(event `EnhancedInput|/Game/GrandOpening/Inputs/Inputs/IA_ToggleBox`
  (params (ActionValue :type Boolean) (ElapsedSeconds :type "Float (double-precision)") (TriggeredSeconds :type "Float (double-precision)") (InputAction :type "InputAction Object Reference" :default "/Game/GrandOpening/Inputs/Inputs/IA_ToggleBox.IA_ToggleBox"))
  ;[0.3958 0.07014 0.1822 0.8] Inputs
  ;;[1 1 1 0.8] IA_ToggleBox
  (:`Started`
    (`self.ToggleCarriedOrFocusedBox`)))

(event `EnhancedInput|/Game/GrandOpening/Inputs/Inputs/IA_Jump`
  (params (ActionValue :type Boolean) (ElapsedSeconds :type "Float (double-precision)") (TriggeredSeconds :type "Float (double-precision)") (InputAction :type "InputAction Object Reference" :default "/Game/GrandOpening/Inputs/Inputs/IA_Jump.IA_Jump"))
  ;[0.3958 0.07014 0.1822 0.8] Inputs
  ;;[1 1 1 0.8] IA_Jump
  (:`Started`
    (if (not (`/Game/GrandOpening/Blueprints/ActorComponents/BP_ViewMotionComponent.Focusing` (`self.BP_ViewMotionComponent`)))
      (`self.Jump`)))
  (:`Completed`
    (`self.StopJumping`)))

(event `EnhancedInput|/Game/GrandOpening/Inputs/Inputs/IA_PlaceUnit`
  (params (ActionValue :type Boolean) (ElapsedSeconds :type "Float (double-precision)") (TriggeredSeconds :type "Float (double-precision)") (InputAction :type "InputAction Object Reference" :default "/Game/GrandOpening/Inputs/Inputs/IA_PlaceUnit.IA_PlaceUnit"))
  ;[0.3958 0.07014 0.1822 0.8] Inputs
  ;;[1 1 1 0.8] IA_PlaceUnit
  (:`Triggered`
    (`self.HandlePlaceUnit`)))

(event `EnhancedInput|/Game/GrandOpening/Inputs/Inputs/IA_TakeUnit`
  (params (ActionValue :type Boolean) (ElapsedSeconds :type "Float (double-precision)") (TriggeredSeconds :type "Float (double-precision)") (InputAction :type "InputAction Object Reference" :default "/Game/GrandOpening/Inputs/Inputs/IA_TakeUnit.IA_TakeUnit"))
  ;[0.3958 0.07014 0.1822 0.8] Inputs
  ;;[1 1 1 0.8] IA_TakeUnit
  (:`Triggered`
    (`self.HandleTakeUnit`)))

(event `EnhancedInput|/Game/GrandOpening/Inputs/Inputs/IA_ExitFocus`
  (params (ActionValue :type Boolean) (ElapsedSeconds :type "Float (double-precision)") (TriggeredSeconds :type "Float (double-precision)") (InputAction :type "InputAction Object Reference" :default "/Game/GrandOpening/Inputs/Inputs/IA_ExitFocus.IA_ExitFocus"))
  ;[0.3958 0.07014 0.1822 0.8] Inputs
  ;;[1 1 1 0.8] IA_ExitFocus
  (:`Started`
    (`self.HandleExitFocusPressed`)))

(event `EnhancedInput|/Game/GrandOpening/Inputs/Inputs/IA_Crouch`
  (params (ActionValue :type Boolean) (ElapsedSeconds :type "Float (double-precision)") (TriggeredSeconds :type "Float (double-precision)") (InputAction :type "InputAction Object Reference" :default "/Game/GrandOpening/Inputs/Inputs/IA_Crouch.IA_Crouch"))
  ;[0.3958 0.07014 0.1822 0.8] Inputs
  ;;[1 1 1 0.8] IA_Crouch
  (:`Started`
    (if (not (`/Game/GrandOpening/Blueprints/ActorComponents/BP_ViewMotionComponent.Focusing` (`self.BP_ViewMotionComponent`)))
      (`self.Crouch`)))
  (:`Completed`
    (if (not (`/Game/GrandOpening/Blueprints/ActorComponents/BP_ViewMotionComponent.Focusing` (`self.BP_ViewMotionComponent`)))
      (`self.StopCrouching`))))

(event `EnhancedInput|/Game/GrandOpening/Inputs/Inputs/IA_Drop`
  (params (ActionValue :type Boolean) (ElapsedSeconds :type "Float (double-precision)") (TriggeredSeconds :type "Float (double-precision)") (InputAction :type "InputAction Object Reference" :default "/Game/GrandOpening/Inputs/Inputs/IA_Drop.IA_Drop"))
  ;[0.3958 0.07014 0.1822 0.8] Inputs
  ;;[1 1 1 0.8] IA_Drop
  (:`Started`
    (`self.HandleDrop`)))

(event `EnhancedInput|/Game/GrandOpening/Inputs/Inputs/IA_RotateStructure`
  (params (ActionValue :type Boolean) (ElapsedSeconds :type "Float (double-precision)") (TriggeredSeconds :type "Float (double-precision)") (InputAction :type "InputAction Object Reference" :default "/Game/GrandOpening/Inputs/Inputs/IA_RotateStructure.IA_RotateStructure"))
  ;[0.3958 0.07014 0.1822 0.8] Inputs
  ;;[1 1 1 0.8] IA_RotateStructure
  (:`Started`
    (`/Game/GrandOpening/Blueprints/ActorComponents/BP_PlacementManager.RotateGhost` (`self.BP_PlacementManager`))))

(event `EnhancedInput|/Game/GrandOpening/Inputs/Inputs/IA_Throw`
  (params (ActionValue :type Boolean) (ElapsedSeconds :type "Float (double-precision)") (TriggeredSeconds :type "Float (double-precision)") (InputAction :type "InputAction Object Reference" :default "/Game/GrandOpening/Inputs/Inputs/IA_Throw.IA_Throw"))
  ;[0.3958 0.07014 0.1822 0.8] Inputs
  ;;[1 1 1 0.8] IA_Throw
  (:`Started`
    (`self.HandleThrow`)))

(event `EnhancedInput|/Game/GrandOpening/Inputs/Inputs/IA_ToggleBuild`
  (params (ActionValue :type Boolean) (ElapsedSeconds :type "Float (double-precision)") (TriggeredSeconds :type "Float (double-precision)") (InputAction :type "InputAction Object Reference" :default "/Game/GrandOpening/Inputs/Inputs/IA_ToggleBuild.IA_ToggleBuild"))
  ;[0.3958 0.07014 0.1822 0.8] Inputs
  ;;[1 1 1 0.8] IA_ToggleBuild
  (:`Started`
    (`/Game/GrandOpening/Blueprints/ActorComponents/BP_PlacementManager.ToggleBuild` (`self.BP_PlacementManager`))))

(event `EnhancedInput|/Game/GrandOpening/Inputs/Inputs/IA_PlaceStructure`
  (params (ActionValue :type Boolean) (ElapsedSeconds :type "Float (double-precision)") (TriggeredSeconds :type "Float (double-precision)") (InputAction :type "InputAction Object Reference" :default "/Game/GrandOpening/Inputs/Inputs/IA_PlaceStructure.IA_PlaceStructure"))
  ;[0.3958 0.07014 0.1822 0.8] Inputs
  ;;[1 1 1 0.8] IA_PlaceStructure
  (:`Started`
    (`/Game/GrandOpening/Blueprints/ActorComponents/BP_PlacementManager.ConfirmPlacement` (`self.BP_PlacementManager`))))

(event `EnhancedInput|/Game/GrandOpening/Inputs/Inputs/IA_RemoveStructure`
  (params (ActionValue :type Boolean) (ElapsedSeconds :type "Float (double-precision)") (TriggeredSeconds :type "Float (double-precision)") (InputAction :type "InputAction Object Reference" :default "/Game/GrandOpening/Inputs/Inputs/IA_RemoveStructure.IA_RemoveStructure"))
  ;[0.3958 0.07014 0.1822 0.8] Inputs
  ;;[1 1 1 0.8] IA_RemoveStructure
  (:`Started`
    (`/Game/GrandOpening/Blueprints/ActorComponents/BP_PlacementManager.PickUpStructure` (`self.BP_PlacementManager`))))

(fn `AddFocusActions`
  (params (Panel :type "/Game/GrandOpening/Blueprints/Widgets/Gameplay/BP_ActionsWidget Object Reference"))
  ;[1 1 1 0.8] Add focus actions
  (bind _actor (`self.FocusedActor` self))
  (`/Engine/EditorBlueprintResources/StandardMacros.IsValid` _actor
    (:`Is Valid`
      (bind _returnvalue (`self.GetComponentByClass` _actor "/Game/GrandOpening/Blueprints/ActorComponents/BP_InteractableComponent.BP_InteractableComponent_C"))
      (if (`/Game/GrandOpening/Blueprints/ActorComponents/BP_InteractableComponent.ShowWhileCarrying` _returnvalue)
        (`/Game/GrandOpening/Blueprints/Widgets/Gameplay/BP_ActionsWidget.AddAction` Panel (`self.InteractAction`) (`/Game/GrandOpening/Blueprints/ActorComponents/BP_InteractableComponent.Label` _returnvalue))))))

(fn `ApplySprint`
  (params (Sprinting :type Boolean))
  ;[1 1 1 0.8] Apply sprint
  (set `self.Sprinting` Sprinting)
  (`self.RefreshWalkSpeed` self))

(fn `CarryObject`
  (params (Item :type "Actor Object Reference"))
  ;[1 1 1 0.8] Carry object
  (`/Game/GrandOpening/Blueprints/ActorComponents/BP_CarryComponent.GrabActor` (`self.BP_CarryComponent`) Item))

(fn `FocusedActor`
  (returns (Actor :type "Actor Object Reference"))
  (bind _focused (`/Game/GrandOpening/Blueprints/ActorComponents/BP_InteractionComponent.Focused` (`self.BP_InteractionComponent`)))
  ;[1 1 1 0.8] Focused actor
  (`/Engine/EditorBlueprintResources/StandardMacros.IsValid` _focused
    (:`Is Valid`
      (return (`ActorComponent.GetOwner` _focused)))
    (:`Is Not Valid`
      (return null))))

(fn `GetCarriedBox`
  (returns (Box :type "/Game/GrandOpening/Blueprints/Environments/Boxes/BP_DeliveryBoxBase Object Reference"))
  ;[1 1 1 0.8] Carried box
  (bind _asbp_delivery_box_base (cast `/Game/GrandOpening/Blueprints/Environments/Boxes/BP_DeliveryBoxBase` (`/Game/GrandOpening/Blueprints/ActorComponents/BP_CarryComponent.CarriedActor` (`self.BP_CarryComponent`)))
    (:`then`
      (return _asbp_delivery_box_base))
    (:`CastFailed`
      (return null))))

(fn `HandleDrop`
  ;[1 1 1 0.8] Handle drop
  (bind _returnvalue (`/Game/GrandOpening/Blueprints/ActorComponents/BP_InteractionComponent.GetAimPoint` (`self.BP_InteractionComponent`)))
  (`/Game/GrandOpening/Blueprints/ActorComponents/BP_CarryComponent.PlaceActor` (`self.BP_CarryComponent`) _returnvalue))

(fn `HandleExitFocusPressed`
  (bind _bp_viewmotioncomponent (`self.BP_ViewMotionComponent`))
  ;[1 1 1 0.8] Handle exit focus pressed
  (if (`/Game/GrandOpening/Blueprints/ActorComponents/BP_ViewMotionComponent.Focusing` _bp_viewmotioncomponent)
    (`/Game/GrandOpening/Blueprints/ActorComponents/BP_ViewMotionComponent.ClearFocus` _bp_viewmotioncomponent)
    (`/Game/GrandOpening/Blueprints/ActorComponents/BP_InteractionComponent.ShowCrosshair` (`self.BP_InteractionComponent`))))

(fn `HandleInteractPressed`
  ;[1 1 1 0.8] Handle interact pressed
  (`/Game/GrandOpening/Blueprints/ActorComponents/BP_InteractionComponent.BeginInteract` (`self.BP_InteractionComponent`)))

(fn `HandlePlaceUnit`
  ;[1 1 1 0.8] Handle place unit
  (bind _box (`self.GetCarriedBox` self))
  (`/Engine/EditorBlueprintResources/StandardMacros.IsValid` _box
    (:`Is Valid`
      (bind _actor (`self.FocusedActor` self))
      (bind _result (`/Game/GrandOpening/Blueprints/Environments/Boxes/BP_DeliveryBoxBase.UnloadOneInto` _box _actor))
      (if _result
        (`GameplayStatics.SpawnSoundAttached` (`self.PlaceSound`) (`/Game/GrandOpening/Blueprints/Environments/Boxes/BP_DeliveryBoxBase.BodyMesh` _box) "None" (0.0 0.0 0.0) (struct) "KeepRelativeOffset" false 1.0 1.0 0.0 null null))
      (`self.RefreshCarriedActions` self))))

(fn `HandleTakeUnit`
  ;[1 1 1 0.8] Handle take unit
  (bind _box (`self.GetCarriedBox` self))
  (`/Engine/EditorBlueprintResources/StandardMacros.IsValid` _box
    (:`Is Valid`
      (bind _actor (`self.FocusedActor` self))
      (bind _result (`/Game/GrandOpening/Blueprints/Environments/Boxes/BP_DeliveryBoxBase.LoadOneFrom` _box _actor))
      (if _result
        (`GameplayStatics.SpawnSoundAttached` (`self.PlaceSound`) (`/Game/GrandOpening/Blueprints/Environments/Boxes/BP_DeliveryBoxBase.BodyMesh` _box) "None" (0.0 0.0 0.0) (struct) "KeepRelativeOffset" false 1.0 1.0 0.0 null null))
      (`self.RefreshCarriedActions` self))))

(fn `HandleThrow`
  ;[1 1 1 0.8] Handle throw
  (`/Game/GrandOpening/Blueprints/ActorComponents/BP_CarryComponent.ThrowActor` (`self.BP_CarryComponent`)))

(fn `LookFromInput`
  (params (ActionValue :type "Vector2D Structure"))
  (bind (_x _y) (`KismetMathLibrary.BreakVector2D` ActionValue))
  ;[1 1 1 0.8] Look from input
  (`self.AddControllerYawInput` self _x)
  (`self.AddControllerPitchInput` self _y))

(fn `MoveFromInput`
  (params (ActionValue :type "Vector2D Structure"))
  (bind (_x _y) (`KismetMathLibrary.BreakVector2D` ActionValue))
  ;[1 1 1 0.8] Move from input
  (`self.AddMovementInput` self (`self.GetActorForwardVector` self) _y false)
  (`self.AddMovementInput` self (`self.GetActorRightVector` self) _x false))

(fn `PlaceObject`
  (params (Location :type "Vector Structure"))
  ;[1 1 1 0.8] Place object
  (`/Game/GrandOpening/Blueprints/ActorComponents/BP_CarryComponent.PlaceActor` (`self.BP_CarryComponent`) Location))

(fn `RefreshCarriedActions`
  ;[1 1 1 0.8] Refresh carried actions
  (bind _asbp_actions_widget (cast `/Game/GrandOpening/Blueprints/Widgets/Gameplay/BP_ActionsWidget` (`WidgetComponent.GetUserWidgetObject` (`self.PromptWidget`))))
  (`/Game/GrandOpening/Blueprints/Widgets/Gameplay/BP_ActionsWidget.ClearActions` _asbp_actions_widget)
  (bind _carrying (`/Game/GrandOpening/Blueprints/ActorComponents/BP_CarryComponent.IsCarrying` (`self.BP_CarryComponent`)))
  (if _carrying
    (`/Game/GrandOpening/Blueprints/Widgets/Gameplay/BP_ActionsWidget.AddAction` _asbp_actions_widget (`self.DropAction`) (`self.DropLabel`))
    (`/Game/GrandOpening/Blueprints/Widgets/Gameplay/BP_ActionsWidget.AddAction` _asbp_actions_widget (`self.ThrowAction`) (`self.ThrowLabel`))
    (`self.AddFocusActions` _asbp_actions_widget)
    (bind _box (`self.GetCarriedBox` self))
    (`/Engine/EditorBlueprintResources/StandardMacros.IsValid` _box
      (:`Is Valid`
        (bind _actor (`self.FocusedActor` self))
        (`/Game/GrandOpening/Blueprints/Environments/Boxes/BP_DeliveryBoxBase.SetFocusTarget` _box _actor)
        (`/Game/GrandOpening/Blueprints/Environments/Boxes/BP_DeliveryBoxBase.AddActionsTo` _box _asbp_actions_widget)))))

(fn `RefreshWalkSpeed`
  ;[1 1 1 0.8] Refresh walk speed
  (bind _carrying (`/Game/GrandOpening/Blueprints/ActorComponents/BP_CarryComponent.IsCarrying` (`self.BP_CarryComponent`)))
  (set `CharacterMovementComponent.MaxWalkSpeed` (* (select `bool` (`self.Sprinting`) :`false` (`self.WalkSpeed`) :`true` (`self.SprintSpeed`)) (select `bool` _carrying :`false` 1.0 :`true` (`self.CarrySpeedScale`))) (`self.CharacterMovement`)))

(fn `ReleaseObject`
  ;[1 1 1 0.8] Release object
  (`/Game/GrandOpening/Blueprints/ActorComponents/BP_CarryComponent.ReleaseActor` (`self.BP_CarryComponent`)))

(fn `SetViewLocked`
  (params (Locked :type Boolean))
  ;[1 1 1 0.8] Set view locked
  (bind _asplayer_controller (cast `PlayerController` (`self.GetController` self)))
  (`Controller.SetIgnoreMoveInput` _asplayer_controller Locked)
  (`Controller.SetIgnoreLookInput` _asplayer_controller Locked))

(fn `ToggleCarriedOrFocusedBox`
  (bind _focused (`/Game/GrandOpening/Blueprints/ActorComponents/BP_InteractionComponent.Focused` (`self.BP_InteractionComponent`)))
  ;[1 1 1 0.8] Toggle carried or focused box
  (bind _asbp_delivery_box_base (cast `/Game/GrandOpening/Blueprints/Environments/Boxes/BP_DeliveryBoxBase` (`/Game/GrandOpening/Blueprints/ActorComponents/BP_CarryComponent.CarriedActor` (`self.BP_CarryComponent`)))
    (:`then`
      (`/Game/GrandOpening/Blueprints/Environments/Boxes/BP_DeliveryBoxBase.ToggleOpen` _asbp_delivery_box_base)
      (`self.RefreshCarriedActions`))
    (:`CastFailed`
      (`/Engine/EditorBlueprintResources/StandardMacros.IsValid` _focused
        (:`Is Valid`
          (bind _asbp_delivery_box_base_2 (cast `/Game/GrandOpening/Blueprints/Environments/Boxes/BP_DeliveryBoxBase` (`ActorComponent.GetOwner` _focused)))
          (`/Game/GrandOpening/Blueprints/Environments/Boxes/BP_DeliveryBoxBase.ToggleOpen` _asbp_delivery_box_base_2)
          (`self.RefreshCarriedActions`))))))

(fn `UserConstructionScript`)
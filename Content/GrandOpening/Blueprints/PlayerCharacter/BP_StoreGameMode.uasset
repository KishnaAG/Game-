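; Store game mode that saves and restores the shop world and resets it between days.
; CollectWorldInto snapshots placed structures with storage, delivery boxes, loose carryable props and customers, folding checkout items into baskets.
; BeginPlay applies any pending GameInstance save, keeping structures that match by type and location and respawning boxes, props and customers.
; CleanForNextDay despawns customers and staff, resets checkouts and teleports the player to PlayerStart.
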(event `self.ReceiveBeginPlay`
  ;[1 1 1 0.8] Event begin play
  (`self.RestoreWorldFromSave`))

(fn `BasketOf`
  (params (Customer :type "Actor Object Reference"))
  (returns (Items :type "Array of /Game/GrandOpening/Blueprints/Structures/S_BasketItem Structure"))
  (locals (Collected :type "Array of /Game/GrandOpening/Blueprints/Structures/S_BasketItem Structure"))
  (bind _returnvalue (`self.GetComponentByClass` Customer "/Game/GrandOpening/Blueprints/ActorComponents/BP_CustomerBrain.BP_CustomerBrain_C"))
  ;[1 1 1 0.8] Basket of
  (`KismetArrayLibrary.Array_Clear` (`local.Collected`))
  (bind _outactors (`GameplayStatics.GetAllActorsOfClass` "/Game/GrandOpening/Blueprints/Environments/Checkout/BP_CheckoutBase.BP_CheckoutBase_C"))
  (for _array_element _outactors
    (if (== (`/Game/GrandOpening/Blueprints/Environments/Checkout/BP_CheckoutBase.CurrentCustomer` _array_element) Customer)
      (`KismetArrayLibrary.Array_Append` (`local.Collected`) (`/Game/GrandOpening/Blueprints/Environments/Checkout/BP_CheckoutBase.Basket` _array_element))
      (`KismetArrayLibrary.Array_Append` (`local.Collected`) (`/Game/GrandOpening/Blueprints/Environments/Checkout/BP_CheckoutBase.Receipt` _array_element))))
  (`/Engine/EditorBlueprintResources/StandardMacros.IsValid` _returnvalue
    (:`Is Valid`
      (`KismetArrayLibrary.Array_Append` (`local.Collected`) (`/Game/GrandOpening/Blueprints/ActorComponents/BP_CustomerBrain.Basket` _returnvalue)))
    (:`Is Not Valid`
      _))
  (return (`local.Collected`)))

(fn `CleanForNextDay`
  ;[1 1 1 0.8] Clean for next day
  (`self.DespawnCustomers`)
  (`self.DespawnStaff`)
  (`self.ResetCheckouts`)
  (`self.MovePlayerToStart`))

(fn `CollectCustomersInto`
  (params (Save :type "/Game/GrandOpening/Blueprints/Misc/SG_StoreSave Object Reference"))
  (locals (Shoppers :type "Array of /Game/GrandOpening/Blueprints/Structures/S_SavedCustomer Structure"))
  ;[1 1 1 0.8] Collect customers into
  (`KismetArrayLibrary.Array_Clear` (`local.Shoppers`))
  (bind _outactors (`GameplayStatics.GetAllActorsOfClass` "/Game/GrandOpening/Blueprints/AI/Customer/BP_Customer.BP_Customer_C"))
  (for _array_element _outactors
    (bind _returnvalue (`self.GetComponentByClass` _array_element "/Game/GrandOpening/Blueprints/ActorComponents/BP_CustomerBrain.BP_CustomerBrain_C"))
    (`/Engine/EditorBlueprintResources/StandardMacros.IsValid` _returnvalue
      (:`Is Valid`
        (bind _items (`self.BasketOf` _array_element))
        (`KismetArrayLibrary.Array_Add` (`local.Shoppers`) (make `/Game/GrandOpening/Blueprints/Structures/S_SavedCustomer` (`/Game/GrandOpening/Blueprints/ActorComponents/BP_CustomerBrain.Archetype` _returnvalue) (`/Game/GrandOpening/Blueprints/ActorComponents/BP_CustomerBrain.BudgetValue` _returnvalue) (`/Game/GrandOpening/Blueprints/ActorComponents/BP_CustomerBrain.TargetItems` _returnvalue) (`/Game/GrandOpening/Blueprints/ActorComponents/BP_CustomerBrain.PatienceLeft` _returnvalue) _items (`/Game/GrandOpening/Blueprints/ActorComponents/BP_CustomerBrain.ReportedStockOut` _returnvalue) (`self.GetTransform` _array_element))))))
  (set `/Game/GrandOpening/Blueprints/Misc/SG_StoreSave.Customers` (`local.Shoppers`) Save))

(fn `CollectPropsInto`
  (params (Save :type "/Game/GrandOpening/Blueprints/Misc/SG_StoreSave Object Reference"))
  (locals (Props :type "Array of /Game/GrandOpening/Blueprints/Structures/S_SavedProp Structure"))
  ;[1 1 1 0.8] Collect props into
  (bind _outactors (`GameplayStatics.GetAllActorsWithInterface` "/Game/GrandOpening/Blueprints/Interfaces/BPI_Carryable.BPI_Carryable_C"))
  (for _array_element _outactors
    (`/Engine/EditorBlueprintResources/StandardMacros.IsValid` (`self.GetParentActor` _array_element)
      (:`Is Not Valid`
        (cast `/Game/GrandOpening/Blueprints/Environments/Boxes/BP_DeliveryBoxBase` _array_element
          (:`CastFailed`
            (`KismetArrayLibrary.Array_Add` (`local.Props`) (make `/Game/GrandOpening/Blueprints/Structures/S_SavedProp` (`GameplayStatics.GetObjectClass` _array_element) (`self.GetTransform` _array_element))))))))
  (set `/Game/GrandOpening/Blueprints/Misc/SG_StoreSave.PlacedProps` (`local.Props`) Save))

(fn `CollectWorldInto`
  (params (Save :type "/Game/GrandOpening/Blueprints/Misc/SG_StoreSave Object Reference"))
  (locals (Placed :type "Array of /Game/GrandOpening/Blueprints/Structures/S_SavedStructure Structure") (Crates :type "Array of /Game/GrandOpening/Blueprints/Structures/S_SavedBox Structure"))
  ;[1 1 1 0.8] Collect world into
  (`KismetArrayLibrary.Array_Clear` (`local.Placed`))
  (`KismetArrayLibrary.Array_Clear` (`local.Crates`))
  (bind _outactors (`GameplayStatics.GetAllActorsOfClass` "/Script/Engine.Actor"))
  (for _array_element _outactors
    (bind _returnvalue (`self.GetComponentByClass` _array_element "/Game/GrandOpening/Blueprints/ActorComponents/BP_PlaceableComponent.BP_PlaceableComponent_C"))
    (`/Engine/EditorBlueprintResources/StandardMacros.IsValid` _returnvalue
      (:`Is Valid`
        (bind _structure (`/Game/GrandOpening/Blueprints/ActorComponents/BP_PlaceableComponent.Structure` _returnvalue))
        (`/Engine/EditorBlueprintResources/StandardMacros.IsValid` _structure
          (:`Is Valid`
            (bind _stacks (`self.ReadStorage` (`self.GetComponentByClass` _array_element "/Game/GrandOpening/Blueprints/ActorComponents/BP_StorageComponent.BP_StorageComponent_C")))
            (`KismetArrayLibrary.Array_Add` (`local.Placed`) (make `/Game/GrandOpening/Blueprints/Structures/S_SavedStructure` _structure (`self.GetTransform` _array_element) _stacks)))))))
  (bind _outactors_2 (`GameplayStatics.GetAllActorsOfClass` "/Game/GrandOpening/Blueprints/Environments/Boxes/BP_DeliveryBoxBase.BP_DeliveryBoxBase_C"))
  (for _array_element_2 _outactors_2
    (`KismetArrayLibrary.Array_Add` (`local.Crates`) (make `/Game/GrandOpening/Blueprints/Structures/S_SavedBox` (`/Game/GrandOpening/Blueprints/Environments/Boxes/BP_DeliveryBoxBase.Size` _array_element_2) (`/Game/GrandOpening/Blueprints/Environments/Boxes/BP_DeliveryBoxBase.Product` _array_element_2) (`/Game/GrandOpening/Blueprints/ActorComponents/BP_StorageRow.Count` (`/Game/GrandOpening/Blueprints/Environments/Boxes/BP_DeliveryBoxBase.Row_Interior` _array_element_2)) (`self.GetTransform` _array_element_2))))
  (set `/Game/GrandOpening/Blueprints/Misc/SG_StoreSave.PlacedStructures` (`local.Placed`) Save)
  (set `/Game/GrandOpening/Blueprints/Misc/SG_StoreSave.PlacedBoxes` (`local.Crates`) Save)
  (`self.CollectPropsInto` Save)
  (`self.CollectCustomersInto` Save))

(fn `DespawnCustomers`
  ;[1 1 1 0.8] Despawn customers
  (bind _outactors (`GameplayStatics.GetAllActorsOfClass` "/Game/GrandOpening/Blueprints/AI/Customer/BP_Customer.BP_Customer_C"))
  (for _array_element _outactors
    (`self.K2_DestroyActor` _array_element)))

(fn `DespawnStaff`
  (bind _returnvalue (`self.GetComponentByClass` (`GameplayStatics.GetGameState`) "/Game/GrandOpening/Blueprints/ActorComponents/BP_StaffManager.BP_StaffManager_C"))
  ;[1 1 1 0.8] Despawn staff
  (`/Engine/EditorBlueprintResources/StandardMacros.IsValid` _returnvalue
    (:`Is Valid`
      (`/Game/GrandOpening/Blueprints/ActorComponents/BP_StaffManager.DespawnAll` _returnvalue))))

(fn `IndexOfSavedStructure`
  (params (Saved :type "Array of /Game/GrandOpening/Blueprints/Structures/S_SavedStructure Structure") (Structure :type "/Game/GrandOpening/Blueprints/DataAssets/Structures/BP_StructureDataAsset Object Reference") (Placement :type "Transform Structure"))
  (returns (Index :type Integer))
  (locals (Match :type Integer))
  ;[1 1 1 0.8] Index of saved structure
  (set `local.Match` -1)
  (for (_array_element _array_index) Saved
    (bind (_structure _placement) (break `/Game/GrandOpening/Blueprints/Structures/S_SavedStructure` _array_element))
    (if (and (== _structure Structure) (== (.location _placement) (.location Placement) :`ErrorTolerance` 1.0))
      (set `local.Match` _array_index)))
  (return (`local.Match`)))

(fn `MovePlayerToStart`
  (bind _returnvalue (`GameplayStatics.GetPlayerController` 0))
  ;[1 1 1 0.8] Move player to start
  (bind _returnvalue_2 (`GameplayStatics.GetActorOfClass` "/Script/Engine.PlayerStart"))
  (`/Engine/EditorBlueprintResources/StandardMacros.IsValid` _returnvalue_2
    (:`Is Valid`
      (bind _rotation (.rotation (`self.GetTransform` _returnvalue_2)))
      (`self.K2_SetActorLocationAndRotation` (`Controller.K2_GetPawn` _returnvalue) (.location (`self.GetTransform` _returnvalue_2)) _rotation false true)
      (`Controller.SetControlRotation` _returnvalue _rotation))))

(fn `ReadStorage`
  (params (Storage :type "/Game/GrandOpening/Blueprints/ActorComponents/BP_StorageComponent Object Reference"))
  (returns (Stacks :type "Array of /Game/GrandOpening/Blueprints/Structures/S_SavedStack Structure"))
  (locals (Collected :type "Array of /Game/GrandOpening/Blueprints/Structures/S_SavedStack Structure"))
  ;[1 1 1 0.8] Read storage
  (`KismetArrayLibrary.Array_Clear` (`local.Collected`))
  (`/Engine/EditorBlueprintResources/StandardMacros.IsValid` Storage
    (:`Is Valid`
      (for _array_element (`/Game/GrandOpening/Blueprints/ActorComponents/BP_StorageComponent.Rows` Storage)
        (`KismetArrayLibrary.Array_Add` (`local.Collected`) (make `/Game/GrandOpening/Blueprints/Structures/S_SavedStack` (`/Game/GrandOpening/Blueprints/ActorComponents/BP_StorageRow.Product` _array_element) (`/Game/GrandOpening/Blueprints/ActorComponents/BP_StorageRow.Count` _array_element)))))
    (:`Is Not Valid`
      _))
  (return (`local.Collected`)))

(fn `ResetCheckouts`
  ;[1 1 1 0.8] Reset checkouts
  (bind _outactors (`GameplayStatics.GetAllActorsOfClass` "/Game/GrandOpening/Blueprints/Environments/Checkout/BP_CheckoutBase.BP_CheckoutBase_C"))
  (for _array_element _outactors
    (`/Game/GrandOpening/Blueprints/Environments/Checkout/BP_CheckoutBase.ResetForNextDay` _array_element)))

(fn `RestoreCustomers`
  (params (Save :type "/Game/GrandOpening/Blueprints/Misc/SG_StoreSave Object Reference"))
  ;[1 1 1 0.8] Restore customers
  (bind _outactors (`GameplayStatics.GetAllActorsOfClass` "/Game/GrandOpening/Blueprints/AI/Customer/BP_Customer.BP_Customer_C"))
  (for _array_element _outactors
    (`self.K2_DestroyActor` _array_element))
  (for _array_element_2 (`/Game/GrandOpening/Blueprints/Misc/SG_StoreSave.Customers` Save)
    (bind (_archetype _budget _itemswanted _patience _basket _stockoutreported _placement) (break `/Game/GrandOpening/Blueprints/Structures/S_SavedCustomer` _array_element_2))
    (bind _returnvalue (`|SpawnActorFromClass` "/Game/GrandOpening/Blueprints/AI/Customer/BP_Customer.BP_Customer_C" _placement "AdjustIfPossibleButAlwaysSpawn" "MultiplyWithRoot" null null))
    (bind _returnvalue_2 (`self.GetComponentByClass` _returnvalue "/Game/GrandOpening/Blueprints/ActorComponents/BP_CustomerBrain.BP_CustomerBrain_C"))
    (set `/Game/GrandOpening/Blueprints/ActorComponents/BP_CustomerBrain.Archetype` _archetype _returnvalue_2)
    (`/Game/GrandOpening/Blueprints/ActorComponents/BP_CustomerBrain.InitializeCustomer` _returnvalue_2)
    (set `/Game/GrandOpening/Blueprints/ActorComponents/BP_CustomerBrain.BudgetValue` _budget _returnvalue_2)
    (set `/Game/GrandOpening/Blueprints/ActorComponents/BP_CustomerBrain.TargetItems` _itemswanted _returnvalue_2)
    (set `/Game/GrandOpening/Blueprints/ActorComponents/BP_CustomerBrain.PatienceLeft` _patience _returnvalue_2)
    (set `/Game/GrandOpening/Blueprints/ActorComponents/BP_CustomerBrain.Basket` _basket _returnvalue_2)
    (set `/Game/GrandOpening/Blueprints/ActorComponents/BP_CustomerBrain.ReportedStockOut` _stockoutreported _returnvalue_2)))

(fn `RestoreProps`
  (params (Save :type "/Game/GrandOpening/Blueprints/Misc/SG_StoreSave Object Reference"))
  ;[1 1 1 0.8] Restore props
  (bind _outactors (`GameplayStatics.GetAllActorsWithInterface` "/Game/GrandOpening/Blueprints/Interfaces/BPI_Carryable.BPI_Carryable_C"))
  (for _array_element _outactors
    (`/Engine/EditorBlueprintResources/StandardMacros.IsValid` (`self.GetParentActor` _array_element)
      (:`Is Not Valid`
        (cast `/Game/GrandOpening/Blueprints/Environments/Boxes/BP_DeliveryBoxBase` _array_element
          (:`CastFailed`
            (`self.K2_DestroyActor` _array_element))))))
  (for _array_element_2 (`/Game/GrandOpening/Blueprints/Misc/SG_StoreSave.PlacedProps` Save)
    (bind (_propclass _placement) (break `/Game/GrandOpening/Blueprints/Structures/S_SavedProp` _array_element_2))
    (`|SpawnActorFromClass` _propclass _placement "AlwaysSpawn" "MultiplyWithRoot" null null)))

(fn `RestoreWorldFromSave`
  (locals (Consumed :type "Array of Integer"))
  ;[1 1 1 0.8] Restore world from save
  (bind _asbp_store_game_instance (cast `/Game/GrandOpening/Blueprints/Misc/BP_StoreGameInstance` (`GameplayStatics.GetGameInstance`)))
  (bind _pendingsave (`/Game/GrandOpening/Blueprints/Misc/BP_StoreGameInstance.PendingSave` _asbp_store_game_instance))
  (`/Engine/EditorBlueprintResources/StandardMacros.IsValid` _pendingsave
    (:`Is Valid`
      (`KismetArrayLibrary.Array_Clear` (`local.Consumed`))
      (bind _outactors (`GameplayStatics.GetAllActorsOfClass` "/Script/Engine.Actor"))
      (for _array_element _outactors
        (bind _returnvalue (`self.GetComponentByClass` _array_element "/Game/GrandOpening/Blueprints/ActorComponents/BP_PlaceableComponent.BP_PlaceableComponent_C"))
        (`/Engine/EditorBlueprintResources/StandardMacros.IsValid` _returnvalue
          (:`Is Valid`
            (bind _structure (`/Game/GrandOpening/Blueprints/ActorComponents/BP_PlaceableComponent.Structure` _returnvalue))
            (`/Engine/EditorBlueprintResources/StandardMacros.IsValid` _structure
              (:`Is Valid`
                (bind _placedstructures (`/Game/GrandOpening/Blueprints/Misc/SG_StoreSave.PlacedStructures` _pendingsave))
                (bind _index (`self.IndexOfSavedStructure` _placedstructures _structure (`self.GetTransform` _array_element)))
                (if (< _index 0)
                  (`self.K2_DestroyActor` _array_element)
                  (else
                    (`KismetArrayLibrary.Array_Add` (`local.Consumed`) _index)
                    (`self.WriteStorage` (`self.GetComponentByClass` _array_element "/Game/GrandOpening/Blueprints/ActorComponents/BP_StorageComponent.BP_StorageComponent_C") (`.Rows_6_74272FE04C9D0B244CCDD682F7769C02` (break `/Game/GrandOpening/Blueprints/Structures/S_SavedStructure` (`|GetArrayItem` _placedstructures _index)))))))))))
      (for _index_2 (range (`KismetArrayLibrary.Array_Length` _placedstructures))
        (if (not (`KismetArrayLibrary.Array_Contains` (`local.Consumed`) _index_2))
          (bind (_structure_2 _placement _rows) (break `/Game/GrandOpening/Blueprints/Structures/S_SavedStructure` (`|GetArrayItem` _placedstructures _index_2)))
          (bind _returnvalue_2 (`|SpawnActorFromClass` (`/Game/GrandOpening/Blueprints/DataAssets/Structures/BP_StructureDataAsset.PlacedClass` _structure_2) _placement "AlwaysSpawn" "MultiplyWithRoot" null null))
          (set `/Game/GrandOpening/Blueprints/ActorComponents/BP_PlaceableComponent.Structure` _structure_2 (`self.GetComponentByClass` _returnvalue_2 "/Game/GrandOpening/Blueprints/ActorComponents/BP_PlaceableComponent.BP_PlaceableComponent_C"))
          (`self.WriteStorage` (`self.GetComponentByClass` _returnvalue_2 "/Game/GrandOpening/Blueprints/ActorComponents/BP_StorageComponent.BP_StorageComponent_C") _rows)))
      (bind _outactors_2 (`GameplayStatics.GetAllActorsOfClass` "/Game/GrandOpening/Blueprints/Environments/Boxes/BP_DeliveryBoxBase.BP_DeliveryBoxBase_C"))
      (for _array_element_2 _outactors_2
        (`self.K2_DestroyActor` _array_element_2))
      (for _array_element_3 (`/Game/GrandOpening/Blueprints/Misc/SG_StoreSave.PlacedBoxes` _pendingsave)
        (bind (_size _product _units _placement_2) (break `/Game/GrandOpening/Blueprints/Structures/S_SavedBox` _array_element_3))
        (`|SpawnActorFromClass` "/Game/GrandOpening/Blueprints/Environments/Boxes/BP_DeliveryBoxBase.BP_DeliveryBoxBase_C" _placement_2 "AlwaysSpawn" "MultiplyWithRoot" null _product _units _size null))
      (`self.RestoreProps` _pendingsave)
      (`self.RestoreCustomers` _pendingsave))))

(fn `UserConstructionScript`)

(fn `WriteStorage`
  (params (Storage :type "/Game/GrandOpening/Blueprints/ActorComponents/BP_StorageComponent Object Reference") (Stacks :type "Array of /Game/GrandOpening/Blueprints/Structures/S_SavedStack Structure"))
  ;[1 1 1 0.8] Write storage
  (`/Engine/EditorBlueprintResources/StandardMacros.IsValid` Storage
    (:`Is Valid`
      (for (_array_element _array_index) (`/Game/GrandOpening/Blueprints/ActorComponents/BP_StorageComponent.Rows` Storage)
        (if (`KismetArrayLibrary.Array_IsValidIndex` Stacks _array_index)
          (bind (_product _count) (break `/Game/GrandOpening/Blueprints/Structures/S_SavedStack` (`|GetArrayItem` Stacks _array_index)))
          (set `/Game/GrandOpening/Blueprints/ActorComponents/BP_StorageRow.Product` _product _array_element)
          (set `/Game/GrandOpening/Blueprints/ActorComponents/BP_StorageRow.Count` _count _array_element)))
      (`/Game/GrandOpening/Blueprints/ActorComponents/BP_StorageComponent.RefreshInstances` Storage))))
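; Player controller for the store game that owns the HUD and drives end-of-day, pause and game-over UI flows.
; Closing the store stops serving and opens a modal; the day report leads to game over if bankrupt, or a transition into the next day.
; The day advances once the transition covers the screen, with a fallback timer guarded by a lock.
; The pause menu routes to save/load slots through the game instance, main menu and quit.
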(event `self.ReceiveBeginPlay`
  ;[1 1 1 0.8] Event begin play
  (bind _returnvalue (`|CreateWidget` "/Game/GrandOpening/Blueprints/Widgets/Gameplay/BP_HudWidget.BP_HudWidget_C" self))
  (bind _output_get (set `self.BP_HudWidget` _returnvalue))
  (`UserWidget.AddToViewport` _output_get 0)
  (`WidgetBlueprintLibrary.SetInputMode_GameOnly` self))

(event `EnhancedInput|/Game/GrandOpening/Inputs/Inputs/IA_Pause`
  (params (ActionValue :type Boolean) (ElapsedSeconds :type "Float (double-precision)") (TriggeredSeconds :type "Float (double-precision)") (InputAction :type "InputAction Object Reference" :default "/Game/GrandOpening/Inputs/Inputs/IA_Pause.IA_Pause"))
  ;[1 1 1 0.8] IA_Pause
  (:`Started`
    (`self.TogglePause`)))

(fn `AdvanceToNextDay`
  (bind _returnvalue (`self.GetComponentByClass` (`GameplayStatics.GetGameState`) "/Game/GrandOpening/Blueprints/ActorComponents/BP_StoreManager.BP_StoreManager_C"))
  ;[1 1 1 0.8] Advance to next day
  (bind _asbp_store_game_mode (cast `/Game/GrandOpening/Blueprints/PlayerCharacter/BP_StoreGameMode` (`GameplayStatics.GetGameMode`)))
  (`/Game/GrandOpening/Blueprints/PlayerCharacter/BP_StoreGameMode.CleanForNextDay` _asbp_store_game_mode)
  (`/Engine/EditorBlueprintResources/StandardMacros.IsValid` _returnvalue
    (:`Is Valid`
      (`/Game/GrandOpening/Blueprints/ActorComponents/BP_StoreManager.FinishCurrentDay` _returnvalue))))

(fn `ConfirmMainMenu`
  ;[1 1 1 0.8] Confirm main menu
  (bind _returnvalue (`|CreateWidget` (`self.ModalClass`) self))
  (set `/Game/GrandOpening/Blueprints/Widgets/Gameplay/BP_ModalWidget.Title` (`self.MainMenuTitle`) _returnvalue)
  (set `/Game/GrandOpening/Blueprints/Widgets/Gameplay/BP_ModalWidget.Message` (`self.MainMenuMessage`) _returnvalue)
  (add `/Game/GrandOpening/Blueprints/Widgets/Gameplay/BP_ModalWidget.OnConfirmed` _returnvalue (`|CreateDelegate` :!event `GoToMainMenu`))
  (`UserWidget.AddToViewport` _returnvalue 0))

(fn `ConfirmQuit`
  ;[1 1 1 0.8] Confirm quit
  (bind _returnvalue (`|CreateWidget` (`self.ModalClass`) self))
  (set `/Game/GrandOpening/Blueprints/Widgets/Gameplay/BP_ModalWidget.Title` (`self.QuitTitle`) _returnvalue)
  (set `/Game/GrandOpening/Blueprints/Widgets/Gameplay/BP_ModalWidget.Message` (`self.QuitMessage`) _returnvalue)
  (add `/Game/GrandOpening/Blueprints/Widgets/Gameplay/BP_ModalWidget.OnConfirmed` _returnvalue (`|CreateDelegate` :!event `QuitToDesktop`))
  (`UserWidget.AddToViewport` _returnvalue 0))

(fn `GoToMainMenu`
  ;[1 1 1 0.8] Go to main menu
  (`GameplayStatics.SetGamePaused` false)
  (`GameplayStatics.OpenLevelBySoftObjectPtr` (`self.MenuLevel`)))

(fn `HandleDayCovered`
  ;[1 1 1 0.8] Handle day covered
  (if (`self.TransitionLocked`)
    (`KismetSystemLibrary.K2_ClearAndInvalidateTimerHandle` (`self.TransitionTimer`))
    (`self.AdvanceToNextDay`)
    (`/Game/GrandOpening/Blueprints/Widgets/Gameplay/BP_DayTransitionWidget.FadeOut` (`self.BP_DayTransitionWidget`))
    (`self.ReturnToGame`)))

(fn `HandleDeleteRequested`
  (params (Index :type Integer))
  ;[1 1 1 0.8] Handle delete requested
  (bind _asbp_store_game_instance (cast `/Game/GrandOpening/Blueprints/Misc/BP_StoreGameInstance` (`GameplayStatics.GetGameInstance`)))
  (`/Game/GrandOpening/Blueprints/Misc/BP_StoreGameInstance.DeleteSlot` _asbp_store_game_instance Index)
  (`/Game/GrandOpening/Blueprints/Widgets/Menu/BP_SlotPickerWidget.ClearSlot` (`self.SlotPicker`) Index))

(fn `HandleGameOverEntry`
  (params (Id :type Name))
  ;[1 1 1 0.8] Handle game over entry
  (if (== Id "MainMenu")
    (`self.GoToMainMenu`)
    (elif (== Id "Quit")
      (`self.QuitToDesktop`))))

(fn `HandleNewDayRequested`
  (bind _returnvalue (`self.GetComponentByClass` (`GameplayStatics.GetGameState`) "/Game/GrandOpening/Blueprints/ActorComponents/BP_StoreManager.BP_StoreManager_C"))
  ;[1 1 1 0.8] Handle new day requested
  (bind _bankrupt (`/Game/GrandOpening/Blueprints/ActorComponents/BP_StoreManager.IsBankrupt` _returnvalue))
  (if _bankrupt
    (`self.ShowGameOver` _returnvalue)
    (else
      (`self.StartNewDay`))))

(fn `HandlePauseEntry`
  (params (Id :type Name))
  ;[1 1 1 0.8] Handle pause entry
  (if (== Id "Resume")
    (`self.ResumeGame`)
    (elif (== Id "SaveGame")
      (`self.OpenSlotPicker` "NewEnumerator2")
      (elif (== Id "LoadGame")
        (`self.OpenSlotPicker` "NewEnumerator1")
        (elif (== Id "MainMenu")
          (`self.ConfirmMainMenu`)
          (elif (== Id "Quit")
            (`self.ConfirmQuit`)))))))

(fn `HandlePickerBack`
  ;[1 1 1 0.8] Handle picker back
  (`/Game/GrandOpening/Blueprints/Widgets/Menu/BP_SlotPickerWidget.Dismiss` (`self.SlotPicker`))
  (`self.ShowPauseMenu`))

(fn `HandleSlotPicked`
  (params (Index :type Integer))
  ;[1 1 1 0.8] Handle slot picked
  (if (`|EnumEquality` (`self.PickerMode`) "NewEnumerator2")
    (`self.SaveSlot` Index)
    (else
      (`self.LoadSlot` Index))))

(fn `LoadSlot`
  (params (Index :type Integer))
  ;[1 1 1 0.8] Load slot
  (bind _asbp_store_game_instance (cast `/Game/GrandOpening/Blueprints/Misc/BP_StoreGameInstance` (`GameplayStatics.GetGameInstance`)))
  (`/Game/GrandOpening/Blueprints/Misc/BP_StoreGameInstance.RequestLoad` _asbp_store_game_instance Index)
  (`GameplayStatics.SetGamePaused` false)
  (bind _returnvalue (`GameplayStatics.GetCurrentLevelName` true))
  (`GameplayStatics.OpenLevel` (`KismetStringLibrary.Conv_StringToName` _returnvalue)))

(fn `OpenPauseMenu`
  (set `self.PauseOpen` true)
  (`GameplayStatics.SetGamePaused` true)
  (set `self.bShowMouseCursor` true)
  (`WidgetBlueprintLibrary.SetInputMode_GameAndUIEx` self null)
  (`self.ShowPauseMenu`))

(fn `OpenSlotPicker`
  (params (Mode :type "/Game/GrandOpening/Blueprints/Enumerations/E_SlotPickerMode Enum" :default "NewEnumerator0"))
  ;[1 1 1 0.8] Open slot picker
  (set `self.PickerMode` Mode)
  (`/Game/GrandOpening/Blueprints/Widgets/Menu/BP_PauseMenuWidget.Dismiss` (`self.PauseMenu`))
  (bind _returnvalue (`|CreateWidget` (`self.SlotPickerClass`) self))
  (set `self.SlotPicker` _returnvalue)
  (`/Game/GrandOpening/Blueprints/Widgets/Menu/BP_SlotPickerWidget.OpenAs` _returnvalue Mode)
  (add `/Game/GrandOpening/Blueprints/Widgets/Menu/BP_SlotPickerWidget.OnSlotPicked` _returnvalue (`|CreateDelegate` :!event `HandleSlotPicked`))
  (add `/Game/GrandOpening/Blueprints/Widgets/Menu/BP_SlotPickerWidget.OnDeleteRequested` _returnvalue (`|CreateDelegate` :!event `HandleDeleteRequested`))
  (add `/Game/GrandOpening/Blueprints/Widgets/Menu/BP_SlotPickerWidget.OnBack` _returnvalue (`|CreateDelegate` :!event `HandlePickerBack`))
  (`UserWidget.AddToViewport` _returnvalue 0))

(fn `QuitToDesktop`
  ;[1 1 1 0.8] Quit to desktop
  (`KismetSystemLibrary.QuitGame` self "Quit"))

(fn `RequestCloseStore`
  ;[1 1 1 0.8] Request close store
  (if (not (`self.ClosingUIOpen`))
    (set `self.ClosingUIOpen` true)
    (bind _returnvalue (`|CreateWidget` (`self.ModalClass`) self))
    (set `/Game/GrandOpening/Blueprints/Widgets/Gameplay/BP_ModalWidget.Title` (`self.CloseStoreTitle`) _returnvalue)
    (set `/Game/GrandOpening/Blueprints/Widgets/Gameplay/BP_ModalWidget.Message` (`self.CloseStoreMessage`) _returnvalue)
    (add `/Game/GrandOpening/Blueprints/Widgets/Gameplay/BP_ModalWidget.OnConfirmed` _returnvalue (`|CreateDelegate` :!event `ShowDayReport`))
    (add `/Game/GrandOpening/Blueprints/Widgets/Gameplay/BP_ModalWidget.OnCancelled` _returnvalue (`|CreateDelegate` :!event `ReturnToGame`))
    (`UserWidget.AddToViewport` _returnvalue 0)
    (set `self.bShowMouseCursor` true)
    (`WidgetBlueprintLibrary.SetInputMode_UIOnlyEx` self null "DoNotLock" true)
    (`self.SetStoreServing` false)))

(fn `ResumeGame`
  ;[1 1 1 0.8] Resume game
  (set `self.PauseOpen` false)
  (`/Game/GrandOpening/Blueprints/Widgets/Menu/BP_PauseMenuWidget.Dismiss` (`self.PauseMenu`))
  (`GameplayStatics.SetGamePaused` false)
  (set `self.bShowMouseCursor` false)
  (`WidgetBlueprintLibrary.SetInputMode_GameOnly` self))

(fn `ReturnToGame`
  ;[1 1 1 0.8] Return to game
  (set `self.ClosingUIOpen` false)
  (set `self.bShowMouseCursor` false)
  (`WidgetBlueprintLibrary.SetInputMode_GameOnly` self)
  (set `self.TransitionLocked` false)
  (`self.SetStoreServing` true))

(fn `SaveSlot`
  (params (Index :type Integer))
  ;[1 1 1 0.8] Save slot
  (bind _asbp_store_game_instance (cast `/Game/GrandOpening/Blueprints/Misc/BP_StoreGameInstance` (`GameplayStatics.GetGameInstance`)))
  (`/Game/GrandOpening/Blueprints/Misc/BP_StoreGameInstance.SaveToSlot` _asbp_store_game_instance Index)
  (`self.HandlePickerBack`))

(fn `SetStoreServing`
  (params (Serving :type Boolean))
  (bind _returnvalue (`self.GetComponentByClass` (`GameplayStatics.GetGameState`) "/Game/GrandOpening/Blueprints/ActorComponents/BP_StoreManager.BP_StoreManager_C"))
  ;[1 1 1 0.8] Set store serving
  (`/Engine/EditorBlueprintResources/StandardMacros.IsValid` _returnvalue
    (:`Is Valid`
      (`/Game/GrandOpening/Blueprints/ActorComponents/BP_StoreManager.SetServingCustomers` _returnvalue Serving))))

(fn `ShowDayReport`
  (bind _returnvalue (`self.GetComponentByClass` (`GameplayStatics.GetGameState`) "/Game/GrandOpening/Blueprints/ActorComponents/BP_StoreManager.BP_StoreManager_C"))
  ;[1 1 1 0.8] Show day report
  (`/Engine/EditorBlueprintResources/StandardMacros.IsValid` _returnvalue
    (:`Is Valid`
      (`/Game/GrandOpening/Blueprints/ActorComponents/BP_StoreManager.CloseCurrentDay` _returnvalue))
    (:`Is Not Valid`
      _))
  (bind _returnvalue_2 (`|CreateWidget` (`self.DayReportClass`) self))
  (set `self.BP_DayReportWidget` _returnvalue_2)
  (add `/Game/GrandOpening/Blueprints/Widgets/Gameplay/BP_DayReportWidget.OnNewDayRequested` _returnvalue_2 (`|CreateDelegate` :!event `HandleNewDayRequested`))
  (`UserWidget.AddToViewport` (`self.BP_DayReportWidget`) 0))

(fn `ShowGameOver`
  (params (StoreManager :type "/Game/GrandOpening/Blueprints/ActorComponents/BP_StoreManager Object Reference"))
  ;[1 1 1 0.8] Show game over
  (`Widget.RemoveFromParent` (`self.BP_DayReportWidget`))
  (bind _returnvalue (`|CreateWidget` (`self.GameOverClass`) self))
  (`/Game/GrandOpening/Blueprints/Widgets/Menu/BP_GameOverWidget.FillOutcome` _returnvalue StoreManager)
  (add `/Game/GrandOpening/Blueprints/Widgets/Menu/BP_GameOverWidget.OnGameOverEntryChosen` _returnvalue (`|CreateDelegate` :!event `HandleGameOverEntry`))
  (`UserWidget.AddToViewport` _returnvalue 0))

(fn `ShowPauseMenu`
  ;[1 1 1 0.8] Show pause menu
  (bind _returnvalue (`|CreateWidget` (`self.PauseMenuClass`) self))
  (set `self.PauseMenu` _returnvalue)
  (add `/Game/GrandOpening/Blueprints/Widgets/Menu/BP_PauseMenuWidget.OnPauseEntryChosen` _returnvalue (`|CreateDelegate` :!event `HandlePauseEntry`))
  (`UserWidget.AddToViewport` _returnvalue 0))

(fn `StartNewDay`
  ;[1 1 1 0.8] Start new day
  (set `self.TransitionLocked` true)
  (`Widget.RemoveFromParent` (`self.BP_DayReportWidget`))
  (bind _returnvalue (`|CreateWidget` (`self.TransitionClass`) self))
  (set `self.BP_DayTransitionWidget` _returnvalue)
  (add `/Game/GrandOpening/Blueprints/Widgets/Gameplay/BP_DayTransitionWidget.OnCovered` _returnvalue (`|CreateDelegate` :!event `HandleDayCovered`))
  (`UserWidget.AddToViewport` (`self.BP_DayTransitionWidget`) 0)
  (bind _returnvalue_2 (`KismetSystemLibrary.K2_SetTimer` self "HandleDayCovered" (`self.TransitionTimeoutSeconds`)))
  (set `self.TransitionTimer` _returnvalue_2))

(fn `TogglePause`
  ;[1 1 1 0.8] Toggle pause
  (if (not (`self.ClosingUIOpen`))
    (if (`self.PauseOpen`)
      (`self.ResumeGame`)
      (else
        (`self.OpenPauseMenu`)))))

(fn `UserConstructionScript`)
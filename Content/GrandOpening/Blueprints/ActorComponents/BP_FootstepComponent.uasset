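; Actor component that plays footstep sounds matched to the surface under its owner.
; PlayFootstep traces downward on the Visibility channel from the owner's location over a configurable distance.
; The hit's physical surface type selects a concrete, ground, metal, water, wood or default sound.
; On a hit, that sound spawns attached to the owner's root component at the volume passed by the caller.
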(fn `PlayFootstep`
  (params (Volume :type "Float (double-precision)"))
  (bind _returnvalue (`self.GetOwner` self))
  (bind _returnvalue_2 (`Actor.K2_GetActorLocation` _returnvalue))
  ;[1 1 1 0.8] Play footstep
  (bind (_outhit _returnvalue_3) (`KismetSystemLibrary.LineTraceSingle` _returnvalue_2 (- _returnvalue_2 (`KismetMathLibrary.MakeVector` 0.0 0.0 (`self.FootstepTraceCm`))) "TraceTypeQuery1"))
  (if _returnvalue_3
    (switch `EPhysicalSurface` (`GameplayStatics.GetSurfaceType` _outhit)
      (:`SurfaceType_Default`
        (set `self.Sound` (`self.FootstepDefault`)))
      (:`SurfaceType1`
        (set `self.Sound` (`self.FootstepConcrete`)))
      (:`SurfaceType2`
        (set `self.Sound` (`self.FootstepGround`)))
      (:`SurfaceType3`
        (set `self.Sound` (`self.FootstepMetal`)))
      (:`SurfaceType4`
        (set `self.Sound` (`self.FootstepWater`)))
      (:`SurfaceType5`
        (set `self.Sound` (`self.FootstepWood`))))
    (`GameplayStatics.SpawnSoundAttached` (`self.Sound`) (`Actor.RootComponent` _returnvalue) "None" (0.0 0.0 0.0) (struct) "KeepRelativeOffset" false Volume 1.0 0.0 null null)))
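; Actor component that manages the store's ad campaigns, each running for a set number of days on registered ad panels.
; Starting a campaign needs a free panel and funds, charges the first day through BP_StoreManager, and daily advancement bills or expires runs.
; Only runs with a panel are live, feeding traffic, rating and promoted-category queries, while extras stay frozen.
; Runs persist via the save and restore on BeginPlay.
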(event `self.ReceiveBeginPlay`
  (bind _storemanager (`self.StoreManager`))
  ;[1 1 1 0.8] Event begin play
  (set `self.StoreManager` (`Actor.GetComponentByClass` (`GameplayStatics.GetGameState`) "/Game/GrandOpening/Blueprints/ActorComponents/BP_StoreManager.BP_StoreManager_C"))
  (`/Engine/EditorBlueprintResources/StandardMacros.IsValid` _storemanager
    (:`Is Valid`
      (add `/Game/GrandOpening/Blueprints/ActorComponents/BP_StoreManager.OnDayEnded` _storemanager (`|CreateDelegate` :!event `AdvanceCampaigns`))
      (`self.RestoreFromSave`))))

(fn `AdvanceCampaigns`
  (params (Day :type Integer))
  (locals (Remaining :type "Array of /Game/GrandOpening/Blueprints/Structures/S_AdRun Structure"))
  (bind _runs (`self.Runs`))
  ;[1 1 1 0.8] Advance campaigns
  (bind _count (`self.LiveRunCount`))
  (for _index (range (`KismetArrayLibrary.Array_Length` _runs))
    (if (< _index _count)
      (bind _output (`|GetArrayItem` _runs _index))
      (bind (_campaign _daysleft) (break `/Game/GrandOpening/Blueprints/Structures/S_AdRun` _output))
      (bind _returnvalue (- _daysleft 1))
      (if (> _returnvalue 0)
        (`/Game/GrandOpening/Blueprints/ActorComponents/BP_StoreManager.AddTransaction` (`self.StoreManager`) (- 0.0 (`/Game/GrandOpening/Blueprints/DataAssets/Ads/BP_AdCampaignDataAsset.CostPerDay` _campaign)) "NewEnumerator8" "None")
        (`KismetArrayLibrary.Array_Add` (`local.Remaining`) (make `/Game/GrandOpening/Blueprints/Structures/S_AdRun` _campaign _returnvalue)))
      (else
        (`KismetArrayLibrary.Array_Add` (`local.Remaining`) _output))))
  (set `self.Runs` (`local.Remaining`))
  (`self.RefreshPanels`))

(fn `CanStartCampaign`
  (params (Campaign :type "/Game/GrandOpening/Blueprints/DataAssets/Ads/BP_AdCampaignDataAsset Object Reference"))
  (returns (Can :type Boolean))
  ;[1 1 1 0.8] Can start campaign
  (`/Engine/EditorBlueprintResources/StandardMacros.IsValid` Campaign
    (:`Is Valid`
      (bind _index (`self.RunIndexForCampaign` Campaign))
      (return (and (and (< (`KismetArrayLibrary.Array_Length` (`self.Runs`)) (`KismetArrayLibrary.Array_Length` (`self.Panels`))) (< _index 0)) (>= (`/Game/GrandOpening/Blueprints/ActorComponents/BP_StoreManager.CurrentBalance` (`self.StoreManager`)) (`/Game/GrandOpening/Blueprints/DataAssets/Ads/BP_AdCampaignDataAsset.CostPerDay` Campaign)))))
    (:`Is Not Valid`
      (return false))))

(fn `CollectInto`
  (params (Save :type "/Game/GrandOpening/Blueprints/Misc/SG_StoreSave Object Reference"))
  ;[1 1 1 0.8] Collect into
  (set `/Game/GrandOpening/Blueprints/Misc/SG_StoreSave.AdRuns` (`self.Runs`) Save))

(fn `DaysLeftFor`
  (params (Campaign :type "/Game/GrandOpening/Blueprints/DataAssets/Ads/BP_AdCampaignDataAsset Object Reference"))
  (returns (Days :type Integer))
  ;[1 1 1 0.8] Days left for
  (bind _index (`self.RunIndexForCampaign` Campaign))
  (if (>= _index 0)
    (return (`.DaysLeft_6_B07693B54202962830BE518503AB7AB1` (break `/Game/GrandOpening/Blueprints/Structures/S_AdRun` (`|GetArrayItem` (`self.Runs`) _index))))
    (else
      (return 0))))

(fn `LiveRunCount`
  (returns (Count :type Integer))
  ;[1 1 1 0.8] Live run count
  (return (`KismetMathLibrary.Min` (`KismetArrayLibrary.Array_Length` (`self.Runs`)) (`KismetArrayLibrary.Array_Length` (`self.Panels`)))))

(fn `PromotedCategories`
  (returns (Categories :type "Array of /Game/GrandOpening/Blueprints/Enumerations/E_ProductCategory Enum"))
  (locals (Found :type "Array of /Game/GrandOpening/Blueprints/Enumerations/E_ProductCategory Enum"))
  ;[1 1 1 0.8] Promoted categories
  (bind _count (`self.LiveRunCount`))
  (for _index (range _count)
    (bind _campaign (break `/Game/GrandOpening/Blueprints/Structures/S_AdRun` (`|GetArrayItem` (`self.Runs`) _index)))
    (`/Engine/EditorBlueprintResources/StandardMacros.IsValid` _campaign
      (:`Is Valid`
        (`KismetArrayLibrary.Array_Append` (`local.Found`) (`/Game/GrandOpening/Blueprints/DataAssets/Ads/BP_AdCampaignDataAsset.PromotedCategories` _campaign)))))
  (return (`local.Found`)))

(fn `RatingDelta`
  (returns (Delta :type "Float (double-precision)"))
  (locals (Sum :type "Float (double-precision)"))
  ;[1 1 1 0.8] Rating delta
  (set `local.Sum` 0.0)
  (bind _count (`self.LiveRunCount`))
  (for _index (range _count)
    (bind _campaign (break `/Game/GrandOpening/Blueprints/Structures/S_AdRun` (`|GetArrayItem` (`self.Runs`) _index)))
    (`/Engine/EditorBlueprintResources/StandardMacros.IsValid` _campaign
      (:`Is Valid`
        (set `local.Sum` (+ (`local.Sum`) (`/Game/GrandOpening/Blueprints/DataAssets/Ads/BP_AdCampaignDataAsset.RatingDelta` _campaign))))))
  (return (`local.Sum`)))

(fn `RefreshPanels`
  (bind _panels (`self.Panels`))
  ;[1 1 1 0.8] Refresh panels
  (bind _count (`self.LiveRunCount`))
  (for _index (range (`KismetArrayLibrary.Array_Length` _panels))
    (bind _output (`|GetArrayItem` _panels _index))
    (`/Engine/EditorBlueprintResources/StandardMacros.IsValid` _output
      (:`Is Valid`
        (if (< _index _count)
          (`/Game/GrandOpening/Blueprints/Environments/Misc/BP_AdPanel.ShowCampaign` _output (`.Campaign_2_3CC1162D46054638CB54CC9DA7A585E7` (break `/Game/GrandOpening/Blueprints/Structures/S_AdRun` (`|GetArrayItem` (`self.Runs`) _index))))
          (else
            (`/Game/GrandOpening/Blueprints/Environments/Misc/BP_AdPanel.ShowCampaign` _output null)))))))

(fn `RegisterPanel`
  (params (Panel :type "/Game/GrandOpening/Blueprints/Environments/Misc/BP_AdPanel Object Reference"))
  ;[1 1 1 0.8] Register panel
  (`/Engine/EditorBlueprintResources/StandardMacros.IsValid` Panel
    (:`Is Valid`
      (`KismetArrayLibrary.Array_AddUnique` (`self.Panels`) Panel)
      (`self.RefreshPanels`))))

(fn `RestoreFromSave`
  ;[1 1 1 0.8] Restore from save
  (bind _asbp_store_game_instance (cast `/Game/GrandOpening/Blueprints/Misc/BP_StoreGameInstance` (`GameplayStatics.GetGameInstance`)))
  (bind _pendingsave (`/Game/GrandOpening/Blueprints/Misc/BP_StoreGameInstance.PendingSave` _asbp_store_game_instance))
  (`/Engine/EditorBlueprintResources/StandardMacros.IsValid` _pendingsave
    (:`Is Valid`
      (set `self.Runs` (`/Game/GrandOpening/Blueprints/Misc/SG_StoreSave.AdRuns` _pendingsave))
      (`self.RefreshPanels`))))

(fn `RunIndexForCampaign`
  (params (Campaign :type "/Game/GrandOpening/Blueprints/DataAssets/Ads/BP_AdCampaignDataAsset Object Reference"))
  (returns (Index :type Integer))
  (bind _runs (`self.Runs`))
  ;[1 1 1 0.8] Run index for campaign
  (for _index (range (`KismetArrayLibrary.Array_Length` _runs))
    (if (== (`.Campaign_2_3CC1162D46054638CB54CC9DA7A585E7` (break `/Game/GrandOpening/Blueprints/Structures/S_AdRun` (`|GetArrayItem` _runs _index))) Campaign)
      (return _index)))
  (return -1))

(fn `StartCampaign`
  (params (Campaign :type "/Game/GrandOpening/Blueprints/DataAssets/Ads/BP_AdCampaignDataAsset Object Reference"))
  (returns (Started :type Boolean))
  ;[1 1 1 0.8] Start campaign
  (bind _can (`self.CanStartCampaign` Campaign))
  (if _can
    (`/Game/GrandOpening/Blueprints/ActorComponents/BP_StoreManager.AddTransaction` (`self.StoreManager`) (- 0.0 (`/Game/GrandOpening/Blueprints/DataAssets/Ads/BP_AdCampaignDataAsset.CostPerDay` Campaign)) "NewEnumerator8" "None")
    (`KismetArrayLibrary.Array_Add` (`self.Runs`) (make `/Game/GrandOpening/Blueprints/Structures/S_AdRun` Campaign (`/Game/GrandOpening/Blueprints/DataAssets/Ads/BP_AdCampaignDataAsset.DurationDays` Campaign)))
    (`self.RefreshPanels`)
    (return true)
    (else
      (return false))))

(fn `StopCampaign`
  (params (Campaign :type "/Game/GrandOpening/Blueprints/DataAssets/Ads/BP_AdCampaignDataAsset Object Reference"))
  ;[1 1 1 0.8] Stop campaign
  (bind _index (`self.RunIndexForCampaign` Campaign))
  (if (>= _index 0)
    (`KismetArrayLibrary.Array_Remove` (`self.Runs`) _index)
    (`self.RefreshPanels`)))

(fn `TrafficMultiplier`
  (returns (Multiplier :type "Float (double-precision)"))
  (locals (Factor :type "Float (double-precision)"))
  ;[1 1 1 0.8] Traffic multiplier
  (set `local.Factor` 1.0)
  (bind _count (`self.LiveRunCount`))
  (for _index (range _count)
    (bind _campaign (break `/Game/GrandOpening/Blueprints/Structures/S_AdRun` (`|GetArrayItem` (`self.Runs`) _index)))
    (`/Engine/EditorBlueprintResources/StandardMacros.IsValid` _campaign
      (:`Is Valid`
        (set `local.Factor` (* (`local.Factor`) (`/Game/GrandOpening/Blueprints/DataAssets/Ads/BP_AdCampaignDataAsset.TrafficMultiplier` _campaign))))))
  (return (`local.Factor`)))

(fn `UnregisterPanel`
  (params (Panel :type "/Game/GrandOpening/Blueprints/Environments/Misc/BP_AdPanel Object Reference"))
  ;[1 1 1 0.8] Unregister panel
  (`KismetArrayLibrary.Array_RemoveItem` (`self.Panels`) Panel)
  (`self.RefreshPanels`))
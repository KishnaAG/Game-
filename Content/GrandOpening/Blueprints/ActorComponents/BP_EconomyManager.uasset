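; Economy manager component that charges the store's daily running costs and simulates fluctuating wholesale prices per product.
; When BP_StoreManager ends a day, it posts rent, utilities and revenue tax as transactions, then drifts the market quotes.
; A matching product transaction that day raises its multiplier, otherwise it eases toward 1.0, with random volatility and clamping.
; Multipliers scale cost price into wholesale price, and quotes persist through the save.
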(event `self.ReceiveBeginPlay`
  ;[1 1 1 0.8] Event begin play
  (set `self.StoreManager` (`Actor.GetComponentByClass` (`GameplayStatics.GetGameState`) "/Game/GrandOpening/Blueprints/ActorComponents/BP_StoreManager.BP_StoreManager_C"))
  (`/Engine/EditorBlueprintResources/StandardMacros.IsValid` (`self.StoreManager`)
    (:`Is Valid`
      (add `/Game/GrandOpening/Blueprints/ActorComponents/BP_StoreManager.OnDayEnded` (`self.StoreManager`) (`|CreateDelegate` :!event `HandleDayEnded`))
      (`self.InitializeQuotes`)
      (`self.RestoreFromSave`))))

(fn `ChargeDailyCosts`
  (params (Day :type Integer))
  (bind _economyconfig (`self.EconomyConfig`))
  (bind _storemanager (`self.StoreManager`))
  ;[1 1 1 0.8] Charge daily costs
  (`/Game/GrandOpening/Blueprints/ActorComponents/BP_StoreManager.AddTransaction` _storemanager (- 0.0 (`/Game/GrandOpening/Blueprints/DataAssets/Economy/BP_EconomyConfigDataAsset.DailyRent` _economyconfig)) "NewEnumerator2" "None")
  (`/Game/GrandOpening/Blueprints/ActorComponents/BP_StoreManager.AddTransaction` _storemanager (- 0.0 (`/Game/GrandOpening/Blueprints/DataAssets/Economy/BP_EconomyConfigDataAsset.DailyUtilities` _economyconfig)) "NewEnumerator3" "None")
  (bind _report (`/Game/GrandOpening/Blueprints/ActorComponents/BP_StoreManager.GetDayReport` _storemanager Day))
  (`/Game/GrandOpening/Blueprints/ActorComponents/BP_StoreManager.AddTransaction` _storemanager (- 0.0 (* (`.Revenue_7_D1C29FE9478FF9FEBF50D1B0FE303101` (break `/Game/GrandOpening/Blueprints/Structures/S_DayReport` _report)) (`/Game/GrandOpening/Blueprints/DataAssets/Economy/BP_EconomyConfigDataAsset.TaxRate` _economyconfig))) "NewEnumerator5" "None"))

(fn `CollectInto`
  (params (Save :type "/Game/GrandOpening/Blueprints/Misc/SG_StoreSave Object Reference"))
  ;[1 1 1 0.8] Collect into
  (set `/Game/GrandOpening/Blueprints/Misc/SG_StoreSave.MarketQuotes` (`self.Quotes`) Save))

(fn `DriftMarket`
  (params (Day :type Integer))
  (bind _economyconfig (`self.EconomyConfig`))
  (bind _quotes (`self.Quotes`))
  (bind _demandamplitude (`/Game/GrandOpening/Blueprints/DataAssets/Economy/BP_EconomyConfigDataAsset.DemandAmplitude` _economyconfig))
  (bind _marketrange (`/Game/GrandOpening/Blueprints/DataAssets/Economy/BP_EconomyConfigDataAsset.MarketRange` _economyconfig))
  (bind _marketvolatility (`/Game/GrandOpening/Blueprints/DataAssets/Economy/BP_EconomyConfigDataAsset.MarketVolatility` _economyconfig))
  ;[1 1 1 0.8] Drift market
  (for (_array_element _array_index) _quotes
    (bind (_product _multiplier) (break `/Game/GrandOpening/Blueprints/Structures/S_MarketQuote` _array_element))
    (bind _found (`/Game/GrandOpening/Blueprints/ActorComponents/BP_StoreManager.HasTransaction` (`self.StoreManager`) Day "NewEnumerator1" (`/Game/GrandOpening/Blueprints/DataAssets/Products/BP_ProductDataAsset.Id` _product)))
    (`KismetArrayLibrary.Array_Set` _quotes _array_index (make `/Game/GrandOpening/Blueprints/Structures/S_MarketQuote` _product (`KismetMathLibrary.FClamp` (+ (`KismetMathLibrary.SelectFloat` (+ _multiplier _demandamplitude) (`KismetMathLibrary.FInterpTo_Constant` _multiplier 1.0 1.0 _demandamplitude) _found) (`KismetMathLibrary.RandomFloatInRange` (- 0.0 _marketvolatility) _marketvolatility)) (- 1.0 _marketrange) (+ 1.0 _marketrange))))))

(fn `GetWholesalePrice`
  (params (Product :type "/Game/GrandOpening/Blueprints/DataAssets/Products/BP_ProductDataAsset Object Reference"))
  (returns (Price :type "Float (double-precision)"))
  (locals (Multiplier :type "Float (double-precision)"))
  ;[1 1 1 0.8] Get wholesale price
  (set `local.Multiplier` 1.0)
  (for _array_element (`self.Quotes`)
    (bind (_product _multiplier) (break `/Game/GrandOpening/Blueprints/Structures/S_MarketQuote` _array_element))
    (if (== _product Product)
      (set `local.Multiplier` _multiplier)))
  (return (* (`/Game/GrandOpening/Blueprints/DataAssets/Products/BP_ProductDataAsset.CostPrice` Product) (`local.Multiplier`))))

(fn `HandleDayEnded`
  (params (Day :type Integer))
  ;[1 1 1 0.8] Handle day ended
  (`self.ChargeDailyCosts` Day)
  (`self.DriftMarket` Day))

(fn `InitializeQuotes`
  ;[1 1 1 0.8] Initialize quotes
  (`KismetArrayLibrary.Array_Clear` (`self.Quotes`))
  (for _array_element (`/Game/GrandOpening/Blueprints/DataAssets/Apps/BP_MarketAppDataAsset.AvailableProducts` (`self.MarketCatalog`))
    (`KismetArrayLibrary.Array_Add` (`self.Quotes`) (make `/Game/GrandOpening/Blueprints/Structures/S_MarketQuote` _array_element))))

(fn `RestoreFromSave`
  ;[1 1 1 0.8] Restore from save
  (bind _asbp_store_game_instance (cast `/Game/GrandOpening/Blueprints/Misc/BP_StoreGameInstance` (`GameplayStatics.GetGameInstance`)))
  (bind _pendingsave (`/Game/GrandOpening/Blueprints/Misc/BP_StoreGameInstance.PendingSave` _asbp_store_game_instance))
  (`/Engine/EditorBlueprintResources/StandardMacros.IsValid` _pendingsave
    (:`Is Valid`
      (set `self.Quotes` (`/Game/GrandOpening/Blueprints/Misc/SG_StoreSave.MarketQuotes` _pendingsave)))))
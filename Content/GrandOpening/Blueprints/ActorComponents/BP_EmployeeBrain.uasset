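; Employee brain component that lets hired store staff man checkouts and stock shelves.
; It pulls role-matched tasks from BP_StoreManager, supplies move and focus points, and roams when idle.
; FinishWork runs the task as Continuing, Completed or Refused; stocking carries delivery boxes to shelves, then racks, or trashes empties.
; It locks player interaction on reserved targets, negotiates door passage and releases everything on EndPlay.
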(event `self.ReceiveEndPlay`
  (params (EndPlayReason :type "EEndPlayReason Enum" :default "Destroyed"))
  ;[1 1 1 0.8] Event end play
  (`self.ReleaseCurrentTask` self)
  (`self.LeaveCheckout`)
  (`self.DropStockBox`)
  (`self.ReleaseDoors`))

(fn `AdvanceStocking`
  (params (Box :type "/Game/GrandOpening/Blueprints/Environments/Boxes/BP_DeliveryBoxBase Object Reference"))
  (returns (Outcome :type "/Game/GrandOpening/Blueprints/Enumerations/E_TaskOutcome Enum"))
  (locals (Result :type "/Game/GrandOpening/Blueprints/Enumerations/E_TaskOutcome Enum"))
  (bind _returnvalue (`KismetSystemLibrary.GetGameTimeInSeconds`))
  (bind _stocktarget (`self.StockTarget`))
  ;[1 1 1 0.8] Advance stocking
  (set `local.Result` "NewEnumerator0")
  (cast `/Game/GrandOpening/Blueprints/Environments/Shelves/BP_ShelfBase` _stocktarget
    (:`then`
      (if (>= _returnvalue (`self.NextRestockAt`))
        (set `self.NextRestockAt` (+ _returnvalue (/ (`self.RestockSeconds`) (`/Game/GrandOpening/Blueprints/DataAssets/Employees/BP_EmployeeCandidateDataAsset.WorkSpeed` (`self.Candidate`)))))
        (bind _result (`/Game/GrandOpening/Blueprints/Environments/Boxes/BP_DeliveryBoxBase.UnloadOneInto` Box _stocktarget))
        (bind _returnvalue_2 (`/Game/GrandOpening/Blueprints/Environments/Boxes/BP_DeliveryBoxBase.IsTransferring` Box))
        (if (or _result _returnvalue_2)
          (set `local.Result` "NewEnumerator1" :!label _label)
          (else
            (bind _outcome (`self.RetargetStocking` Box))
            (set `local.Result` _outcome)))
        (else
          (goto _label))))
    (:`CastFailed`
      (bind _asbp_trash_bin (cast `/Game/GrandOpening/Blueprints/Environments/Misc/BP_TrashBin` _stocktarget)
        (:`then`
          (bind _outcome_2 (`self.DisposeStockBox` _asbp_trash_bin))
          (set `local.Result` _outcome_2))
        (:`CastFailed`
          (bind _outcome_3 (`self.StoreBoxOnRack` _stocktarget))
          (set `local.Result` _outcome_3)))))
  (return (`local.Result`)))

(fn `ApproachPointFor`
  (params (TargetActor :type "Actor Object Reference"))
  (returns (Point :type "Vector Structure"))
  (bind _returnvalue (`Actor.K2_GetActorLocation` TargetActor))
  (bind _returnvalue_2 (`self.GetOwner` self))
  (bind _returnvalue_3 (`Actor.K2_GetActorLocation` _returnvalue_2))
  (bind _returnvalue_4 (+ (`KismetMathLibrary.VSizeXY` (`.BoxExtent` (`Actor.GetActorBounds` TargetActor true false))) (`self.StandOffCm`)))
  (bind (_projectedlocation _returnvalue_5) (`NavigationSystemV1.K2_ProjectPointToNavigation` _returnvalue null null (`KismetMathLibrary.MakeVector` _returnvalue_4 _returnvalue_4 _returnvalue_4)))
  ;[1 1 1 0.8] Approach point for
  (bind _asbp_checkout_base (cast `/Game/GrandOpening/Blueprints/Environments/Checkout/BP_CheckoutBase` TargetActor)
    (:`then`
      (bind _location (`/Game/GrandOpening/Blueprints/Environments/Checkout/BP_CheckoutBase.CashierSpotLocation` _asbp_checkout_base))
      (return _location))
    (:`CastFailed`
      (return (`KismetMathLibrary.SelectVector` (`KismetMathLibrary.MakeVector` (.x (+ _returnvalue (* (`KismetMathLibrary.Vector_Normal2D` (- _returnvalue_3 _returnvalue)) _returnvalue_4))) (.y (+ _returnvalue (* (`KismetMathLibrary.Vector_Normal2D` (- _returnvalue_3 _returnvalue)) _returnvalue_4))) (.z _returnvalue_3)) (`KismetMathLibrary.SelectVector` _projectedlocation _returnvalue _returnvalue_5) (`Controller.LineOfSightTo` (`AIBlueprintHelperLibrary.GetAIController` _returnvalue_2) TargetActor (0.0 0.0 0.0) false))))))

(fn `AvoidsOthers`
  (returns (ReturnValue :type Boolean))
  ;[1 1 1 0.8] Avoids others
  (return (> (`KismetMathLibrary.Vector_Distance` (`Actor.K2_GetActorLocation` (`self.GetOwner`)) (`self.TargetLocation`)) (`self.ArrivalAvoidanceCm`))))

(fn `BeginStocking`
  (params (Target :type "Actor Object Reference"))
  (returns (Outcome :type "/Game/GrandOpening/Blueprints/Enumerations/E_TaskOutcome Enum"))
  (locals (Result :type "/Game/GrandOpening/Blueprints/Enumerations/E_TaskOutcome Enum"))
  ;[1 1 1 0.8] Begin stocking
  (set `local.Result` "NewEnumerator0")
  (bind _asbp_delivery_box_base (cast `/Game/GrandOpening/Blueprints/Environments/Boxes/BP_DeliveryBoxBase` Target)
    (:`then`
      (bind _carried (`/Game/GrandOpening/Blueprints/Environments/Boxes/BP_DeliveryBoxBase.IsCarriedByPlayer` _asbp_delivery_box_base))
      (if (not _carried)
        (bind (_destination _found) (`self.FindStockDestination` _asbp_delivery_box_base))
        (if _found
          (`self.CarryStockBox` _asbp_delivery_box_base)
          (set `self.StockTarget` _destination)
          (set `local.Result` "NewEnumerator1"))))
    (:`CastFailed`
      _))
  (return (`local.Result`)))

(fn `CarryLeftGripPoint`
  (returns (Point :type "Vector Structure"))
  (bind _carriedbox (`self.CarriedBox`))
  ;[1 1 1 0.8] Carry left grip point
  (`/Engine/EditorBlueprintResources/StandardMacros.IsValid` _carriedbox
    (:`Is Valid`
      (bind _point (`/Game/GrandOpening/Blueprints/Environments/Boxes/BP_DeliveryBoxBase.LeftGripPoint` _carriedbox (`self.CarryHandOffsetCm`)))
      (return _point))))

(fn `CarryStockBox`
  (params (Box :type "/Game/GrandOpening/Blueprints/Environments/Boxes/BP_DeliveryBoxBase Object Reference"))
  ;[1 1 1 0.8] Carry stock box
  (`/Game/GrandOpening/Blueprints/Environments/Boxes/BP_DeliveryBoxBase.AttachBoxTo` Box (`Actor.GetComponentByClass` (`self.GetOwner`) "/Script/Engine.SkeletalMeshComponent") (`self.CarrySocket`) (`self.CarryHandOffsetCm`))
  (set `self.CarriedBox` Box)
  (bind _open (`/Game/GrandOpening/Blueprints/Environments/Boxes/BP_DeliveryBoxBase.IsBoxOpen` Box))
  (if (not _open)
    (`/Game/GrandOpening/Blueprints/Environments/Boxes/BP_DeliveryBoxBase.ToggleOpen` Box)))

(fn `ChooseRoamPoint`
  (returns (RoamPoint :type "Vector Structure"))
  (locals (Point :type "Vector Structure"))
  ;[1 1 1 0.8] Choose roam point
  (set `local.Point` (`Actor.K2_GetActorLocation` (`self.GetOwner` self)))
  (bind _volume (`/Game/GrandOpening/Blueprints/Functions/BFL_Zones.FindZoneVolume` "NewEnumerator0" self))
  (`/Engine/EditorBlueprintResources/StandardMacros.IsValid` _volume
    (:`Is Valid`
      (bind (_point _found) (`/Game/GrandOpening/Blueprints/Environments/Build/BP_StoreZoneVolume.RandomNavigablePoint` _volume))
      (if _found
        (set `local.Point` _point)))
    (:`Is Not Valid`
      _))
  (return (`local.Point`)))

(fn `CurrentWorkTarget`
  (returns (Target :type "Actor Object Reference"))
  (locals (Picked :type "Actor Object Reference"))
  (bind _stocktarget (`self.StockTarget`))
  ;[1 1 1 0.8] Current work target
  (set `local.Picked` (`.Target_9_7D3E28B343CA528FCE132590CD40F0A5` (break `/Game/GrandOpening/Blueprints/Structures/S_StoreTask` (`self.CurrentTask`))))
  (`/Engine/EditorBlueprintResources/StandardMacros.IsValid` _stocktarget
    (:`Is Valid`
      (set `local.Picked` _stocktarget))
    (:`Is Not Valid`
      _))
  (return (`local.Picked`)))

(fn `DisposeStockBox`
  (params (Bin :type "/Game/GrandOpening/Blueprints/Environments/Misc/BP_TrashBin Object Reference"))
  (returns (Outcome :type "/Game/GrandOpening/Blueprints/Enumerations/E_TaskOutcome Enum"))
  ;[1 1 1 0.8] Dispose stock box
  (`/Game/GrandOpening/Blueprints/Environments/Misc/BP_TrashBin.Dispose` Bin (`self.CarriedBox`))
  (set `self.StockTarget` null)
  (set `self.CarriedBox` null)
  (return "NewEnumerator0"))

(fn `DropStockBox`
  (locals (Dropped :type "/Game/GrandOpening/Blueprints/Environments/Boxes/BP_DeliveryBoxBase Object Reference"))
  ;[1 1 1 0.8] Drop stock box
  (set `local.Dropped` (`self.CarriedBox`))
  (set `self.StockTarget` null)
  (set `self.CarriedBox` null)
  (`/Engine/EditorBlueprintResources/StandardMacros.IsValid` (`local.Dropped`)
    (:`Is Valid`
      (`/Game/GrandOpening/Blueprints/Environments/Boxes/BP_DeliveryBoxBase.DetachBoxFromCarrier` (`local.Dropped`)))))

(fn `FindStockDestination`
  (params (Box :type "/Game/GrandOpening/Blueprints/Environments/Boxes/BP_DeliveryBoxBase Object Reference"))
  (returns (Destination :type "Actor Object Reference") (Found :type Boolean))
  (locals (Pick :type "Actor Object Reference") (Picked :type Boolean) (BestDistanceCm :type "Float (double-precision)"))
  ;[1 1 1 0.8] Find stock destination
  (set `local.Picked` false)
  (bind _result (`/Game/GrandOpening/Blueprints/Environments/Boxes/BP_DeliveryBoxBase.HasUnit` Box))
  (if _result
    (bind _outactors (`GameplayStatics.GetAllActorsOfClass` "/Game/GrandOpening/Blueprints/Environments/Shelves/BP_ShelfBase.BP_ShelfBase_C"))
    (for _array_element _outactors
      (if (not (`local.Picked`))
        (bind _hasroom (`/Game/GrandOpening/Blueprints/Environments/Shelves/BP_ShelfBase.HasRoomFor` _array_element (`/Game/GrandOpening/Blueprints/Environments/Boxes/BP_DeliveryBoxBase.Product` Box)))
        (if _hasroom
          (set `local.Pick` _array_element)
          (set `local.Picked` true))))
    (if (not (`local.Picked`))
      (bind _outactors_2 (`GameplayStatics.GetAllActorsOfClass` "/Game/GrandOpening/Blueprints/Environments/Shelves/BP_StorageRack.BP_StorageRack_C"))
      (for _array_element_2 _outactors_2
        (if (not (`local.Picked`))
          (bind (_slot _found) (`/Game/GrandOpening/Blueprints/Environments/Shelves/BP_StorageRack.FindFreeSlotFor` _array_element_2 Box))
          (if _found
            (set `local.Pick` _array_element_2)
            (set `local.Picked` true))))))
  (if (not _result)
    (bind _outactors_3 (`GameplayStatics.GetAllActorsOfClass` "/Game/GrandOpening/Blueprints/Environments/Misc/BP_TrashBin.BP_TrashBin_C"))
    (for _array_element_3 _outactors_3
      (bind _returnvalue (`Actor.GetDistanceTo` (`self.GetOwner`) _array_element_3))
      (if (or (not (`local.Picked`)) (< _returnvalue (`local.BestDistanceCm`)))
        (set `local.Pick` _array_element_3)
        (set `local.BestDistanceCm` _returnvalue)
        (set `local.Picked` true))))
  (return (`local.Pick`) (`local.Picked`)))

(fn `FinishWork`
  ;[1 1 1 0.8] Finish work
  (if (`self.HasTask`)
    (bind _outcome (`self.PerformTask`))
    (switch `/Game/GrandOpening/Blueprints/Enumerations/E_TaskOutcome` _outcome
      (:`NewEnumerator0`
        (set `self.HasTask` false)
        (`/Game/GrandOpening/Blueprints/ActorComponents/BP_StoreManager.CompleteTask` (`self.StoreManager`) (`self.GetOwner`)))
      (:`NewEnumerator2`
        (set `self.HasTask` false)
        (`/Game/GrandOpening/Blueprints/ActorComponents/BP_StoreManager.ReleaseTaskOf` (`self.StoreManager`) (`self.GetOwner`))))))

(fn `GetFocusPoint`
  (returns (Point :type "Vector Structure") (HasFocus :type Boolean))
  ;[1 1 1 0.8] Get focus point
  (if (`self.HasTask`)
    (bind _target (`self.CurrentWorkTarget`))
    (`/Engine/EditorBlueprintResources/StandardMacros.IsValid` _target
      (:`Is Valid`
        (return (+ (`Actor.K2_GetActorLocation` _target) (`KismetMathLibrary.MakeVector` 0.0 0.0 (`self.EyeHeightCm`))) true))
      (:`Is Not Valid`
        _)))
  (return (0.0 0.0 0.0) false))

(fn `HoldsPosition`
  (returns (ReturnValue :type Boolean))
  (locals (Held :type Boolean))
  ;[1 1 1 0.8] Holds position
  (set `local.Held` false)
  (for _array_element (`self.Doors`)
    (bind _returnvalue (`/Game/GrandOpening/Blueprints/Environments/Openings/BP_EntranceDoor.RequestPassage` _array_element (`self.GetOwner`) (`self.TargetLocation`)))
    (if (not _returnvalue)
      (set `local.Held` true)))
  (return (`local.Held`)))

(fn `InitializeEmployee`
  (params (NewCandidate :type "/Game/GrandOpening/Blueprints/DataAssets/Employees/BP_EmployeeCandidateDataAsset Object Reference"))
  (bind _returnvalue (`self.GetOwner` self))
  ;[1 1 1 0.8] Initialize employee
  (set `self.Candidate` NewCandidate)
  (set `self.StoreManager` (`Actor.GetComponentByClass` (`GameplayStatics.GetGameState`) "/Game/GrandOpening/Blueprints/ActorComponents/BP_StoreManager.BP_StoreManager_C"))
  (set `CharacterMovementComponent.MaxWalkSpeed` (`/Game/GrandOpening/Blueprints/DataAssets/Employees/BP_EmployeeCandidateDataAsset.WalkSpeed` NewCandidate) (`Actor.GetComponentByClass` _returnvalue "/Script/Engine.CharacterMovementComponent"))
  (`/Game/GrandOpening/Blueprints/ActorComponents/BP_CosmeticComponent.ApplyCosmeticSet` (`Actor.GetComponentByClass` _returnvalue "/Game/GrandOpening/Blueprints/ActorComponents/BP_CosmeticComponent.BP_CosmeticComponent_C") (`/Game/GrandOpening/Blueprints/DataAssets/Employees/BP_EmployeeCandidateDataAsset.CosmeticSet` NewCandidate))
  (`self.OnInitialized`)
  (bind _outactors (`GameplayStatics.GetAllActorsOfClass` "/Game/GrandOpening/Blueprints/Environments/Openings/BP_EntranceDoor.BP_EntranceDoor_C"))
  (set `self.Doors` _outactors))

(fn `IsCarryingBox`
  (returns (Carrying :type Boolean))
  (locals (Held :type Boolean))
  ;[1 1 1 0.8] Is carrying box
  (set `local.Held` false)
  (`/Engine/EditorBlueprintResources/StandardMacros.IsValid` (`self.CarriedBox`)
    (:`Is Valid`
      (set `local.Held` true))
    (:`Is Not Valid`
      _))
  (return (`local.Held`)))

(fn `LeaveCheckout`
  (bind _mannedcheckout (`self.MannedCheckout`))
  (bind _pairedscanner (`/Game/GrandOpening/Blueprints/Environments/Checkout/BP_CheckoutBase.PairedScanner` _mannedcheckout))
  ;[1 1 1 0.8] Leave checkout
  (`/Engine/EditorBlueprintResources/StandardMacros.IsValid` _mannedcheckout
    (:`Is Valid`
      (`/Game/GrandOpening/Blueprints/Environments/Checkout/BP_CheckoutBase.ReleaseCashier` _mannedcheckout (`self.GetOwner`))
      (`/Engine/EditorBlueprintResources/StandardMacros.IsValid` _pairedscanner
        (:`Is Valid`
          (`/Game/GrandOpening/Blueprints/Environments/Tools/BP_BarcodeScanner.ReleaseFromHand` _pairedscanner))
        (:`Is Not Valid`
          _)))
    (:`Is Not Valid`
      _))
  (set `self.MannedCheckout` null))

(fn `PerformTask`
  (returns (Outcome :type "/Game/GrandOpening/Blueprints/Enumerations/E_TaskOutcome Enum"))
  (locals (Result :type "/Game/GrandOpening/Blueprints/Enumerations/E_TaskOutcome Enum"))
  (bind (_type _target) (break `/Game/GrandOpening/Blueprints/Structures/S_StoreTask` (`self.CurrentTask`)))
  ;[1 1 1 0.8] Perform task
  (set `local.Result` "NewEnumerator0")
  (`/Engine/EditorBlueprintResources/StandardMacros.IsValid` _target
    (:`Is Valid`
      (switch `/Game/GrandOpening/Blueprints/Enumerations/E_TaskType` _type
        (:`NewEnumerator2`
          (bind _outcome (`self.WorkManCheckout` _target))
          (set `local.Result` _outcome))
        (:`NewEnumerator4`
          (bind _outcome_2 (`self.WorkStockShelves` _target))
          (set `local.Result` _outcome_2))))
    (:`Is Not Valid`
      _))
  (return (`local.Result`)))

(fn `ReleaseCurrentTask`
  ;[1 1 1 0.8] Release current task
  (if (`self.HasTask`)
    (`/Game/GrandOpening/Blueprints/ActorComponents/BP_StoreManager.ReleaseTaskOf` (`self.StoreManager`) (`self.GetOwner`))
    (set `self.HasTask` false))
  (`self.UpdateReservation`))

(fn `ReleaseDoors`
  ;[1 1 1 0.8] Release doors
  (for _array_element (`self.Doors`)
    (`/Game/GrandOpening/Blueprints/Environments/Openings/BP_EntranceDoor.ReleasePassage` _array_element (`self.GetOwner`))))

(fn `RetargetStocking`
  (params (Box :type "/Game/GrandOpening/Blueprints/Environments/Boxes/BP_DeliveryBoxBase Object Reference"))
  (returns (Outcome :type "/Game/GrandOpening/Blueprints/Enumerations/E_TaskOutcome Enum"))
  (locals (Result :type "/Game/GrandOpening/Blueprints/Enumerations/E_TaskOutcome Enum"))
  ;[1 1 1 0.8] Retarget stocking
  (bind (_destination _found) (`self.FindStockDestination` Box))
  (set `local.Result` "NewEnumerator0")
  (if _found
    (set `self.StockTarget` _destination)
    (set `local.Result` "NewEnumerator1")
    (else
      (`self.DropStockBox`)
      (bind _result (`/Game/GrandOpening/Blueprints/Environments/Boxes/BP_DeliveryBoxBase.HasUnit` Box))
      (if (not _result)
        (`/Game/GrandOpening/Blueprints/ActorComponents/BP_ReactionComponent.React` (`Actor.GetComponentByClass` (`self.GetOwner`) "/Game/GrandOpening/Blueprints/ActorComponents/BP_ReactionComponent.BP_ReactionComponent_C") "NewEnumerator3" ""))))
  (return (`local.Result`)))

(fn `SetReservation`
  (params (Wanted :type "Actor Object Reference"))
  ;[1 1 1 0.8] Set reservation
  (if (!= (`self.Reserved`) Wanted)
    (`/Engine/EditorBlueprintResources/StandardMacros.IsValid` (`self.Reserved`)
      (:`Is Valid`
        (`/Game/GrandOpening/Blueprints/ActorComponents/BP_InteractableComponent.SetInteractable` (`Actor.GetComponentByClass` (`self.Reserved`) "/Game/GrandOpening/Blueprints/ActorComponents/BP_InteractableComponent.BP_InteractableComponent_C") true))
      (:`Is Not Valid`
        _))
    (set `self.Reserved` Wanted)
    (`/Engine/EditorBlueprintResources/StandardMacros.IsValid` Wanted
      (:`Is Valid`
        (`/Game/GrandOpening/Blueprints/ActorComponents/BP_InteractableComponent.SetInteractable` (`Actor.GetComponentByClass` Wanted "/Game/GrandOpening/Blueprints/ActorComponents/BP_InteractableComponent.BP_InteractableComponent_C") false)))))

(fn `StoreBoxOnRack`
  (params (Rack :type "Actor Object Reference"))
  (returns (Outcome :type "/Game/GrandOpening/Blueprints/Enumerations/E_TaskOutcome Enum"))
  (locals (Result :type "/Game/GrandOpening/Blueprints/Enumerations/E_TaskOutcome Enum"))
  (bind _carriedbox (`self.CarriedBox`))
  ;[1 1 1 0.8] Store box on rack
  (set `local.Result` "NewEnumerator0")
  (bind _asbp_storage_rack (cast `/Game/GrandOpening/Blueprints/Environments/Shelves/BP_StorageRack` Rack)
    (:`then`
      (bind (_slot _found) (`/Game/GrandOpening/Blueprints/Environments/Shelves/BP_StorageRack.FindFreeSlotFor` _asbp_storage_rack _carriedbox))
      (if _found
        (`/Game/GrandOpening/Blueprints/Environments/Boxes/BP_DeliveryBoxBase.PlaceBoxInSlot` _carriedbox _slot)
        (set `self.StockTarget` null)
        (set `self.CarriedBox` null)
        (else
          (bind _outcome (`self.RetargetStocking` _carriedbox))
          (set `local.Result` _outcome))))
    (:`CastFailed`
      (`self.DropStockBox`)))
  (return (`local.Result`)))

(fn `UpdateReservation`
  (bind (_type _target) (break `/Game/GrandOpening/Blueprints/Structures/S_StoreTask` (`self.CurrentTask`)))
  ;[1 1 1 0.8] Update reservation
  (if (`self.HasTask`)
    (bind _asbp_checkout_base (cast `/Game/GrandOpening/Blueprints/Environments/Checkout/BP_CheckoutBase` _target)
      (:`then`
        (`self.SetReservation` (`/Game/GrandOpening/Blueprints/Environments/Checkout/BP_CheckoutBase.PairedScanner` _asbp_checkout_base)))
      (:`CastFailed`
        (`self.SetReservation` _target)))
    (else
      (`self.SetReservation` null))))

(fn `UpdateTarget`
  (bind _returnvalue (`KismetSystemLibrary.GetGameTimeInSeconds`))
  (bind _returnvalue_2 (`self.GetOwner` self))
  ;[1 1 1 0.8] Update target
  (if (not (`self.HasTask`))
    (bind (_task _found) (`/Game/GrandOpening/Blueprints/ActorComponents/BP_StoreManager.PullTaskForRoles` (`self.StoreManager`) (`/Game/GrandOpening/Blueprints/DataAssets/Employees/BP_EmployeeCandidateDataAsset.Roles` (`self.Candidate`)) _returnvalue_2))
    (if _found
      (set `self.CurrentTask` _task)
      (set `self.HasTask` true)))
  (`self.UpdateReservation`)
  (bind _target (`self.CurrentWorkTarget`))
  (if (`self.HasTask`)
    (`/Engine/EditorBlueprintResources/StandardMacros.IsValid` _target
      (:`Is Valid`
        (bind _point (`self.ApproachPointFor` self _target))
        (set `self.TargetLocation` _point))
      (:`Is Not Valid`
        (set `self.TargetLocation` (`Actor.K2_GetActorLocation` _returnvalue_2))))
    (else
      (`/Engine/EditorBlueprintResources/StandardMacros.IsValid` (`self.MannedCheckout`)
        (:`Is Not Valid`
          (if (>= _returnvalue (`self.RoamUntil`))
            (set `self.RoamUntil` (+ _returnvalue (`self.RoamLegSeconds`)))
            (bind _roampoint (`self.ChooseRoamPoint`))
            (set `self.TargetLocation` _roampoint)
            (`/Game/GrandOpening/Blueprints/ActorComponents/BP_ReactionComponent.React` (`Actor.GetComponentByClass` _returnvalue_2 "/Game/GrandOpening/Blueprints/ActorComponents/BP_ReactionComponent.BP_ReactionComponent_C") "NewEnumerator0" "")))))))

(fn `WorkManCheckout`
  (params (Target :type "Actor Object Reference"))
  (returns (Outcome :type "/Game/GrandOpening/Blueprints/Enumerations/E_TaskOutcome Enum"))
  (bind _returnvalue (`self.GetOwner`))
  (bind _mannedcheckout (`self.MannedCheckout`))
  ;[1 1 1 0.8] Work man checkout
  (bind _asbp_checkout_base (cast `/Game/GrandOpening/Blueprints/Environments/Checkout/BP_CheckoutBase` Target)
    (:`then`
      (bind _returnvalue_2 (== _mannedcheckout _asbp_checkout_base))
      (if (not _returnvalue_2)
        (bind _pairedscanner (`/Game/GrandOpening/Blueprints/Environments/Checkout/BP_CheckoutBase.PairedScanner` _asbp_checkout_base))
        (`/Engine/EditorBlueprintResources/StandardMacros.IsValid` _pairedscanner
          (:`Is Valid`
            (`self.LeaveCheckout`)
            (bind _claimed (`/Game/GrandOpening/Blueprints/Environments/Checkout/BP_CheckoutBase.TryClaimCashier` _asbp_checkout_base _returnvalue))
            (if _claimed
              (set `self.MannedCheckout` _asbp_checkout_base)
              (`/Game/GrandOpening/Blueprints/Environments/Checkout/BP_CheckoutBase.SetOpen` _asbp_checkout_base true)
              (`/Game/GrandOpening/Blueprints/Environments/Tools/BP_BarcodeScanner.AttachToHand` _pairedscanner (`Actor.GetComponentByClass` _returnvalue "/Script/Engine.SkeletalMeshComponent") (`self.ScannerSocket`))))
          (:`Is Not Valid`
            _))))
    (:`CastFailed`
      _))
  (return (select `bool` (and _returnvalue_2 (!= _mannedcheckout null)) :`false` "NewEnumerator2" :`true` "NewEnumerator1" :!type "/Game/GrandOpening/Blueprints/Enumerations/E_TaskOutcome Enum")))

(fn `WorkStockShelves`
  (params (Target :type "Actor Object Reference"))
  (returns (Outcome :type "/Game/GrandOpening/Blueprints/Enumerations/E_TaskOutcome Enum"))
  (locals (Result :type "/Game/GrandOpening/Blueprints/Enumerations/E_TaskOutcome Enum"))
  (bind _carriedbox (`self.CarriedBox`))
  ;[1 1 1 0.8] Work stock shelves
  (set `local.Result` "NewEnumerator0")
  (`/Engine/EditorBlueprintResources/StandardMacros.IsValid` _carriedbox
    (:`Is Valid`
      (bind _outcome (`self.AdvanceStocking` _carriedbox))
      (set `local.Result` _outcome))
    (:`Is Not Valid`
      (bind _outcome_2 (`self.BeginStocking` Target))
      (set `local.Result` _outcome_2)))
  (return (`local.Result`)))
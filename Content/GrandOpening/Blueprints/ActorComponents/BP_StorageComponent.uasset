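; Storage component that manages the product units held on its owner's BP_StorageRow components, collected at begin play.
; Queries and add/remove operations use the first row that fits or holds the product, while counts and stocked products span all rows.
; Each change rebuilds every row's collision-free instanced static mesh, created on demand, from that row's product mesh and unit transforms.
; Next and top unit transforms expose where a unit lands or leaves.
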(event `self.ReceiveBeginPlay`
  ;[1 1 1 0.8] Event begin play
  (`self.CollectRows` self))

(fn `AddRowInstances`
  (params (Row :type "/Game/GrandOpening/Blueprints/ActorComponents/BP_StorageRow Object Reference"))
  (bind _count (`/Game/GrandOpening/Blueprints/ActorComponents/BP_StorageRow.Count` Row))
  (bind _instances (`/Game/GrandOpening/Blueprints/ActorComponents/BP_StorageRow.Instances` Row))
  ;[1 1 1 0.8] Add row instances
  (`/Engine/EditorBlueprintResources/StandardMacros.IsValid` _instances
    (:`Is Valid`
      (`self.FillRow` self Row _instances _count))
    (:`Is Not Valid`
      (bind _returnvalue (`|AddComponentByClass` :`self` (`self.GetOwner` self) :`Class` "/Script/Engine.InstancedStaticMeshComponent"))
      (`self.K2_AttachToComponent` _returnvalue self "None" "KeepRelative" "KeepRelative" "KeepRelative" true)
      (`PrimitiveComponent.SetCollisionEnabled` _returnvalue "NoCollision")
      (set `/Game/GrandOpening/Blueprints/ActorComponents/BP_StorageRow.Instances` _returnvalue Row)
      (`self.FillRow` self Row _returnvalue _count))))

(fn `AddUnit`
  (params (Product :type "/Game/GrandOpening/Blueprints/DataAssets/Products/BP_ProductDataAsset Object Reference"))
  ;[1 1 1 0.8] Add unit
  (for _array_element (`self.Rows`)
    (bind _hasroom (`/Game/GrandOpening/Blueprints/ActorComponents/BP_StorageRow.HasRoomFor` _array_element Product))
    (if _hasroom
      (`/Game/GrandOpening/Blueprints/ActorComponents/BP_StorageRow.AddUnit` _array_element Product)
      (break)))
  (`self.RefreshInstances` self))

(fn `CollectRows`
  ;[1 1 1 0.8] Collect rows
  (`KismetArrayLibrary.Array_Clear` (`self.Rows`))
  (for _array_element (`Actor.K2_GetComponentsByClass` (`self.GetOwner` self) "/Game/GrandOpening/Blueprints/ActorComponents/BP_StorageRow.BP_StorageRow_C")
    (`KismetArrayLibrary.Array_Add` (`self.Rows`) _array_element)))

(fn `CountOf`
  (params (Product :type "/Game/GrandOpening/Blueprints/DataAssets/Products/BP_ProductDataAsset Object Reference"))
  (returns (Units :type Integer))
  (locals (Total :type Integer))
  ;[1 1 1 0.8] Count of
  (set `local.Total` 0)
  (for _array_element (`self.Rows`)
    (bind _hasunit (`/Game/GrandOpening/Blueprints/ActorComponents/BP_StorageRow.HasUnitOf` _array_element Product))
    (if _hasunit
      (set `local.Total` (+ (`local.Total`) (`/Game/GrandOpening/Blueprints/ActorComponents/BP_StorageRow.Count` _array_element)))))
  (return (`local.Total`)))

(fn `FillRow`
  (params (Row :type "/Game/GrandOpening/Blueprints/ActorComponents/BP_StorageRow Object Reference") (Ism :type "InstancedStaticMeshComponent Object Reference") (Count :type Integer))
  (bind _product (`/Game/GrandOpening/Blueprints/ActorComponents/BP_StorageRow.Product` Row))
  ;[1 1 1 0.8] Fill row
  (`InstancedStaticMeshComponent.ClearInstances` Ism)
  (if (> Count 0)
    (`StaticMeshComponent.SetStaticMesh` Ism (`/Game/GrandOpening/Blueprints/DataAssets/Products/BP_ProductDataAsset.Mesh` _product))
    (for _index (range Count)
      (bind _placement (`/Game/GrandOpening/Blueprints/ActorComponents/BP_StorageRow.UnitTransform` Row _product _index))
      (`InstancedStaticMeshComponent.AddInstance` Ism _placement true))))

(fn `HasRoomFor`
  (params (Product :type "/Game/GrandOpening/Blueprints/DataAssets/Products/BP_ProductDataAsset Object Reference"))
  (returns (HasRoom :type Boolean))
  ;[1 1 1 0.8] Has room for
  (for _array_element (`self.Rows`)
    (bind _hasroom (`/Game/GrandOpening/Blueprints/ActorComponents/BP_StorageRow.HasRoomFor` _array_element Product))
    (if _hasroom
      (return true)))
  (return false))

(fn `HasUnitOf`
  (params (Product :type "/Game/GrandOpening/Blueprints/DataAssets/Products/BP_ProductDataAsset Object Reference"))
  (returns (HasUnit :type Boolean))
  ;[1 1 1 0.8] Has unit of
  (for _array_element (`self.Rows`)
    (bind _hasunit (`/Game/GrandOpening/Blueprints/ActorComponents/BP_StorageRow.HasUnitOf` _array_element Product))
    (if _hasunit
      (return true)))
  (return false))

(fn `NextUnitTransform`
  (params (Product :type "/Game/GrandOpening/Blueprints/DataAssets/Products/BP_ProductDataAsset Object Reference"))
  (returns (Placement :type "Transform Structure"))
  ;[1 1 1 0.8] Next unit transform
  (for _array_element (`self.Rows`)
    (bind _hasroom (`/Game/GrandOpening/Blueprints/ActorComponents/BP_StorageRow.HasRoomFor` _array_element Product))
    (if _hasroom
      (bind _placement (`/Game/GrandOpening/Blueprints/ActorComponents/BP_StorageRow.UnitTransform` _array_element Product (`/Game/GrandOpening/Blueprints/ActorComponents/BP_StorageRow.Count` _array_element)))
      (return _placement)))
  (return))

(fn `RefreshInstances`
  ;[1 1 1 0.8] Refresh instances
  (for _array_element (`self.Rows`)
    (`self.AddRowInstances` self _array_element)))

(fn `RemoveUnit`
  (params (Product :type "/Game/GrandOpening/Blueprints/DataAssets/Products/BP_ProductDataAsset Object Reference"))
  ;[1 1 1 0.8] Remove unit
  (for _array_element (`self.Rows`)
    (bind _hasunit (`/Game/GrandOpening/Blueprints/ActorComponents/BP_StorageRow.HasUnitOf` _array_element Product))
    (if _hasunit
      (`/Game/GrandOpening/Blueprints/ActorComponents/BP_StorageRow.RemoveUnit` _array_element)
      (break)))
  (`self.RefreshInstances` self))

(fn `StockedProducts`
  (returns (Products :type "Array of /Game/GrandOpening/Blueprints/DataAssets/Products/BP_ProductDataAsset Object Reference"))
  (locals (Stocked :type "Array of /Game/GrandOpening/Blueprints/DataAssets/Products/BP_ProductDataAsset Object Reference"))
  ;[1 1 1 0.8] Stocked products
  (for _array_element (`self.Rows`)
    (if (> (`/Game/GrandOpening/Blueprints/ActorComponents/BP_StorageRow.Count` _array_element) 0)
      (`KismetArrayLibrary.Array_AddUnique` (`local.Stocked`) (`/Game/GrandOpening/Blueprints/ActorComponents/BP_StorageRow.Product` _array_element))))
  (return (`local.Stocked`)))

(fn `TopUnitTransform`
  (params (Product :type "/Game/GrandOpening/Blueprints/DataAssets/Products/BP_ProductDataAsset Object Reference"))
  (returns (Placement :type "Transform Structure"))
  ;[1 1 1 0.8] Top unit transform
  (for _array_element (`self.Rows`)
    (bind _hasunit (`/Game/GrandOpening/Blueprints/ActorComponents/BP_StorageRow.HasUnitOf` _array_element Product))
    (if _hasunit
      (bind _placement (`/Game/GrandOpening/Blueprints/ActorComponents/BP_StorageRow.UnitTransform` _array_element Product (- (`/Game/GrandOpening/Blueprints/ActorComponents/BP_StorageRow.Count` _array_element) 1)))
      (return _placement)))
  (return))
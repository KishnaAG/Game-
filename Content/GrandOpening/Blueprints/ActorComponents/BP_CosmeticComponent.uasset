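; Actor component that dresses its owning Character in a randomized outfit from a cosmetic set.
; ApplyCosmeticSet adds a skeletal mesh component for each slot with options, attached to the character's mesh with collision disabled.
; Each piece follows the body's animation through leader pose.
; The random option is rolled separately for the validity check and the mesh assignment, so the two can differ.
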(fn `ApplyCosmeticSet`
  (params (CosmeticSet :type "/Game/GrandOpening/Blueprints/DataAssets/Cosmetics/BP_CosmeticSetDataAsset Object Reference"))
  ;[1 1 1 0.8] Apply cosmetic set
  (`/Engine/EditorBlueprintResources/StandardMacros.IsValid` CosmeticSet
    (:`Is Valid`
      (bind _ascharacter (cast `Character` (`self.GetOwner` self)))
      (for _array_element (`/Game/GrandOpening/Blueprints/DataAssets/Cosmetics/BP_CosmeticSetDataAsset.Slots` CosmeticSet)
        (bind _options (`/Game/GrandOpening/Blueprints/DataAssets/Cosmetics/BP_CosmeticSlotDataAsset.Options` _array_element))
        (bind _returnvalue (`KismetArrayLibrary.Array_Length` _options))
        (if (> _returnvalue 0)
          (bind _output (`|GetArrayItem` _options (`KismetMathLibrary.RandomIntegerInRange` 0 (- _returnvalue 1))))
          (`/Engine/EditorBlueprintResources/StandardMacros.IsValid` _output
            (:`Is Valid`
              (bind _returnvalue_2 (`|AddComponentByClass` :`self` _ascharacter :`Class` "/Script/Engine.SkeletalMeshComponent"))
              (bind _mesh (`Character.Mesh` _ascharacter))
              (`SceneComponent.K2_AttachToComponent` _returnvalue_2 _mesh "None" "SnapToTarget" "SnapToTarget" "SnapToTarget" true)
              (`SkinnedMeshComponent.SetSkinnedAssetAndUpdate` _returnvalue_2 _output true)
              (`SkinnedMeshComponent.SetLeaderPoseComponent` _returnvalue_2 _mesh false false)
              (`PrimitiveComponent.SetCollisionEnabled` _returnvalue_2 "NoCollision"))))))))
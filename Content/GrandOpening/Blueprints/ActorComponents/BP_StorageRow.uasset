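; BP_StorageRow is a spline-based component that models a storage row holding stacked units of one product type at a time.
; Capacity is units along the spline, deep and up, derived from product footprint, stack limits, row depth and clearance.
; UnitTransform maps a unit index to a world slot following the spline, uniformly shrinking units taller than the clearance.
; Add and remove functions track only a count and product, clearing the product when empty.
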(fn `AddUnit`
  (params (Product :type "/Game/GrandOpening/Blueprints/DataAssets/Products/BP_ProductDataAsset Object Reference"))
  ;[1 1 1 0.8] Add unit
  (set `self.Product` Product)
  (set `self.Count` (+ (`self.Count`) 1)))

(fn `GetCapacity`
  (params (Product :type "/Game/GrandOpening/Blueprints/DataAssets/Products/BP_ProductDataAsset Object Reference"))
  (returns (Units :type Integer))
  ;[1 1 1 0.8] Get capacity
  (bind _units (`self.UnitsAlong` self Product))
  (bind _units_2 (`self.UnitsDeep` self Product))
  (bind _returnvalue (`self.UnitsUp` self Product))
  (return (* (* _units _units_2) _returnvalue)))

(fn `HasRoomFor`
  (params (Product :type "/Game/GrandOpening/Blueprints/DataAssets/Products/BP_ProductDataAsset Object Reference"))
  (returns (HasRoom :type Boolean))
  (bind _count (`self.Count`))
  ;[1 1 1 0.8] Has room for
  (if (and (> _count 0) (!= (`self.Product`) Product))
    (return false)
    (else
      (bind _units (`self.GetCapacity` self Product))
      (return (< _count _units)))))

(fn `HasUnitOf`
  (params (Product :type "/Game/GrandOpening/Blueprints/DataAssets/Products/BP_ProductDataAsset Object Reference"))
  (returns (HasUnit :type Boolean))
  ;[1 1 1 0.8] Has unit of
  (return (and (> (`self.Count`) 0) (== (`self.Product`) Product))))

(fn `RemoveUnit`
  (bind _count (`self.Count`))
  ;[1 1 1 0.8] Remove unit
  (if (> _count 1)
    (set `self.Count` (- _count 1))
    (else
      (set `self.Count` 0)
      (set `self.Product` null))))

(fn `UnitsAlong`
  (params (Product :type "/Game/GrandOpening/Blueprints/DataAssets/Products/BP_ProductDataAsset Object Reference"))
  (returns (Units :type Integer))
  ;[1 1 1 0.8] Unit along
  (return (`KismetMathLibrary.Max` 1 (`KismetMathLibrary.FFloor` (/ (`self.GetSplineLength` self) (`KismetMathLibrary.BreakVector2D` (`/Game/GrandOpening/Blueprints/DataAssets/Products/BP_ProductDataAsset.FootprintCm` Product)))))))

(fn `UnitsDeep`
  (params (Product :type "/Game/GrandOpening/Blueprints/DataAssets/Products/BP_ProductDataAsset Object Reference"))
  (returns (Units :type Integer))
  ;[1 1 1 0.8] Units deep
  (return (`KismetMathLibrary.Max` 1 (`KismetMathLibrary.FFloor` (/ (`self.DepthCm`) (`.Y` (`KismetMathLibrary.BreakVector2D` (`/Game/GrandOpening/Blueprints/DataAssets/Products/BP_ProductDataAsset.FootprintCm` Product))))))))

(fn `UnitsUp`
  (params (Product :type "/Game/GrandOpening/Blueprints/DataAssets/Products/BP_ProductDataAsset Object Reference"))
  (returns (ReturnValue :type Integer))
  ;[1 1 1 0.8] Units up
  (return (`KismetMathLibrary.Max` 1 (`KismetMathLibrary.Min` (`/Game/GrandOpening/Blueprints/DataAssets/Products/BP_ProductDataAsset.StackMax` Product) (`KismetMathLibrary.FFloor` (/ (`self.ClearanceCm`) (`/Game/GrandOpening/Blueprints/DataAssets/Products/BP_ProductDataAsset.StackHeightCm` Product)))))))

(fn `UnitTransform`
  (params (Product :type "/Game/GrandOpening/Blueprints/DataAssets/Products/BP_ProductDataAsset Object Reference") (UnitIndex :type Integer))
  (returns (Placement :type "Transform Structure"))
  (bind _stackheightcm (`/Game/GrandOpening/Blueprints/DataAssets/Products/BP_ProductDataAsset.StackHeightCm` Product))
  (bind (_x _y) (`KismetMathLibrary.BreakVector2D` (`/Game/GrandOpening/Blueprints/DataAssets/Products/BP_ProductDataAsset.FootprintCm` Product)))
  (bind _returnvalue (`KismetMathLibrary.FMin` 1.0 (/ (`self.ClearanceCm`) _stackheightcm)))
  ;[1 1 1 0.8] Unit transform
  (bind _units (`self.UnitsAlong` self Product))
  (bind _units_2 (`self.UnitsDeep` self Product))
  (bind _returnvalue_2 (* _units _units_2))
  (bind _returnvalue_3 (mod UnitIndex _returnvalue_2))
  (bind _returnvalue_4 (* _x (+ (`KismetMathLibrary.Conv_IntToDouble` (mod _returnvalue_3 _units)) 0.5)))
  (return (`KismetMathLibrary.MakeTransform` (+ (+ (`self.GetLocationAtDistanceAlongSpline` self _returnvalue_4 "World") (* (`self.GetRightVectorAtDistanceAlongSpline` self _returnvalue_4 "World") (* _y (+ (`KismetMathLibrary.Conv_IntToDouble` (/ _returnvalue_3 _units)) 0.5)))) (* (`self.GetUpVectorAtDistanceAlongSpline` self _returnvalue_4 "World") (* _stackheightcm (`KismetMathLibrary.Conv_IntToDouble` (/ UnitIndex _returnvalue_2))))) (`self.GetRotationAtDistanceAlongSpline` self _returnvalue_4 "World") (`KismetMathLibrary.MakeVector` _returnvalue _returnvalue _returnvalue))))
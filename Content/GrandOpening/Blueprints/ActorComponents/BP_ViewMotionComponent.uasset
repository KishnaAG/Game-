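; Actor component that drives procedural first-person camera motion and surface-based footstep sounds for a Character.
; Each tick it layers head bob, breathing, look sway, acceleration lean, landing, air and crouch offsets and sprint FOV, tuned by Motion.
; Springs and interpolation shape these layers and a focus mode that eases the view onto a world point.
; Focus temporarily swaps anti-aliasing to avoid 3D widget ghosting, restoring it on clear or EndPlay.
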(event `self.ReceiveBeginPlay`
  ;[1 1 1 0.8] Event begin play
  (bind _resolved (`self.ResolveViewComponents` self))
  (`/Engine/EditorBlueprintResources/StandardMacros.IsValid` (`self.Motion`)
    (:`Is Valid`
      (if _resolved
        (`self.SetComponentTickEnabled` self true)))))

(event `self.ReceiveTick`
  (params (DeltaSeconds :type "Float (single-precision)"))
  (bind _returnvalue (`KismetMathLibrary.FMin` DeltaSeconds (`/Game/GrandOpening/Blueprints/DataAssets/ViewMotion/BP_ViewMotionDataAsset.MaxViewDeltaTime` (`self.Motion`))))
  ;[1 1 1 0.8] Event tick
  (`self.AdvanceWalkClock` self _returnvalue)
  (`self.AdvanceViewSway` self _returnvalue)
  (`self.AdvanceViewOffsets` self _returnvalue)
  (`self.AdvanceFocus` self _returnvalue)
  (`self.ApplyViewTransform` self)
  (`self.AdvanceFootsteps` self))

(event `self.ReceiveEndPlay`
  (params (EndPlayReason :type "EEndPlayReason Enum" :default "Destroyed"))
  ;[1 1 1 0.8] Event end play
  ;;[1 0.3141 0.8218 0.8] This event is used to restore the AA method even if we close the PIE while being in a focus mode. Without this your editor will be stuck in a non-AA rendering.
  (if (`self.Focusing`)
    (`self.SetAntiAliasingMethod` self (`self.PreviousAntiAliasingMethod`))))

(fn `AddCrouchTransition`
  (params (HeightAdjust :type "Float (double-precision)"))
  ;[1 1 1 0.8] Add crouch transition
  (set `self.CrouchOffset` (+ (`self.CrouchOffset`) HeightAdjust)))

(fn `AdvanceFocus`
  (params (DeltaTime :type "Float (double-precision)"))
  (bind _motion (`self.Motion`))
  (bind _focusing (`self.Focusing`))
  (bind _focusoffset (`self.FocusOffset`))
  (bind _focusblendspeed (`/Game/GrandOpening/Blueprints/DataAssets/ViewMotion/BP_ViewMotionDataAsset.FocusBlendSpeed` _motion))
  (bind _focusdipstiffness (`/Game/GrandOpening/Blueprints/DataAssets/ViewMotion/BP_ViewMotionDataAsset.FocusDipStiffness` _motion))
  (bind _focusdipdamping (`/Game/GrandOpening/Blueprints/DataAssets/ViewMotion/BP_ViewMotionDataAsset.FocusDipDamping` _motion))
  ;[1 1 1 0.8] Advance focus
  (bind (_newvalue _newvelocity) (`self.StepSpring` self (.z _focusoffset) (`self.FocusVerticalVelocity`) (.z (`KismetMathLibrary.SelectVector` (`KismetMathLibrary.MakeVector` (.x (`KismetMathLibrary.InverseTransformLocation` (`Actor.GetTransform` (`self.OwnerPawn`)) (`self.FocusWorldLocation`))) (.y (`KismetMathLibrary.InverseTransformLocation` (`Actor.GetTransform` (`self.OwnerPawn`)) (`self.FocusWorldLocation`))) (- (.z (`KismetMathLibrary.InverseTransformLocation` (`Actor.GetTransform` (`self.OwnerPawn`)) (`self.FocusWorldLocation`))) (`self.BaseEyeHeight`))) (0.0 0.0 0.0) _focusing)) _focusdipstiffness _focusdipdamping DeltaTime))
  (set `self.FocusOffset` (`KismetMathLibrary.MakeVector` (`KismetMathLibrary.FInterpTo` (.x _focusoffset) (.x (`KismetMathLibrary.SelectVector` (`KismetMathLibrary.MakeVector` (.x (`KismetMathLibrary.InverseTransformLocation` (`Actor.GetTransform` (`self.OwnerPawn`)) (`self.FocusWorldLocation`))) (.y (`KismetMathLibrary.InverseTransformLocation` (`Actor.GetTransform` (`self.OwnerPawn`)) (`self.FocusWorldLocation`))) (- (.z (`KismetMathLibrary.InverseTransformLocation` (`Actor.GetTransform` (`self.OwnerPawn`)) (`self.FocusWorldLocation`))) (`self.BaseEyeHeight`))) (0.0 0.0 0.0) _focusing)) DeltaTime _focusblendspeed) (`KismetMathLibrary.FInterpTo` (.y _focusoffset) (.y (`KismetMathLibrary.SelectVector` (`KismetMathLibrary.MakeVector` (.x (`KismetMathLibrary.InverseTransformLocation` (`Actor.GetTransform` (`self.OwnerPawn`)) (`self.FocusWorldLocation`))) (.y (`KismetMathLibrary.InverseTransformLocation` (`Actor.GetTransform` (`self.OwnerPawn`)) (`self.FocusWorldLocation`))) (- (.z (`KismetMathLibrary.InverseTransformLocation` (`Actor.GetTransform` (`self.OwnerPawn`)) (`self.FocusWorldLocation`))) (`self.BaseEyeHeight`))) (0.0 0.0 0.0) _focusing)) DeltaTime _focusblendspeed) _newvalue))
  (set `self.FocusVerticalVelocity` _newvelocity)
  (bind (_newvalue_2 _newvelocity_2) (`self.StepSpring` self (`self.FocusPitch`) (`self.FocusPitchVelocity`) (`self.FocusTargetPitch`) _focusdipstiffness _focusdipdamping DeltaTime))
  (set `self.FocusPitch` _newvalue_2)
  (set `self.FocusPitchVelocity` _newvelocity_2)
  (set `self.FocusYaw` (`KismetMathLibrary.FInterpTo` (`self.FocusYaw`) (`self.FocusTargetYaw`) DeltaTime _focusblendspeed))
  (set `self.FocusFov` (`KismetMathLibrary.FInterpTo` (`self.FocusFov`) (`KismetMathLibrary.SelectFloat` (`/Game/GrandOpening/Blueprints/DataAssets/ViewMotion/BP_ViewMotionDataAsset.FocusFovAdd` _motion) 0.0 _focusing) DeltaTime _focusblendspeed)))

(fn `AdvanceFootsteps`
  (bind _returnvalue (`KismetMathLibrary.FFloor` (/ (`self.StridePhase`) 180.0)))
  ;[1 1 1 0.8] Advance footsteps
  (if (!= _returnvalue (`self.LastStepIndex`))
    (set `self.LastStepIndex` _returnvalue)
    (if (`NavMovementInterface.IsMovingOnGround` (`self.Movement`))
      (`self.PlayFootstep` self (`self.FootstepVolume`)))))

(fn `AdvanceViewOffsets`
  (params (DeltaTime :type "Float (double-precision)"))
  (bind _motion (`self.Motion`))
  (bind _movement (`self.Movement`))
  ;[1 1 1 0.8] Advance view offsets
  (bind (_newvalue _newvelocity) (`self.StepSpring` self (`self.ImpulseOffset`) (`self.ImpulseVelocity`) 0.0 (`/Game/GrandOpening/Blueprints/DataAssets/ViewMotion/BP_ViewMotionDataAsset.LandStiffness` _motion) (`/Game/GrandOpening/Blueprints/DataAssets/ViewMotion/BP_ViewMotionDataAsset.LandDamping` _motion) DeltaTime))
  (set `self.ImpulseOffset` _newvalue)
  (set `self.ImpulseVelocity` _newvelocity)
  (set `self.AirOffset` (`KismetMathLibrary.FInterpTo` (`self.AirOffset`) (select `bool` (`NavMovementInterface.IsFalling` _movement) :`true` (* (`KismetMathLibrary.FClamp` (/ (.z (`MovementComponent.Velocity` _movement)) (`/Game/GrandOpening/Blueprints/DataAssets/ViewMotion/BP_ViewMotionDataAsset.AirVelocityReference` _motion)) -1.0) (`/Game/GrandOpening/Blueprints/DataAssets/ViewMotion/BP_ViewMotionDataAsset.AirOffsetCm` _motion))) DeltaTime (`/Game/GrandOpening/Blueprints/DataAssets/ViewMotion/BP_ViewMotionDataAsset.AirBlendSpeed` _motion)))
  (set `self.CrouchOffset` (`KismetMathLibrary.FInterpTo` (`self.CrouchOffset`) 0.0 DeltaTime (`/Game/GrandOpening/Blueprints/DataAssets/ViewMotion/BP_ViewMotionDataAsset.CrouchBlendSpeed` _motion)))
  (set `self.FovOffset` (`KismetMathLibrary.FInterpTo` (`self.FovOffset`) (* (`KismetMathLibrary.FClamp` (/ (- (`self.MotionAlpha`) 1.0) (- (`/Game/GrandOpening/Blueprints/DataAssets/ViewMotion/BP_ViewMotionDataAsset.MaxMotionScale` _motion) 1.0))) (`/Game/GrandOpening/Blueprints/DataAssets/ViewMotion/BP_ViewMotionDataAsset.SprintFovAdd` _motion)) DeltaTime (`/Game/GrandOpening/Blueprints/DataAssets/ViewMotion/BP_ViewMotionDataAsset.FovBlendSpeed` _motion))))

(fn `AdvanceViewSway`
  (params (DeltaTime :type "Float (double-precision)"))
  (bind _motion (`self.Motion`))
  (bind _ownerpawn (`self.OwnerPawn`))
  (bind _movement (`self.Movement`))
  (bind _lastcontrolrotation (`self.LastControlRotation`))
  (bind _returnvalue (`Pawn.GetControlRotation` _ownerpawn))
  (bind _returnvalue_2 (`CharacterMovementComponent.GetCurrentAcceleration` _movement))
  (bind _returnvalue_3 (`CharacterMovementComponent.GetMaxAcceleration` _movement))
  (bind _leanstiffness (`/Game/GrandOpening/Blueprints/DataAssets/ViewMotion/BP_ViewMotionDataAsset.LeanStiffness` _motion))
  (bind _leandamping (`/Game/GrandOpening/Blueprints/DataAssets/ViewMotion/BP_ViewMotionDataAsset.LeanDamping` _motion))
  (bind _lookrateblend (`/Game/GrandOpening/Blueprints/DataAssets/ViewMotion/BP_ViewMotionDataAsset.LookRateBlend` _motion))
  (bind _lookswayreferencerate (`/Game/GrandOpening/Blueprints/DataAssets/ViewMotion/BP_ViewMotionDataAsset.LookSwayReferenceRate` _motion))
  (bind _returnvalue_4 (`KismetMathLibrary.FClamp` (/ (`self.LookYawRate`) _lookswayreferencerate) -1.0))
  ;[1 1 1 0.8] Advance view sway
  (set `self.LookYawRate` (`KismetMathLibrary.FInterpTo` (`self.LookYawRate`) (/ (`KismetMathLibrary.NormalizeAxis` (- (.yaw _returnvalue) (.yaw _lastcontrolrotation))) DeltaTime) DeltaTime _lookrateblend))
  (set `self.LookPitchRate` (`KismetMathLibrary.FInterpTo` (`self.LookPitchRate`) (/ (`KismetMathLibrary.NormalizeAxis` (- (.pitch _returnvalue) (.pitch _lastcontrolrotation))) DeltaTime) DeltaTime _lookrateblend))
  (set `self.LastControlRotation` _returnvalue)
  (set `self.LookYaw` (* (- 0.0 _returnvalue_4) (`/Game/GrandOpening/Blueprints/DataAssets/ViewMotion/BP_ViewMotionDataAsset.LookSwayYawDeg` _motion)))
  (set `self.LookPitch` (* (- 0.0 (`KismetMathLibrary.FClamp` (/ (`self.LookPitchRate`) _lookswayreferencerate) -1.0)) (`/Game/GrandOpening/Blueprints/DataAssets/ViewMotion/BP_ViewMotionDataAsset.LookSwayPitchDeg` _motion)))
  (set `self.LookRoll` (* (- 0.0 _returnvalue_4) (`/Game/GrandOpening/Blueprints/DataAssets/ViewMotion/BP_ViewMotionDataAsset.LookSwayRollDeg` _motion)))
  (bind (_newvalue _newvelocity) (`self.StepSpring` self (`self.LeanPitch`) (`self.LeanPitchVelocity`) (- 0.0 (* (`KismetMathLibrary.FClamp` (/ (`KismetMathLibrary.Dot_VectorVector` _returnvalue_2 (`Actor.GetActorForwardVector` _ownerpawn)) _returnvalue_3) -1.0) (`/Game/GrandOpening/Blueprints/DataAssets/ViewMotion/BP_ViewMotionDataAsset.AccelPitchDeg` _motion))) _leanstiffness _leandamping DeltaTime))
  (set `self.LeanPitch` _newvalue)
  (set `self.LeanPitchVelocity` _newvelocity)
  (bind (_newvalue_2 _newvelocity_2) (`self.StepSpring` self (`self.LeanRoll`) (`self.LeanRollVelocity`) (* (`KismetMathLibrary.FClamp` (/ (`KismetMathLibrary.Dot_VectorVector` _returnvalue_2 (`Actor.GetActorRightVector` _ownerpawn)) _returnvalue_3) -1.0) (`/Game/GrandOpening/Blueprints/DataAssets/ViewMotion/BP_ViewMotionDataAsset.StrafeRollDeg` _motion)) _leanstiffness _leandamping DeltaTime))
  (set `self.LeanRoll` _newvalue_2)
  (set `self.LeanRollVelocity` _newvelocity_2))

(fn `AdvanceWalkClock`
  (params (DeltaTime :type "Float (double-precision)"))
  (bind _motion (`self.Motion`))
  (bind _movement (`self.Movement`))
  (bind _returnvalue (`KismetMathLibrary.VSizeXY` (`MovementComponent.Velocity` _movement)))
  ;[1 1 1 0.8] Advance walk clock
  (set `self.MotionAlpha` (`KismetMathLibrary.FInterpTo` (`self.MotionAlpha`) (select `bool` (`NavMovementInterface.IsMovingOnGround` _movement) :`true` (`KismetMathLibrary.FClamp` (/ _returnvalue (`/Game/GrandOpening/Blueprints/DataAssets/ViewMotion/BP_ViewMotionDataAsset.FullMotionSpeed` _motion)) 0.0 (`/Game/GrandOpening/Blueprints/DataAssets/ViewMotion/BP_ViewMotionDataAsset.MaxMotionScale` _motion))) DeltaTime (`/Game/GrandOpening/Blueprints/DataAssets/ViewMotion/BP_ViewMotionDataAsset.MotionBlendSpeed` _motion)))
  (set `self.StridePhase` (+ (`self.StridePhase`) (/ (* _returnvalue (* DeltaTime 180.0)) (`/Game/GrandOpening/Blueprints/DataAssets/ViewMotion/BP_ViewMotionDataAsset.StepLengthCm` _motion))))
  (set `self.BreathPhase` (+ (`self.BreathPhase`) (* (`/Game/GrandOpening/Blueprints/DataAssets/ViewMotion/BP_ViewMotionDataAsset.BreathRateHz` _motion) (* DeltaTime 360.0)))))

(fn `ApplyLandImpact`
  (params (FallSpeed :type "Float (double-precision)"))
  (bind _motion (`self.Motion`))
  ;[1 1 1 0.8] Apply land impact
  (set `self.ImpulseOffset` (- 0.0 (* (`KismetMathLibrary.FClamp` (/ (`KismetMathLibrary.Abs` FallSpeed) (`/Game/GrandOpening/Blueprints/DataAssets/ViewMotion/BP_ViewMotionDataAsset.LandFullImpactSpeed` _motion))) (`/Game/GrandOpening/Blueprints/DataAssets/ViewMotion/BP_ViewMotionDataAsset.LandDipCm` _motion))))
  (set `self.ImpulseVelocity` 0.0)
  (`self.PlayFootstep` (`self.LandingVolume`)))

(fn `ApplyViewTransform`
  (bind _motion (`self.Motion`))
  (bind _motionalpha (`self.MotionAlpha`))
  (bind _viewcamera (`self.ViewCamera`))
  (bind _stridephase (`self.StridePhase`))
  (bind _returnvalue (`KismetMathLibrary.DegSin` _stridephase))
  (bind _returnvalue_2 (* _stridephase 2.0))
  ;[1 1 1 0.8] Apply view transform
  (`SceneComponent.K2_SetRelativeLocation` (`self.ViewRoot`) (`KismetMathLibrary.MakeVector` (.x (`self.FocusOffset`)) (+ (* (* _returnvalue (`/Game/GrandOpening/Blueprints/DataAssets/ViewMotion/BP_ViewMotionDataAsset.BobLateralCm` _motion)) _motionalpha) (.y (`self.FocusOffset`))) (+ (+ (+ (`self.BaseEyeHeight`) (`self.CrouchOffset`)) (+ (+ (* (* (- 0.0 (`KismetMathLibrary.DegCos` _returnvalue_2)) (`/Game/GrandOpening/Blueprints/DataAssets/ViewMotion/BP_ViewMotionDataAsset.BobVerticalCm` _motion)) _motionalpha) (* (* (`KismetMathLibrary.DegSin` (`self.BreathPhase`)) (`KismetMathLibrary.SelectFloat` 0.0 (`/Game/GrandOpening/Blueprints/DataAssets/ViewMotion/BP_ViewMotionDataAsset.BreathCm` _motion) (`self.Focusing`))) (`KismetMathLibrary.FClamp` (- 1.0 _motionalpha)))) (+ (`self.ImpulseOffset`) (`self.AirOffset`)))) (.z (`self.FocusOffset`)))) false false)
  (`SceneComponent.K2_SetRelativeRotation` _viewcamera (`KismetMathLibrary.MakeRotator` (+ (+ (`self.LeanRoll`) (`self.LookRoll`)) (* (* _returnvalue (`/Game/GrandOpening/Blueprints/DataAssets/ViewMotion/BP_ViewMotionDataAsset.BobRollDeg` _motion)) _motionalpha)) (+ (+ (+ (.pitch (`Pawn.GetControlRotation` (`self.OwnerPawn`))) (+ (`self.LeanPitch`) (`self.LookPitch`))) (* (* (`KismetMathLibrary.DegSin` _returnvalue_2) (`/Game/GrandOpening/Blueprints/DataAssets/ViewMotion/BP_ViewMotionDataAsset.BobPitchDeg` _motion)) _motionalpha)) (`self.FocusPitch`)) (+ (`self.LookYaw`) (`self.FocusYaw`))) false false)
  (`CameraComponent.SetFieldOfView` _viewcamera (+ (+ (`self.BaseFieldOfView`) (`self.FovOffset`)) (`self.FocusFov`))))

(fn `ClearFocus`
  ;[1 1 1 0.8] Clear focus
  (set `self.FocusTargetPitch` 0.0)
  (set `self.FocusTargetYaw` 0.0)
  (set `self.Focusing` false)
  (`self.SetAntiAliasingMethod` (`self.PreviousAntiAliasingMethod`))
  (`self.OnFocusEnded`))

(fn `FocusOn`
  (params (WorldLocation :type "Vector Structure") (WorldRotation :type "Rotator Structure"))
  (bind _returnvalue (`Pawn.GetControlRotation` (`self.OwnerPawn`)))
  ;[1 1 1 0.8] Focus on
  (set `self.FocusWorldLocation` WorldLocation)
  (set `self.FocusTargetPitch` (`KismetMathLibrary.NormalizeAxis` (- (.pitch WorldRotation) (.pitch _returnvalue))))
  (set `self.FocusTargetYaw` (`KismetMathLibrary.NormalizeAxis` (- (.yaw WorldRotation) (.yaw _returnvalue))))
  (set `self.Focusing` true)
  (bind _returnvalue_2 (`KismetSystemLibrary.GetConsoleVariableIntValue` "r.AntiAliasingMethod"))
  (set `self.PreviousAntiAliasingMethod` _returnvalue_2)
  (`self.SetAntiAliasingMethod` (`self.FocusAntiAliasingMethod`))
  (`self.OnFocusBegan`))

(fn `PlayFootstep`
  (params (Volume :type "Float (double-precision)"))
  (locals (Sound :type "SoundBase Object Reference"))
  (bind _ownerpawn (`self.OwnerPawn`))
  (bind _returnvalue (`Actor.K2_GetActorLocation` _ownerpawn))
  ;[1 1 1 0.8] Play footstep
  (bind (_outhit _returnvalue_2) (`KismetSystemLibrary.LineTraceSingle` _returnvalue (- _returnvalue (`KismetMathLibrary.MakeVector` 0.0 0.0 (`self.FootstepTraceCm`))) "TraceTypeQuery1"))
  (if _returnvalue_2
    (switch `EPhysicalSurface` (`GameplayStatics.GetSurfaceType` _outhit)
      (:`SurfaceType_Default`
        (set `local.Sound` (`self.FootstepDefault`)))
      (:`SurfaceType1`
        (set `local.Sound` (`self.FootstepConcrete`)))
      (:`SurfaceType2`
        (set `local.Sound` (`self.FootstepGround`)))
      (:`SurfaceType3`
        (set `local.Sound` (`self.FootstepMetal`)))
      (:`SurfaceType4`
        (set `local.Sound` (`self.FootstepWater`)))
      (:`SurfaceType5`
        (set `local.Sound` (`self.FootstepWood`))))
    (`GameplayStatics.SpawnSoundAttached` (`local.Sound`) (`Actor.RootComponent` _ownerpawn) "None" (0.0 0.0 0.0) (struct) "KeepRelativeOffset" false Volume 1.0 0.0 null null)))

(fn `ResolveViewComponents`
  (returns (Resolved :type Boolean))
  ;[1 1 1 0.8] Resolve view components
  (bind _ascharacter (cast `Character` (`self.GetOwner`))
    (:`then`
      (set `self.OwnerPawn` _ascharacter)
      (bind _charactermovement (`Character.CharacterMovement` _ascharacter))
      (set `self.Movement` _charactermovement)
      (`self.AddTickPrerequisiteComponent` self _charactermovement)
      (set `self.LastControlRotation` (`Pawn.GetControlRotation` _ascharacter))
      (bind _returnvalue (`Actor.GetComponentByClass` _ascharacter "/Script/Engine.CameraComponent"))
      (set `self.ViewCamera` _returnvalue)
      (set `self.BaseFieldOfView` (`CameraComponent.FieldOfView` _returnvalue))
      (bind _returnvalue_2 (`SceneComponent.GetAttachParent` _returnvalue))
      (set `self.ViewRoot` _returnvalue_2)
      (set `self.BaseEyeHeight` (.z (`SceneComponent.RelativeLocation` _returnvalue_2)))
      (return true))
    (:`CastFailed`
      (return false))))

(fn `SetAntiAliasingMethod`
  (params (Method :type Integer))
  ;[1 0.3141 0.8218 0.8] Set anti aliasing method - This is used to prevent ghosting effect on 3D widgets in the world.
  ; You can remove this to get better result when focusing something, but you will have some trouble with 3D widgets, specially with non-static 3D widgets
  (`KismetSystemLibrary.ExecuteConsoleCommand` (`KismetStringLibrary.Concat_StrStr` "r.AntiAliasingMethod " (`KismetStringLibrary.Conv_IntToString` Method)) null))

(fn `StepSpring`
  (params (Current :type "Float (double-precision)") (Velocity :type "Float (double-precision)") (Target :type "Float (double-precision)") (Stiffness :type "Float (double-precision)") (Damping :type "Float (double-precision)") (DeltaTime :type "Float (double-precision)"))
  (returns (NewValue :type "Float (double-precision)") (NewVelocity :type "Float (double-precision)"))
  (bind _returnvalue (+ Velocity (* (- (* (- Target Current) Stiffness) (* Velocity Damping)) DeltaTime)))
  ;[1 1 1 0.8] Step spring
  (return (+ Current (* _returnvalue DeltaTime)) _returnvalue))
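; BP_ReactionComponent is a widget component that shows reaction speech bubbles when named events happen.
; React finds the entry matching the event in its Reactions list, skipping events while the bubble is already showing.
; A weighted chance decides whether to react, then a random line from that entry is formatted with the subject and displayed for the entry's duration.
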(fn `React`
  (params (Event :type "/Game/GrandOpening/Blueprints/Enumerations/E_ReactionEvent Enum" :default "NewEnumerator0") (Subject :type Text))
  (locals (Match :type "/Game/GrandOpening/Blueprints/DataAssets/Reactions/BP_ReactionDataAsset Object Reference"))
  (bind _match (`local.Match`))
  ;[1 1 1 0.8] React
  (bind _asbp_reaction_bubble_widget (cast `/Game/GrandOpening/Blueprints/Widgets/Gameplay/BP_ReactionBubbleWidget` (`self.GetUserWidgetObject` self)))
  (if (not (`/Game/GrandOpening/Blueprints/Widgets/Gameplay/BP_ReactionBubbleWidget.Showing` _asbp_reaction_bubble_widget))
    (for _array_element (`self.Reactions`)
      (if (`|EnumEquality` (`/Game/GrandOpening/Blueprints/DataAssets/Reactions/BP_ReactionDataAsset.Event` _array_element) Event)
        (set `local.Match` _array_element)))
    (`/Engine/EditorBlueprintResources/StandardMacros.IsValid` _match
      (:`Is Valid`
        (if (`KismetMathLibrary.RandomBoolWithWeight` (`/Game/GrandOpening/Blueprints/DataAssets/Reactions/BP_ReactionDataAsset.Chance` _match))
          (`/Game/GrandOpening/Blueprints/Widgets/Gameplay/BP_ReactionBubbleWidget.Show` _asbp_reaction_bubble_widget (`|FormatText` (`KismetArrayLibrary.Array_Random` (`/Game/GrandOpening/Blueprints/DataAssets/Reactions/BP_ReactionDataAsset.Lines` _match)) (`local.Subject`)) (`/Game/GrandOpening/Blueprints/DataAssets/Reactions/BP_ReactionDataAsset.Seconds` _match)))))))
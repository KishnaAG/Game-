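; Player character component that drives first-person-style look-at interaction with actors carrying an enabled BP_InteractableComponent.
; Each tick, once owner and controller resolve, it traces from the camera to set focus, updates the crosshair prompt and broadcasts focus changes.
; BeginInteract fires the target's interacted event instantly or after its hold time, with EndInteract or lost focus cancelling.
; Other systems can suspend focus, ignore an actor, toggle the crosshair or query the aim point.
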(event `self.ReceiveBeginPlay`
  ;[1 1 1 0.8] Event begin play
  (bind _resolved (`self.ResolveInteraction` self))
  (bind _resolved_2 (`self.ResolvePrompt` self))
  (if (and _resolved _resolved_2)
    (`self.SetComponentTickEnabled` self true)))

(event `self.ReceiveTick`
  (params (DeltaSeconds :type "Float (single-precision)"))
  ;[1 1 1 0.8] Event tick
  (`self.AdvanceFocus` self)
  (`self.AdvanceHold` self DeltaSeconds)
  (`self.AdvancePrompt` self))

(fn `AdvanceFocus`
  (bind _viewcamera (`self.ViewCamera`))
  (bind _returnvalue (`SceneComponent.K2_GetComponentLocation` _viewcamera))
  ;[1 1 1 0.8] Advance focus
  (if (`self.Suspended`)
    (set `self.Focused` null)
    (else
      (bind (_outhit _returnvalue_2) (`KismetSystemLibrary.LineTraceSingle` _returnvalue (+ _returnvalue (* (`SceneComponent.GetForwardVector` _viewcamera) (`self.TraceLength`))) "TraceTypeQuery1" false (`|MakeArray` (`self.Ignored`))))
      (set `self.Focused` null)
      (if _returnvalue_2
        (bind _returnvalue_3 (`Actor.GetComponentByClass` (`.HitActor` (`GameplayStatics.BreakHitResult` _outhit)) "/Game/GrandOpening/Blueprints/ActorComponents/BP_InteractableComponent.BP_InteractableComponent_C"))
        (`/Engine/EditorBlueprintResources/StandardMacros.IsValid` _returnvalue_3
          (:`Is Valid`
            (if (`/Game/GrandOpening/Blueprints/ActorComponents/BP_InteractableComponent.Enabled` _returnvalue_3)
              (set `self.Focused` _returnvalue_3))))))))

(fn `AdvanceHold`
  (params (DeltaTime :type "Float (double-precision)"))
  (bind _returnvalue (+ (`self.HoldElapsed`) DeltaTime))
  (bind _holdseconds (`/Game/GrandOpening/Blueprints/ActorComponents/BP_InteractableComponent.HoldSeconds` (`self.Focused`)))
  ;[1 1 1 0.8] Advance hold
  (if (`self.Holding`)
    (`/Engine/EditorBlueprintResources/StandardMacros.IsValid` (`self.Focused`)
      (:`Is Valid`
        (set `self.HoldElapsed` _returnvalue)
        (if (and (> _holdseconds 0.0) (>= _returnvalue _holdseconds))
          (`self.FireInteract` self)))
      (:`Is Not Valid`
        (set `self.Holding` false)
        (set `self.HoldElapsed` 0.0)))))

(fn `AdvancePrompt`
  (bind _focused (`self.Focused`))
  ;[1 1 1 0.8] Advance prompt
  (`self.RefreshPrompt` self)
  (if (!= _focused (`self.LastFocused`))
    (set `self.LastFocused` _focused)
    (`self.OnFocusChanged`)))

(fn `BeginInteract`
  (bind _focused (`self.Focused`))
  ;[1 1 1 0.8] Begin interact
  (`/Engine/EditorBlueprintResources/StandardMacros.IsValid` _focused
    (:`Is Valid`
      (if (<= (`/Game/GrandOpening/Blueprints/ActorComponents/BP_InteractableComponent.HoldSeconds` _focused) 0.0)
        (`self.FireInteract` self)
        (else
          (set `self.HoldElapsed` 0.0)
          (set `self.Holding` true))))))

(fn `EndInteract`
  ;[1 1 1 0.8] End interact
  (set `self.Holding` false)
  (set `self.HoldElapsed` 0.0))

(fn `FireInteract`
  (bind _focused (`self.Focused`))
  ;[1 1 1 0.8] Fire interact
  (set `self.Holding` false)
  (set `self.HoldElapsed` 0.0)
  (`/Engine/EditorBlueprintResources/StandardMacros.IsValid` _focused
    (:`Is Valid`
      (`/Game/GrandOpening/Blueprints/ActorComponents/BP_InteractableComponent.OnInteracted` _focused (`self.OwnerPawn`)))))

(fn `GetAimPoint`
  (returns (ReturnValue :type "Vector Structure"))
  (bind _viewcamera (`self.ViewCamera`))
  (bind _returnvalue (`SceneComponent.K2_GetComponentLocation` _viewcamera))
  (bind _returnvalue_2 (+ _returnvalue (* (`SceneComponent.GetForwardVector` _viewcamera) (`self.TraceLength`))))
  ;[1 1 1 0.8] Get aim point
  (bind (_outhit _returnvalue_3) (`KismetSystemLibrary.LineTraceSingle` _returnvalue _returnvalue_2 "TraceTypeQuery1" false (`|MakeArray` (`self.Ignored`))))
  (return (select `bool` _returnvalue_3 :`false` _returnvalue_2 :`true` (`.Location` (`GameplayStatics.BreakHitResult` _outhit)))))

(fn `HideCrosshair`
  ;[1 1 1 0.8] Hide crosshair
  (`Widget.SetVisibility` (`self.Crosshair`) "Collapsed"))

(fn `RefreshPrompt`
  (bind _crosshair (`self.Crosshair`))
  (bind _focused (`self.Focused`))
  ;[1 1 1 0.8] Refresh prompt
  (`/Engine/EditorBlueprintResources/StandardMacros.IsValid` _focused
    (:`Is Valid`
      (`/Game/GrandOpening/Blueprints/Widgets/Gameplay/BP_CrosshairWidget.ShowPrompt` _crosshair (`/Game/GrandOpening/Blueprints/ActorComponents/BP_InteractableComponent.Label` _focused)))
    (:`Is Not Valid`
      (`/Game/GrandOpening/Blueprints/Widgets/Gameplay/BP_CrosshairWidget.HidePrompt` _crosshair))))

(fn `ResolveInteraction`
  (returns (Resolved :type Boolean))
  ;[1 1 1 0.8] Resolve interaction
  (bind _ascharacter (cast `Character` (`self.GetOwner`))
    (:`then`
      (set `self.OwnerPawn` _ascharacter)
      (set `self.ViewCamera` (`Actor.GetComponentByClass` _ascharacter "/Script/Engine.CameraComponent"))
      (return true))
    (:`CastFailed`
      (return false))))

(fn `ResolvePrompt`
  (returns (Resolved :type Boolean))
  ;[1 1 1 0.8] Resolve prompt
  (bind _asplayer_controller (cast `PlayerController` (`Pawn.GetController` (`self.OwnerPawn`)))
    (:`then`
      (bind _returnvalue (`|CreateWidget` (`self.CrosshairClass`) _asplayer_controller))
      (set `self.Crosshair` _returnvalue)
      (`UserWidget.AddToViewport` _returnvalue 0)
      (return true))
    (:`CastFailed`
      (return false))))

(fn `SetIgnored`
  (params (Target :type "Actor Object Reference"))
  ;[1 1 1 0.8] Set ignored
  (set `self.Ignored` Target))

(fn `SetSuspended`
  (params (Suspended :type Boolean))
  ;[1 1 1 0.8] Set suspended
  (set `self.Suspended` Suspended))

(fn `ShowCrosshair`
  ;[1 1 1 0.8] Show crosshair
  (bind _asplayer_controller (cast `PlayerController` (`Pawn.GetController` (`self.OwnerPawn`))))
  (`Widget.SetVisibility` (`self.Crosshair`) "SelfHitTestInvisible")
  (set `PlayerController.bShowMouseCursor` false _asplayer_controller)
  (`WidgetBlueprintLibrary.SetInputMode_GameOnly` _asplayer_controller))
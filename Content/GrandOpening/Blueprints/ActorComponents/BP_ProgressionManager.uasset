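; Progression component for a store game that grants catalog unlocks based on store metrics such as balance, revenue, rating, day and customers served.
; Unlocks check prerequisite unlocks and metric thresholds; free ones are granted by Evaluate on day end, priced ones are bought through StoreManager transactions.
; Assets absent from every unlock's rewards count as unlocked.
; Grants record their day, save out, and rebroadcast OnUnlocked when restored from a pending save.
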(event `self.ReceiveBeginPlay`
  (bind _storemanager (`self.StoreManager`))
  ;[1 1 1 0.8] Event begin play
  (set `self.StoreManager` (`Actor.GetComponentByClass` (`GameplayStatics.GetGameState`) "/Game/GrandOpening/Blueprints/ActorComponents/BP_StoreManager.BP_StoreManager_C"))
  (`/Engine/EditorBlueprintResources/StandardMacros.IsValid` _storemanager
    (:`Is Valid`
      (add `/Game/GrandOpening/Blueprints/ActorComponents/BP_StoreManager.OnDayEnded` _storemanager (`|CreateDelegate` :!event `HandleDayEnded`))
      (`self.RestoreFromSave`))))

(fn `CollectInto`
  (params (Save :type "/Game/GrandOpening/Blueprints/Misc/SG_StoreSave Object Reference"))
  ;[1 1 1 0.8] Collect into
  (set `/Game/GrandOpening/Blueprints/Misc/SG_StoreSave.GrantedUnlocks` (`self.Granted`) Save))

(fn `Evaluate`
  ;[1 1 1 0.8] Evaluate
  (for _array_element (`self.Catalog`)
    (bind _available (`self.IsAvailable` _array_element))
    (if (and _available (<= (`/Game/GrandOpening/Blueprints/DataAssets/Unlocks/BP_UnlockDataAsset.Price` _array_element) 0.0))
      (`self.GrantUnlock` _array_element))))

(fn `FindGranted`
  (params (Unlock :type "/Game/GrandOpening/Blueprints/DataAssets/Unlocks/BP_UnlockDataAsset Object Reference"))
  (returns (Found :type Boolean) (Day :type Integer))
  (locals (FoundEntry :type Boolean) (FoundDay :type Integer))
  ;[1 1 1 0.8] Find granted
  (set `local.FoundEntry` false)
  (set `local.FoundDay` 0)
  (for _array_element (`self.Granted`)
    (bind (_unlock _day) (break `/Game/GrandOpening/Blueprints/Structures/S_GrantedUnlock` _array_element))
    (if (== _unlock Unlock)
      (set `local.FoundEntry` true)
      (set `local.FoundDay` _day)))
  (return (`local.FoundEntry`) (`local.FoundDay`)))

(fn `GetCustomersServed`
  (returns (Value :type Integer))
  (locals (Total :type Integer))
  ;[1 1 1 0.8] Get customers served
  (set `local.Total` 0)
  (for _array_element (`/Game/GrandOpening/Blueprints/ActorComponents/BP_StoreManager.CustomersServedPerDay` (`self.StoreManager`))
    (set `local.Total` (+ (`local.Total`) _array_element)))
  (return (`local.Total`)))

(fn `GetMetric`
  (params (Condition :type "/Game/GrandOpening/Blueprints/Enumerations/E_UnlockCondition Enum" :default "NewEnumerator0"))
  (returns (Value :type "Float (double-precision)"))
  (locals (Metric :type "Float (double-precision)"))
  (bind _storemanager (`self.StoreManager`))
  ;[1 1 1 0.8] Get metric
  (switch `/Game/GrandOpening/Blueprints/Enumerations/E_UnlockCondition` Condition
    (:`NewEnumerator0`
      (set `local.Metric` (`/Game/GrandOpening/Blueprints/ActorComponents/BP_StoreManager.CurrentBalance` _storemanager)))
    (:`NewEnumerator4`
      (bind _value (`self.GetSalesRevenue`))
      (set `local.Metric` _value))
    (:`NewEnumerator1`
      (set `local.Metric` (`/Game/GrandOpening/Blueprints/ActorComponents/BP_StoreManager.StoreRating` _storemanager)))
    (:`NewEnumerator2`
      (set `local.Metric` (`KismetMathLibrary.Conv_IntToDouble` (`/Game/GrandOpening/Blueprints/ActorComponents/BP_StoreManager.CurrentDay` _storemanager))))
    (:`NewEnumerator5`
      (bind _value_2 (`self.GetCustomersServed`))
      (set `local.Metric` (`KismetMathLibrary.Conv_IntToDouble` _value_2))))
  (return (`local.Metric`)))

(fn `GetSalesRevenue`
  (returns (Value :type "Float (double-precision)"))
  (locals (Total :type "Float (double-precision)"))
  ;[1 1 1 0.8] Get sales revenue
  (set `local.Total` 0.0)
  (for _array_element (`/Game/GrandOpening/Blueprints/ActorComponents/BP_StoreManager.TransactionJournal` (`self.StoreManager`))
    (bind (_amount _reason) (break `/Game/GrandOpening/Blueprints/Structures/S_Transaction` _array_element))
    (switch `/Game/GrandOpening/Blueprints/Enumerations/E_TransactionReason` _reason
      (:`NewEnumerator0`
        (set `local.Total` (+ (`local.Total`) _amount)))))
  (return (`local.Total`)))

(fn `GrantUnlock`
  (params (Unlock :type "/Game/GrandOpening/Blueprints/DataAssets/Unlocks/BP_UnlockDataAsset Object Reference"))
  ;[1 1 1 0.8] Grant unlock
  (bind _found (`self.FindGranted` Unlock))
  (if (not _found)
    (`KismetArrayLibrary.Array_Add` (`self.Granted`) (make `/Game/GrandOpening/Blueprints/Structures/S_GrantedUnlock` Unlock (`/Game/GrandOpening/Blueprints/ActorComponents/BP_StoreManager.CurrentDay` (`self.StoreManager`))))
    (`self.OnUnlocked` Unlock)))

(fn `HandleDayEnded`
  (params (Day :type Integer))
  ;[1 1 1 0.8] Handle day ended
  (`self.Evaluate`))

(fn `IsAvailable`
  (params (Unlock :type "/Game/GrandOpening/Blueprints/DataAssets/Unlocks/BP_UnlockDataAsset Object Reference"))
  (returns (Available :type Boolean))
  (locals (Ok :type Boolean))
  ;[1 1 1 0.8] Is available
  (bind _found (`self.FindGranted` Unlock))
  (set `local.Ok` (not _found))
  (for _array_element (`/Game/GrandOpening/Blueprints/DataAssets/Unlocks/BP_UnlockDataAsset.Requires` Unlock)
    (bind _found_2 (`self.FindGranted` _array_element))
    (if (not _found_2)
      (set `local.Ok` false)))
  (for _array_element_2 (`/Game/GrandOpening/Blueprints/DataAssets/Unlocks/BP_UnlockDataAsset.Requirements` Unlock)
    (bind (_condition _value) (break `/Game/GrandOpening/Blueprints/Structures/S_UnlockRequirement` _array_element_2))
    (bind _value_2 (`self.GetMetric` _condition))
    (if (< _value_2 _value)
      (set `local.Ok` false)))
  (return (`local.Ok`)))

(fn `IsUnlocked`
  (params (Asset :type "PrimaryDataAsset Object Reference"))
  (returns (Unlocked :type Boolean))
  (locals (Found :type Boolean) (Gated :type Boolean))
  ;[1 1 1 0.8] Is unlocked
  (set `local.Gated` false)
  (set `local.Found` false)
  (for _array_element (`self.Catalog`)
    (if (`KismetArrayLibrary.Array_Contains` (`/Game/GrandOpening/Blueprints/DataAssets/Unlocks/BP_UnlockDataAsset.Rewards` _array_element) Asset)
      (set `local.Gated` true)
      (bind _found (`self.FindGranted` _array_element))
      (if _found
        (set `local.Found` true))))
  (return (or (`local.Found`) (not (`local.Gated`)))))

(fn `PurchaseUnlock`
  (params (Unlock :type "/Game/GrandOpening/Blueprints/DataAssets/Unlocks/BP_UnlockDataAsset Object Reference"))
  (returns (Purchased :type Boolean))
  (locals (Done :type Boolean) (Done_0 :type Boolean))
  (bind _storemanager (`self.StoreManager`))
  (bind _price (`/Game/GrandOpening/Blueprints/DataAssets/Unlocks/BP_UnlockDataAsset.Price` Unlock))
  ;[1 1 1 0.8] Purchase unlock
  (set `local.Done` false)
  (bind _available (`self.IsAvailable` Unlock))
  (if (and _available (and (> _price 0.0) (>= (`/Game/GrandOpening/Blueprints/ActorComponents/BP_StoreManager.CurrentBalance` _storemanager) _price)))
    (`/Game/GrandOpening/Blueprints/ActorComponents/BP_StoreManager.AddTransaction` _storemanager (- 0.0 _price) "NewEnumerator1" "None")
    (`self.GrantUnlock` Unlock)
    (set `local.Done` true))
  (return (`local.Done`)))

(fn `RestoreFromSave`
  ;[1 1 1 0.8] Restore from save
  (bind _asbp_store_game_instance (cast `/Game/GrandOpening/Blueprints/Misc/BP_StoreGameInstance` (`GameplayStatics.GetGameInstance`)))
  (bind _pendingsave (`/Game/GrandOpening/Blueprints/Misc/BP_StoreGameInstance.PendingSave` _asbp_store_game_instance))
  (`/Engine/EditorBlueprintResources/StandardMacros.IsValid` _pendingsave
    (:`Is Valid`
      (set `self.Granted` (`/Game/GrandOpening/Blueprints/Misc/SG_StoreSave.GrantedUnlocks` _pendingsave))
      (for _array_element (`self.Granted`)
        (`self.OnUnlocked` (`.Unlock_2_CD1822C74AECE89CA997E88A20D76C20` (break `/Game/GrandOpening/Blueprints/Structures/S_GrantedUnlock` _array_element)))))))
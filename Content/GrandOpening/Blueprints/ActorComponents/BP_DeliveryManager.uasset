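; Actor component that schedules product orders and delivers them as boxes at a registered delivery bay.
; Orders get an arrival day and hour from the store manager, either next opening or a product delay, and hourly clock changes deliver due ones.
; Delivery picks the smallest box size fitting a case, else the largest, and spawns boxes into bay slots until units run out.
; Pending orders persist through the save system.
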(event `self.ReceiveBeginPlay`
  ;[1 1 1 0.8] Event begin play
  (set `self.StoreManager` (`Actor.GetComponentByClass` (`GameplayStatics.GetGameState`) "/Game/GrandOpening/Blueprints/ActorComponents/BP_StoreManager.BP_StoreManager_C"))
  (`/Engine/EditorBlueprintResources/StandardMacros.IsValid` (`self.StoreManager`)
    (:`Is Valid`
      (add `/Game/GrandOpening/Blueprints/ActorComponents/BP_StoreManager.OnHourChanged` (`self.StoreManager`) (delegate `OnHourChanged_Event`))
      (`self.RestoreFromSave`))))

(event `OnHourChanged_Event`
  (params (Day :type Integer) (Hour :type Integer))
  ;[1 1 1 0.8] Event begin play
  ;;[1 1 1 0.8] On hour changed delegate
  (`self.DeliverDueOrders` Day Hour))

(fn `CollectInto`
  (params (Save :type "/Game/GrandOpening/Blueprints/Misc/SG_StoreSave Object Reference"))
  ;[1 1 1 0.8] Collect into
  (set `/Game/GrandOpening/Blueprints/Misc/SG_StoreSave.DeliveryOrders` (`self.PendingOrders`) Save))

(fn `DeliverDueOrders`
  (params (Day :type Integer) (Hour :type Integer))
  (locals (Remaining :type "Array of /Game/GrandOpening/Blueprints/Structures/S_PendingOrder Structure"))
  ;[1 1 1 0.8] Deliver due orders
  (for _array_element (`self.PendingOrders`)
    (bind (_product _cases _arrivalday _arrivalhour) (break `/Game/GrandOpening/Blueprints/Structures/S_PendingOrder` _array_element))
    (if (or (< _arrivalday Day) (and (== _arrivalday Day) (<= _arrivalhour Hour)))
      (`self.DeliverOrder` self _array_element)
      (else
        (`KismetArrayLibrary.Array_Add` (`local.Remaining`) _array_element))))
  (set `self.PendingOrders` (`local.Remaining`)))

(fn `DeliverOrder`
  (params (Order :type "/Game/GrandOpening/Blueprints/Structures/S_PendingOrder Structure"))
  (locals (Remaining :type Integer))
  (bind (_product _cases) (break `/Game/GrandOpening/Blueprints/Structures/S_PendingOrder` Order))
  (bind _bay (`self.Bay`))
  ;[1 1 1 0.8] Deliver order
  (bind _boxsize (`self.PickBoxFor` self _product))
  (`/Engine/EditorBlueprintResources/StandardMacros.IsValid` _boxsize
    (:`Is Valid`
      (`/Engine/EditorBlueprintResources/StandardMacros.IsValid` _bay
        (:`Is Valid`
          (set `local.Remaining` (* _cases (`/Game/GrandOpening/Blueprints/DataAssets/Products/BP_ProductDataAsset.UnitsPerCase` _product)))
          (bind _capacity (`/Game/GrandOpening/Blueprints/DataAssets/Boxes/BP_BoxDataAsset.CapacityFor` _boxsize _product))
          (while (> (`local.Remaining`) 0)
            (bind _slottransform (`/Game/GrandOpening/Blueprints/Environments/Misc/Zones/BP_DeliveryBay.TakeNextSlot` _bay))
            (bind _returnvalue (`KismetMathLibrary.Min` _capacity (`local.Remaining`)))
            (`|SpawnActorFromClass` "/Game/GrandOpening/Blueprints/Environments/Boxes/BP_DeliveryBoxBase.BP_DeliveryBoxBase_C" _slottransform "AdjustIfPossibleButAlwaysSpawn" "MultiplyWithRoot" null _product _returnvalue _boxsize null)
            (set `local.Remaining` (- (`local.Remaining`) _returnvalue))))))))

(fn `PickBoxFor`
  (params (Product :type "/Game/GrandOpening/Blueprints/DataAssets/Products/BP_ProductDataAsset Object Reference"))
  (returns (BoxSize :type "/Game/GrandOpening/Blueprints/DataAssets/Boxes/BP_BoxDataAsset Object Reference"))
  (locals (Best :type "/Game/GrandOpening/Blueprints/DataAssets/Boxes/BP_BoxDataAsset Object Reference") (BestCapacity :type Integer) (Capacity :type Integer))
  (bind _unitspercase (`/Game/GrandOpening/Blueprints/DataAssets/Products/BP_ProductDataAsset.UnitsPerCase` Product))
  ;[1 1 1 0.8] Pick box for
  (for _array_element (`self.BoxSizes`)
    (bind _capacity (`/Game/GrandOpening/Blueprints/DataAssets/Boxes/BP_BoxDataAsset.CapacityFor` _array_element Product))
    (set `local.Capacity` _capacity)
    (if (or (and (< (`local.BestCapacity`) _unitspercase) (> (`local.Capacity`) (`local.BestCapacity`))) (and (>= (`local.Capacity`) _unitspercase) (< (`local.Capacity`) (`local.BestCapacity`))))
      (set `local.Best` _array_element)
      (set `local.BestCapacity` (`local.Capacity`))))
  (return (`local.Best`)))

(fn `QueueOrder`
  (params (Product :type "/Game/GrandOpening/Blueprints/DataAssets/Products/BP_ProductDataAsset Object Reference") (Cases :type Integer))
  (locals (Hours :type Integer))
  (bind _storemanager (`self.StoreManager`))
  ;[1 1 1 0.8] Queue order
  (if (`/Game/GrandOpening/Blueprints/DataAssets/Products/BP_ProductDataAsset.DeliversNextDay` Product)
    (bind _hours (`/Game/GrandOpening/Blueprints/ActorComponents/BP_StoreManager.HoursUntilNextOpening` _storemanager))
    (set `local.Hours` _hours)
    (else
      (set `local.Hours` (`/Game/GrandOpening/Blueprints/DataAssets/Products/BP_ProductDataAsset.DeliveryDelayHours` Product))))
  (bind (_day _hour) (`/Game/GrandOpening/Blueprints/ActorComponents/BP_StoreManager.ClockAfterHours` _storemanager (`local.Hours`)))
  (`KismetArrayLibrary.Array_Add` (`self.PendingOrders`) (make `/Game/GrandOpening/Blueprints/Structures/S_PendingOrder` Product Cases _day _hour)))

(fn `RegisterBay`
  (params (NewBay :type "/Game/GrandOpening/Blueprints/Environments/Misc/Zones/BP_DeliveryBay Object Reference"))
  ;[1 1 1 0.8] Register bay
  (set `self.Bay` NewBay))

(fn `RestoreFromSave`
  ;[1 1 1 0.8] Restore from save
  (bind _asbp_store_game_instance (cast `/Game/GrandOpening/Blueprints/Misc/BP_StoreGameInstance` (`GameplayStatics.GetGameInstance`)))
  (bind _pendingsave (`/Game/GrandOpening/Blueprints/Misc/BP_StoreGameInstance.PendingSave` _asbp_store_game_instance))
  (`/Engine/EditorBlueprintResources/StandardMacros.IsValid` _pendingsave
    (:`Is Valid`
      (set `self.PendingOrders` (`/Game/GrandOpening/Blueprints/Misc/SG_StoreSave.DeliveryOrders` _pendingsave)))))
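; Customer AI component that runs a shopper's state machine from entering through browsing, queuing and paying to leaving, possibly angry.
; Archetype data and promoted ad categories decide wanted products within budget.
; UpdateTarget sets destinations and drains patience while waiting, and ActAtTarget performs shelf, checkout, payment-wait and exit steps.
; Shelf approach points use random navmesh samples with line-of-sight traces, and entrance doors gate movement through passage requests.
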(event `self.ReceiveBeginPlay`
  ;[1 1 1 0.8] Event begin play
  (bind _asbp_payment_offer (cast `/Game/GrandOpening/Blueprints/Environments/Checkout/Parts/Payment/BP_PaymentOffer` (`ChildActorComponent.ChildActor` (`Actor.GetComponentByClass` (`self.GetOwner` self) "/Script/Engine.ChildActorComponent"))))
  (bind _output_get (set `self.HeldOffer` _asbp_payment_offer))
  (add `/Game/GrandOpening/Blueprints/Environments/Checkout/Parts/Payment/BP_PaymentOffer.OnTaken` _output_get (`|CreateDelegate` :!event `HandOverPayment`)))

(event `self.ReceiveEndPlay`
  (params (EndPlayReason :type "EEndPlayReason Enum" :default "Destroyed"))
  ;[1 1 1 0.8] Event end play
  (`self.ReleaseDoors`))

(fn `ActAtTarget`
  (bind _returnvalue (`KismetSystemLibrary.GetGameTimeInSeconds`))
  (bind _returnvalue_2 (`KismetSystemLibrary.GetGameTimeInSeconds`))
  (bind _returnvalue_3 (`self.GetOwner` self))
  ;[1 1 1 0.8] Act at target
  (switch `/Game/GrandOpening/Blueprints/Enumerations/E_CustomerState` (`self.State`)
    (:`NewEnumerator1`
      (if (<= (`self.BrowseUntil`) 0.0)
        (set `self.BrowseUntil` (+ _returnvalue (`self.BrowseSeconds`)))
        (elif (>= _returnvalue (`self.BrowseUntil`))
          (set `self.BrowseUntil` 0.0)
          (set `self.State` "NewEnumerator2"))))
    (:`NewEnumerator2`
      (`self.PickFromShelf` self)
      (`self.ContinueShopping` self))
    (:`NewEnumerator8`
      (if (<= (`self.BrowseUntil`) 0.0)
        (set `self.BrowseUntil` (+ _returnvalue_2 (`self.BrowseSeconds`)))
        (elif (>= _returnvalue_2 (`self.BrowseUntil`))
          (set `self.BrowseUntil` 0.0)
          (`self.ChooseCheckout`))))
    (:`NewEnumerator3`
      (`self.PresentAtCheckout` self))
    (:`NewEnumerator4`
      (bind _index (`/Game/GrandOpening/Blueprints/Environments/Checkout/BP_CheckoutBase.SlotIndexOf` (`self.TargetCheckout`) (`self.GetOwner` self) :!label _label))
      (if (< _index 0)
        (set `self.State` "NewEnumerator6")))
    (:`NewEnumerator5`
      (goto _label))
    (:`NewEnumerator6`
      (if (<= (`KismetMathLibrary.Vector_Distance` (`Actor.K2_GetActorLocation` _returnvalue_3) (`self.ExitLocation`)) 150.0) :!label _label_2
        (`Actor.K2_DestroyActor` _returnvalue_3)))
    (:`NewEnumerator7`
      (goto _label_2))))

(fn `AddToBasket`
  (params (Product :type "/Game/GrandOpening/Blueprints/DataAssets/Products/BP_ProductDataAsset Object Reference"))
  ;[1 1 1 0.8] Add to basket
  (`KismetArrayLibrary.Array_Add` (`self.Basket`) (make `/Game/GrandOpening/Blueprints/Structures/S_BasketItem` Product 1)))

(fn `AdvanceQueue`
  (params (DeltaSeconds :type "Float (double-precision)"))
  (bind _targetcheckout (`self.TargetCheckout`))
  (bind _returnvalue (`self.GetOwner` self))
  ;[1 1 1 0.8] Advance queue
  (if (== (`/Game/GrandOpening/Blueprints/Environments/Checkout/BP_CheckoutBase.CurrentCustomer` _targetcheckout) _returnvalue)
    (bind _location (`/Game/GrandOpening/Blueprints/Environments/Checkout/BP_CheckoutBase.BuyerSpotLocation` _targetcheckout))
    (set `self.TargetLocation` _location)
    (else
      (set `self.PatienceLeft` (- (`self.PatienceLeft`) DeltaSeconds))
      (if (<= (`self.PatienceLeft`) 0)
        (`/Game/GrandOpening/Blueprints/Environments/Checkout/BP_CheckoutBase.LeaveQueue` _targetcheckout _returnvalue)
        (`self.LeaveAngry` self)
        (`/Game/GrandOpening/Blueprints/ActorComponents/BP_ReactionComponent.React` (`Actor.GetComponentByClass` _returnvalue "/Game/GrandOpening/Blueprints/ActorComponents/BP_ReactionComponent.BP_ReactionComponent_C") "NewEnumerator2" "")
        (set `self.TargetLocation` (`self.ExitLocation`))
        (else
          (bind _index (`/Game/GrandOpening/Blueprints/Environments/Checkout/BP_CheckoutBase.SlotIndexOf` _targetcheckout _returnvalue))
          (if (== _index 0)
            (bind _location_2 (`/Game/GrandOpening/Blueprints/Environments/Checkout/BP_CheckoutBase.BuyerSpotLocation` _targetcheckout))
            (set `self.TargetLocation` _location_2)
            (else
              (bind _slot (`/Game/GrandOpening/Blueprints/Environments/Checkout/BP_CheckoutBase.SlotWorldTransform` _targetcheckout _index))
              (set `self.TargetLocation` (.location _slot)))))))))

(fn `ApproachPointFor`
  (params (Shelf :type "/Game/GrandOpening/Blueprints/Environments/Shelves/BP_ShelfBase Object Reference"))
  (returns (Location :type "Vector Structure") (Found :type Boolean))
  (bind (_origin _boxextent) (`Actor.GetActorBounds` Shelf false false))
  (bind _returnvalue (`KismetMathLibrary.MakeVector` 0.0 0.0 (`self.EyeHeightCm`)))
  (bind _returnvalue_2 (- _origin (`KismetMathLibrary.MakeVector` 0.0 0.0 (.z _boxextent))))
  ;[1 1 1 0.8] Approach point for
  (for _ (range (`self.ApproachTries`))
    (bind (_randomlocation _returnvalue_3) (`NavigationSystemV1.K2_GetRandomLocationInNavigableRadius` _returnvalue_2 (+ (`KismetMathLibrary.FMax` (.x _boxextent) (.y _boxextent)) (`self.StandOffCm`)) null null))
    (if _returnvalue_3
      (bind (_outhit _returnvalue_4) (`KismetSystemLibrary.LineTraceSingle` (+ _randomlocation _returnvalue) (+ _returnvalue_2 _returnvalue) "TraceTypeQuery1" false (`|MakeArray` Shelf :!type "Actor Object Reference")))
      (if (not _returnvalue_4)
        (return _randomlocation true))))
  (return (0.0 0.0 0.0) false))

(fn `AvoidsOthers`
  (returns (ReturnValue :type Boolean))
  ;[1 1 1 0.8] Avoids others
  (return (and (`|EnumInequality` (`self.State`) "NewEnumerator3") (> (`KismetMathLibrary.Vector_Distance` (`Actor.K2_GetActorLocation` (`self.GetOwner`)) (`self.TargetLocation`)) (`self.ArrivalAvoidanceCm`)))))

(fn `BeginPayment`
  (bind _heldoffer (`self.HeldOffer`))
  ;[1 1 1 0.8] Begin payment
  (switch `/Game/GrandOpening/Blueprints/Enumerations/E_PaymentType` (`KismetArrayLibrary.Array_Random` (`/Game/GrandOpening/Blueprints/Environments/Checkout/BP_CheckoutBase.AcceptedPayments` (`self.TargetCheckout`)))
    (:`NewEnumerator0`
      (set `self.State` "NewEnumerator4")
      (`/Game/GrandOpening/Blueprints/Environments/Checkout/Parts/Payment/BP_PaymentOffer.OfferCash` _heldoffer))
    (:`NewEnumerator1`
      (set `self.State` "NewEnumerator5")
      (`/Game/GrandOpening/Blueprints/Environments/Checkout/Parts/Payment/BP_PaymentOffer.OfferCard` _heldoffer))))

(fn `ChooseCheckout`
  ;[1 1 1 0.8] Choose checkout
  (set `self.TargetCheckout` null)
  (bind _outactors (`GameplayStatics.GetAllActorsOfClass` "/Game/GrandOpening/Blueprints/Environments/Checkout/BP_CheckoutBase.BP_CheckoutBase_C"))
  (for _array_element _outactors
    (bind _joined (`/Game/GrandOpening/Blueprints/Environments/Checkout/BP_CheckoutBase.TryJoinQueue` _array_element (`self.GetOwner` self)))
    (if _joined
      (set `self.TargetCheckout` _array_element)
      (set `self.State` "NewEnumerator3")
      (break)))
  (`/Engine/EditorBlueprintResources/StandardMacros.IsValid` (`self.TargetCheckout`)
    (:`Is Not Valid`
      (`self.WanderForCheckout` self))))

(fn `ChooseShelf`
  (locals (WantedShelves :type "Array of /Game/GrandOpening/Blueprints/Environments/Shelves/BP_ShelfBase Object Reference") (Placed :type Boolean))
  (bind _wantedshelves (`local.WantedShelves`))
  ;[1 1 1 0.8] Choose shelf
  (bind _outactors (`GameplayStatics.GetAllActorsOfClass` "/Game/GrandOpening/Blueprints/Environments/Shelves/BP_ShelfBase.BP_ShelfBase_C"))
  (for _array_element _outactors
    (bind _product (`self.WantedProductOn` self _array_element))
    (`/Engine/EditorBlueprintResources/StandardMacros.IsValid` _product
      (:`Is Valid`
        (`KismetArrayLibrary.Array_Add` (`local.WantedShelves`) _array_element))))
  (while (and (not (`local.Placed`)) (> (`KismetArrayLibrary.Array_Length` _wantedshelves) 0))
    (bind _output_get (set `self.TargetShelf` (`KismetArrayLibrary.Array_Random` _wantedshelves)))
    (bind (_location _found) (`self.ApproachPointFor` self _output_get))
    (if _found
      (set `self.TargetLocation` _location)
      (set `self.BrowseUntil` 0.0)
      (set `self.State` "NewEnumerator1")
      (set `local.Placed` true)
      (else
        (`KismetArrayLibrary.Array_RemoveItem` _wantedshelves _output_get))))
  (if (== (`KismetArrayLibrary.Array_Length` _wantedshelves) 0)
    (`self.ReportStockOut` self)
    (if (> (`KismetArrayLibrary.Array_Length` (`self.Basket`)) 0)
      (`self.ChooseCheckout` self)
      (else
        (set `self.State` "NewEnumerator6")))))

(fn `ContinueShopping`
  ;[1 1 1 0.8] Continue shopping
  (if (>= (`KismetArrayLibrary.Array_Length` (`self.Basket`)) (`self.TargetItems`))
    (`self.ChooseCheckout` self)
    (else
      (`self.ChooseShelf` self))))

(fn `GetFocusPoint`
  (returns (Point :type "Vector Structure") (HasFocus :type Boolean))
  (bind _targetcheckout (`self.TargetCheckout`))
  (bind _targetshelf (`self.TargetShelf`))
  (bind _returnvalue (`self.GetOwner` self))
  ;[1 1 1 0.8] Get focus point
  (if (> (`self.BrowseUntil`) 0.0)
    (`/Engine/EditorBlueprintResources/StandardMacros.IsValid` _targetshelf
      (:`Is Valid`
        (return (`Actor.K2_GetActorLocation` _targetshelf) true))
      (:`Is Not Valid`
        _))
    (else
      (`/Engine/EditorBlueprintResources/StandardMacros.IsValid` _targetcheckout
        (:`Is Valid`
          (if (== (`/Game/GrandOpening/Blueprints/Environments/Checkout/BP_CheckoutBase.CurrentCustomer` _targetcheckout) _returnvalue)
            (bind _location (`/Game/GrandOpening/Blueprints/Environments/Checkout/BP_CheckoutBase.CashierSpotLocation` _targetcheckout))
            (return _location true)
            (else
              (bind _index (`/Game/GrandOpening/Blueprints/Environments/Checkout/BP_CheckoutBase.SlotIndexOf` _targetcheckout _returnvalue))
              (if (>= _index 0)
                (bind _slot (`/Game/GrandOpening/Blueprints/Environments/Checkout/BP_CheckoutBase.SlotWorldTransform` _targetcheckout _index))
                (return (- (.location _slot) (* (`KismetMathLibrary.GetForwardVector` (.rotation _slot)) 500.0)) true)
                (else
                  (return (`KismetMathLibrary.MakeVector` 0.0) false))))))
        (:`Is Not Valid`
          _))))
  (return (`KismetMathLibrary.MakeVector` 0.0) false))

(fn `HandOverPayment`
  (bind _targetcheckout (`self.TargetCheckout`))
  (bind _heldoffer (`self.HeldOffer`))
  ;[1 1 1 0.8] Hand over payment
  (switch `/Game/GrandOpening/Blueprints/Enumerations/E_CustomerState` (`self.State`)
    (:`NewEnumerator4`
      (bind _amount (`/Game/GrandOpening/Blueprints/Environments/Checkout/BP_CheckoutBase.CashOffer` _targetcheckout))
      (`/Game/GrandOpening/Blueprints/Environments/Checkout/BP_CheckoutBase.TakeCash` _targetcheckout _amount)
      (`/Game/GrandOpening/Blueprints/Environments/Checkout/Parts/Payment/BP_PaymentOffer.Withdraw` _heldoffer))
    (:`NewEnumerator5`
      (`/Game/GrandOpening/Blueprints/Environments/Checkout/BP_CheckoutBase.TakeCard` _targetcheckout (`Actor.GetTransform` _heldoffer))
      (`/Game/GrandOpening/Blueprints/Environments/Checkout/Parts/Payment/BP_PaymentOffer.Withdraw` _heldoffer))))

(fn `HoldsPosition`
  (returns (ReturnValue :type Boolean))
  (locals (Held :type Boolean))
  ;[1 1 1 0.8] Holds position
  (set `local.Held` false)
  (for _array_element (`self.Doors`)
    (bind _returnvalue (`/Game/GrandOpening/Blueprints/Environments/Openings/BP_EntranceDoor.RequestPassage` _array_element (`self.GetOwner`) (`self.TargetLocation`)))
    (if (not _returnvalue)
      (set `local.Held` true)))
  (return (`local.Held`)))

(fn `InitializeCustomer`
  (bind _archetype (`self.Archetype`))
  (bind _returnvalue (`Actor.GetComponentByClass` (`GameplayStatics.GetGameState`) "/Game/GrandOpening/Blueprints/ActorComponents/BP_AdManager.BP_AdManager_C"))
  ;[1 1 1 0.8] Initialize customer
  (bind _returnvalue_2 (`GameplayStatics.GetActorOfClass` "/Game/GrandOpening/Blueprints/Environments/Misc/Zones/BP_CustomerExit.BP_CustomerExit_C"))
  (set `self.ExitLocation` (`Actor.K2_GetActorLocation` _returnvalue_2))
  (set `self.BudgetValue` (`KismetMathLibrary.RandomFloatInRange` (`/Game/GrandOpening/Blueprints/DataAssets/Customers/BP_CustomerArchetypeDataAsset.BudgetMin` _archetype) (`/Game/GrandOpening/Blueprints/DataAssets/Customers/BP_CustomerArchetypeDataAsset.BudgetMax` _archetype)))
  (set `self.TargetItems` (`KismetMathLibrary.RandomIntegerInRange` (`/Game/GrandOpening/Blueprints/DataAssets/Customers/BP_CustomerArchetypeDataAsset.TargetItemsMin` _archetype) (`/Game/GrandOpening/Blueprints/DataAssets/Customers/BP_CustomerArchetypeDataAsset.TargetItemsMax` _archetype)))
  (set `self.PatienceLeft` (`/Game/GrandOpening/Blueprints/DataAssets/Customers/BP_CustomerArchetypeDataAsset.PatienceSeconds` _archetype))
  (set `CharacterMovementComponent.MaxWalkSpeed` (`/Game/GrandOpening/Blueprints/DataAssets/Customers/BP_CustomerArchetypeDataAsset.WalkSpeed` _archetype) (`Actor.GetComponentByClass` (`self.GetOwner` self) "/Script/Engine.CharacterMovementComponent"))
  (set `self.State` "NewEnumerator0")
  (`/Game/GrandOpening/Blueprints/ActorComponents/BP_CosmeticComponent.ApplyCosmeticSet` (`Actor.GetComponentByClass` (`self.GetOwner`) "/Game/GrandOpening/Blueprints/ActorComponents/BP_CosmeticComponent.BP_CosmeticComponent_C") (`/Game/GrandOpening/Blueprints/DataAssets/Customers/BP_CustomerArchetypeDataAsset.CosmeticSet` _archetype))
  (set `self.BrowseSeconds` (`/Game/GrandOpening/Blueprints/DataAssets/Customers/BP_CustomerArchetypeDataAsset.BrowseSeconds` _archetype))
  (`self.OnInitialized`)
  (bind _outactors (`GameplayStatics.GetAllActorsOfClass` "/Game/GrandOpening/Blueprints/Environments/Openings/BP_EntranceDoor.BP_EntranceDoor_C"))
  (set `self.Doors` _outactors)
  (`/Engine/EditorBlueprintResources/StandardMacros.IsValid` _returnvalue
    (:`Is Valid`
      (bind _categories (`/Game/GrandOpening/Blueprints/ActorComponents/BP_AdManager.PromotedCategories` _returnvalue))
      (set `self.PromotedCategories` _categories))))

(fn `IsOfferingPayment`
  (returns (Offering :type Boolean))
  (bind _heldoffer (`self.HeldOffer`))
  ;[1 1 1 0.8] Is offering payment
  (`/Engine/EditorBlueprintResources/StandardMacros.IsValid` _heldoffer
    (:`Is Valid`
      (return (not (`Actor.bHidden` _heldoffer))))
    (:`Is Not Valid`
      (return false))))

(fn `IsProductWanted`
  (params (Product :type "/Game/GrandOpening/Blueprints/DataAssets/Products/BP_ProductDataAsset Object Reference"))
  (returns (Wanted :type Boolean))
  (bind _archetype (`self.Archetype`))
  (bind _budgetvalue (`self.BudgetValue`))
  ;[1 1 1 0.8] Is product wanted
  (`/Engine/EditorBlueprintResources/StandardMacros.IsValid` Product
    (:`Is Valid`
      (`/Engine/EditorBlueprintResources/StandardMacros.IsValid` _archetype
        (:`Is Valid`
          (bind _wanted (`/Game/GrandOpening/Blueprints/DataAssets/Customers/BP_CustomerArchetypeDataAsset.GetWants` _archetype Product _budgetvalue))
          (if _wanted
            (return true)
            (else
              (return (and (`KismetArrayLibrary.Array_Contains` (`self.PromotedCategories`) (`/Game/GrandOpening/Blueprints/DataAssets/Products/BP_ProductDataAsset.Category` Product)) (<= (`/Game/GrandOpening/Blueprints/DataAssets/Products/BP_ProductDataAsset.SuggestedPrice` Product) _budgetvalue))))))
        (:`Is Not Valid`
          (return false))))
    (:`Is Not Valid`
      (return false))))

(fn `LeaveAngry`
  ;[1 1 1 0.8] Leave angry
  (set `self.State` "NewEnumerator7")
  (`/Game/GrandOpening/Blueprints/ActorComponents/BP_StoreManager.AddCustomerLost` (`Actor.GetComponentByClass` (`GameplayStatics.GetGameState`) "/Game/GrandOpening/Blueprints/ActorComponents/BP_StoreManager.BP_StoreManager_C")))

(fn `PickFromShelf`
  (bind _targetshelf (`self.TargetShelf`))
  ;[1 1 1 0.8] Pick from shelf
  (bind _product (`self.WantedProductOn` self _targetshelf))
  (`/Engine/EditorBlueprintResources/StandardMacros.IsValid` _product
    (:`Is Valid`
      (`/Game/GrandOpening/Blueprints/Environments/Shelves/BP_ShelfBase.TakeOneOf` _targetshelf _product)
      (`self.AddToBasket` self _product)
      (set `self.BudgetValue` (- (`self.BudgetValue`) (`/Game/GrandOpening/Blueprints/DataAssets/Products/BP_ProductDataAsset.SuggestedPrice` _product))))))

(fn `PresentAtCheckout`
  (bind _targetcheckout (`self.TargetCheckout`))
  (bind _returnvalue (`self.GetOwner` self))
  ;[1 1 1 0.8] Present at checkout
  (bind _index (`/Game/GrandOpening/Blueprints/Environments/Checkout/BP_CheckoutBase.SlotIndexOf` _targetcheckout _returnvalue))
  (if (== _index 0)
    (`/Game/GrandOpening/Blueprints/Environments/Checkout/BP_CheckoutBase.PresentBasket` _targetcheckout _returnvalue (`self.Basket`))))

(fn `ReleaseDoors`
  ;[1 1 1 0.8] Release doors
  (for _array_element (`self.Doors`)
    (`/Game/GrandOpening/Blueprints/Environments/Openings/BP_EntranceDoor.ReleasePassage` _array_element (`self.GetOwner`))))

(fn `ReportStockOut`
  (bind _archetype (`self.Archetype`))
  ;[1 1 1 0.8] Report stock out
  (if (not (`self.ReportedStockOut`))
    (set `self.ReportedStockOut` true)
    (`/Game/GrandOpening/Blueprints/ActorComponents/BP_StoreManager.AddStockOut` (`Actor.GetComponentByClass` (`GameplayStatics.GetGameState`) "/Game/GrandOpening/Blueprints/ActorComponents/BP_StoreManager.BP_StoreManager_C"))
    (`/Engine/EditorBlueprintResources/StandardMacros.IsValid` _archetype
      (:`Is Valid`
        (`/Game/GrandOpening/Blueprints/ActorComponents/BP_ReactionComponent.React` (`Actor.GetComponentByClass` (`self.GetOwner` self) "/Game/GrandOpening/Blueprints/ActorComponents/BP_ReactionComponent.BP_ReactionComponent_C") "NewEnumerator1" (`KismetTextLibrary.Conv_StringToText` (`|GetEnumeratorNameAsString` (`|GetArrayItem` (`/Game/GrandOpening/Blueprints/DataAssets/Customers/BP_CustomerArchetypeDataAsset.PreferredCategories` _archetype)))))))))

(fn `UpdateTarget`
  (params (DeltaSeconds :type "Float (double-precision)"))
  ;[1 1 1 0.8] Update target
  (switch `/Game/GrandOpening/Blueprints/Enumerations/E_CustomerState` (`self.State`)
    (:`NewEnumerator0`
      (`self.ChooseShelf` self))
    (:`NewEnumerator8`
      (set `self.PatienceLeft` (- (`self.PatienceLeft`) DeltaSeconds))
      (if (<= (`self.PatienceLeft`) 0.0)
        (`self.LeaveAngry` self)
        (set `self.TargetLocation` (`self.ExitLocation`))))
    (:`NewEnumerator3`
      (`self.AdvanceQueue` self DeltaSeconds))
    (:`NewEnumerator6`
      (set `self.TargetLocation` (`self.ExitLocation`)))
    (:`NewEnumerator7`
      (set `self.TargetLocation` (`self.ExitLocation`)))))

(fn `WanderForCheckout`
  ;[1 1 1 0.8] Wander for checkout
  (set `self.BrowseUntil` 0.0)
  (set `self.State` "NewEnumerator8")
  (set `self.TargetLocation` (`Actor.K2_GetActorLocation` (`self.GetOwner` self)))
  (set `self.TargetShelf` null)
  (bind _volume (`/Game/GrandOpening/Blueprints/Functions/BFL_Zones.FindZoneVolume` "NewEnumerator0" self))
  (`/Engine/EditorBlueprintResources/StandardMacros.IsValid` _volume
    (:`Is Valid`
      (bind (_point _found) (`/Game/GrandOpening/Blueprints/Environments/Build/BP_StoreZoneVolume.RandomNavigablePoint` _volume))
      (if _found
        (set `self.TargetLocation` _point)))))

(fn `WantedProductOn`
  (params (Shelf :type "/Game/GrandOpening/Blueprints/Environments/Shelves/BP_ShelfBase Object Reference"))
  (returns (Product :type "/Game/GrandOpening/Blueprints/DataAssets/Products/BP_ProductDataAsset Object Reference"))
  ;[1 1 1 0.8] Wanted product on
  (bind _products (`/Game/GrandOpening/Blueprints/Environments/Shelves/BP_ShelfBase.StockedProducts` Shelf))
  (for _array_element _products
    (bind _wanted (`self.IsProductWanted` self _array_element))
    (if _wanted
      (return _array_element)))
  (return null))
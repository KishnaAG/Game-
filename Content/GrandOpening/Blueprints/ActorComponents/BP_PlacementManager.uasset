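; Player component for the store's build mode: placing structures from stock and picking up placed ones, with a preview ghost, build menu and action prompts.
; Each tick a camera trace moves the ghost, grid-snapped in a frame aligned to floor, wall or ceiling.
; Validation checks surface type, store zone and overlaps with placeables or customers.
; Edit mode returns a targeted structure to stock and re-arms it, unless it is a busy checkout or stocked shelf.
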(event `self.ReceiveBeginPlay`
  ;[1 1 1 0.8] Event begin play
  (bind _ascharacter (cast `Character` (`self.GetOwner`)))
  (set `self.ViewCamera` (`Actor.GetComponentByClass` _ascharacter "/Script/Engine.CameraComponent"))
  (set `self.Interaction` (`Actor.GetComponentByClass` _ascharacter "/Game/GrandOpening/Blueprints/ActorComponents/BP_InteractionComponent.BP_InteractionComponent_C"))
  (bind _asbp_store_game_state (cast `/Game/GrandOpening/Blueprints/Misc/BP_StoreGameState` (`GameplayStatics.GetGameState`)))
  (set `self.StoreManager` (`/Game/GrandOpening/Blueprints/Misc/BP_StoreGameState.BP_StoreManager` _asbp_store_game_state)))

(event `self.ReceiveTick`
  (params (DeltaSeconds :type "Float (single-precision)"))
  ;[1 1 1 0.8] Event tick
  (if (`self.Building`)
    (if (`self.Editing`)
      (`self.UpdateEditGhost`)
      (else
        (`self.UpdateGhost`)))))

(fn `AllowsSurface`
  (params (Structure :type "/Game/GrandOpening/Blueprints/DataAssets/Structures/BP_StructureDataAsset Object Reference") (SurfaceNormal :type "Vector Structure"))
  (returns (Allowed :type Boolean))
  ;[1 1 1 0.8] Allows surface
  (return (select `bool` (>= (.z SurfaceNormal) 0.7) :`false` (select `bool` (<= (.z SurfaceNormal) -0.7) :`false` (`/Game/GrandOpening/Blueprints/DataAssets/Structures/BP_StructureDataAsset.CanPlaceOnWall` Structure) :`true` (`/Game/GrandOpening/Blueprints/DataAssets/Structures/BP_StructureDataAsset.CanPlaceOnCeiling` Structure)) :`true` (`/Game/GrandOpening/Blueprints/DataAssets/Structures/BP_StructureDataAsset.CanPlaceOnFloor` Structure))))

(fn `ArmStructure`
  (params (Structure :type "/Game/GrandOpening/Blueprints/DataAssets/Structures/BP_StructureDataAsset Object Reference") (Rotation :type "Rotator Structure"))
  (bind _ghostactor (`self.GhostActor`))
  ;[1 1 1 0.8] Arm structure
  (set `self.ArmedStructure` Structure)
  (set `self.GhostRotation` Rotation)
  (`/Game/GrandOpening/Blueprints/Environments/Build/BP_PlacementGhost.SetPreviewMesh` _ghostactor (`/Game/GrandOpening/Blueprints/DataAssets/Structures/BP_StructureDataAsset.PreviewMesh` Structure))
  (`self.RefreshBuildActions`)
  (`/Game/GrandOpening/Blueprints/Environments/Build/BP_PlacementGhost.SetCellLayout` _ghostactor (`/Game/GrandOpening/Blueprints/DataAssets/Structures/BP_StructureDataAsset.FootprintCells` Structure) (`/Game/GrandOpening/Blueprints/DataAssets/Structures/BP_StructureDataAsset.SnapStepCm` Structure)))

(fn `CloseBuildMenu`
  (bind _returnvalue (`GameplayStatics.GetPlayerController` 0))
  ;[1 1 1 0.8] Close build menu
  (`/Engine/EditorBlueprintResources/StandardMacros.IsValid` (`self.BuildMenu`)
    (:`Is Valid`
      (`Widget.RemoveFromParent` (`self.BuildMenu`))
      (set `self.BuildMenu` null)
      (`WidgetBlueprintLibrary.SetInputMode_GameOnly` _returnvalue)
      (set `PlayerController.bShowMouseCursor` false _returnvalue))))

(fn `ConfirmPlacement`
  (bind _armedstructure (`self.ArmedStructure`))
  (bind _storemanager (`self.StoreManager`))
  ;[1 1 1 0.8] Confirm placement
  (if (`self.CanPlace`)
    (bind _taken (`/Game/GrandOpening/Blueprints/ActorComponents/BP_StoreManager.TakeStructureFromStock` _storemanager _armedstructure))
    (if _taken
      (bind _returnvalue (`|SpawnActorFromClass` (`/Game/GrandOpening/Blueprints/DataAssets/Structures/BP_StructureDataAsset.PlacedClass` _armedstructure) (`Actor.GetTransform` (`self.GhostActor`)) "AlwaysSpawn" "MultiplyWithRoot" null null))
      (set `/Game/GrandOpening/Blueprints/ActorComponents/BP_PlaceableComponent.Structure` _armedstructure (`Actor.GetComponentByClass` _returnvalue "/Game/GrandOpening/Blueprints/ActorComponents/BP_PlaceableComponent.BP_PlaceableComponent_C"))
      (if (not (`KismetArrayLibrary.Array_Contains` (`/Game/GrandOpening/Blueprints/ActorComponents/BP_StoreManager.OwnedStructures` _storemanager) _armedstructure))
        (`self.StopBuilding`)))))

(fn `IsLocationAllowedFor`
  (params (Structure :type "/Game/GrandOpening/Blueprints/DataAssets/Structures/BP_StructureDataAsset Object Reference") (Location :type "Vector Structure"))
  (returns (Allowed :type Boolean))
  (locals (Found :type Boolean))
  (bind _allowedzones (`/Game/GrandOpening/Blueprints/DataAssets/Structures/BP_StructureDataAsset.AllowedZones` Structure))
  ;[1 1 1 0.8] Is location allowed for
  (bind _outactors (`GameplayStatics.GetAllActorsOfClass` "/Game/GrandOpening/Blueprints/Environments/Build/BP_StoreZoneVolume.BP_StoreZoneVolume_C"))
  (for _array_element _outactors
    (bind _returnvalue (`KismetMathLibrary.InverseTransformLocation` (`Actor.GetTransform` _array_element) Location))
    (bind _returnvalue_2 (`BoxComponent.GetScaledBoxExtent` (`/Game/GrandOpening/Blueprints/Environments/Build/BP_StoreZoneVolume.ZoneBounds` _array_element)))
    (if (and (and (`KismetMathLibrary.InRange_FloatFloat` (.x _returnvalue) (- 0.0 (.x _returnvalue_2)) (.x _returnvalue_2)) (`KismetMathLibrary.InRange_FloatFloat` (.y _returnvalue) (- 0.0 (.y _returnvalue_2)) (.y _returnvalue_2))) (or (== (`KismetArrayLibrary.Array_Length` _allowedzones) 0) (`KismetArrayLibrary.Array_Contains` _allowedzones (`/Game/GrandOpening/Blueprints/Environments/Build/BP_StoreZoneVolume.Zone` _array_element))))
      (set `local.Found` true)))
  (return (`local.Found`)))

(fn `OpenBuildMenu`
  (bind _returnvalue (`GameplayStatics.GetPlayerController` 0))
  ;[1 1 1 0.8] Open build menu
  (bind _returnvalue_2 (`|CreateWidget` "/Game/GrandOpening/Blueprints/Widgets/Gameplay/BP_BuildMenuWidget.BP_BuildMenuWidget_C"))
  (set `/Game/GrandOpening/Blueprints/Widgets/Gameplay/BP_BuildMenuWidget.PlacementManager` self _returnvalue_2)
  (set `self.BuildMenu` _returnvalue_2)
  (`UserWidget.AddToViewport` _returnvalue_2 0)
  (`WidgetBlueprintLibrary.SetInputMode_UIOnlyEx` _returnvalue _returnvalue_2 "DoNotLock" true)
  (set `PlayerController.bShowMouseCursor` true _returnvalue))

(fn `PickUpStructure`
  (bind _edittarget (`self.EditTarget`))
  (bind _structure (`/Game/GrandOpening/Blueprints/ActorComponents/BP_PlaceableComponent.Structure` (`Actor.GetComponentByClass` _edittarget "/Game/GrandOpening/Blueprints/ActorComponents/BP_PlaceableComponent.BP_PlaceableComponent_C")))
  ;[1 1 1 0.8] Pickup structure
  (if (and (`self.Editing`) (`self.CanPickUp`))
    (bind _frame (`self.SurfaceFrame` (`Actor.GetActorUpVector` _edittarget)))
    (`/Game/GrandOpening/Blueprints/ActorComponents/BP_StoreManager.AddStructureToStock` (`self.StoreManager`) _structure)
    (set `self.Editing` false)
    (`/Game/GrandOpening/Blueprints/Widgets/Gameplay/BP_CrosshairWidget.HideMode` (`/Game/GrandOpening/Blueprints/ActorComponents/BP_InteractionComponent.Crosshair` (`self.Interaction`)))
    (`self.ArmStructure` _structure (`KismetMathLibrary.ComposeRotators` (`Actor.K2_GetActorRotation` _edittarget) (`KismetMathLibrary.NegateRotator` _frame)))
    (`Actor.K2_DestroyActor` _edittarget)))

(fn `PlacementNormal`
  (params (Structure :type "/Game/GrandOpening/Blueprints/DataAssets/Structures/BP_StructureDataAsset Object Reference") (SurfaceNormal :type "Vector Structure"))
  (returns (Normal :type "Vector Structure") (Allowed :type Boolean))
  ;[1 1 1 0.8] Placement normal
  (bind _allowed (`self.AllowsSurface` Structure SurfaceNormal))
  (return (select `bool` _allowed :`false` (`KismetMathLibrary.Vector_Up`) :`true` SurfaceNormal) _allowed))

(fn `PresentGhostResult`
  (params (Valid :type Boolean) (Reason :type Text))
  (bind _ghostactor (`self.GhostActor`))
  (bind _ghostmesh (`/Game/GrandOpening/Blueprints/Environments/Build/BP_PlacementGhost.GhostMesh` _ghostactor))
  ;[1 1 1 0.8] Present ghost result
  (`/Game/GrandOpening/Blueprints/Environments/Build/BP_PlacementGhost.SetFootprintValid` _ghostactor Valid)
  (bind _asbp_actions_widget (cast `/Game/GrandOpening/Blueprints/Widgets/Gameplay/BP_ActionsWidget` (`WidgetComponent.GetUserWidgetObject` (`/Game/GrandOpening/Blueprints/Environments/Build/BP_PlacementGhost.PromptWidget` _ghostactor))))
  (`/Game/GrandOpening/Blueprints/Widgets/Gameplay/BP_ActionsWidget.SetHint` _asbp_actions_widget Reason)
  (for _index (range (`PrimitiveComponent.GetNumMaterials` _ghostmesh))
    (`PrimitiveComponent.SetMaterial` _ghostmesh _index (select `bool` Valid :`false` (`self.GhostInvalidMaterial`) :`true` (`self.GhostValidMaterial`)))))

(fn `RefreshBuildActions`
  ;[1 1 1 0.8] Refresh build actions
  (bind _asbp_actions_widget (cast `/Game/GrandOpening/Blueprints/Widgets/Gameplay/BP_ActionsWidget` (`WidgetComponent.GetUserWidgetObject` (`/Game/GrandOpening/Blueprints/Environments/Build/BP_PlacementGhost.PromptWidget` (`self.GhostActor`)))))
  (`/Game/GrandOpening/Blueprints/Widgets/Gameplay/BP_ActionsWidget.ClearActions` _asbp_actions_widget)
  (`/Game/GrandOpening/Blueprints/Widgets/Gameplay/BP_ActionsWidget.AddAction` _asbp_actions_widget (`self.PlaceAction`) (`self.PlaceLabel`))
  (`/Game/GrandOpening/Blueprints/Widgets/Gameplay/BP_ActionsWidget.AddAction` _asbp_actions_widget (`self.RotateAction`) (`self.RotateLabel`))
  (`/Game/GrandOpening/Blueprints/Widgets/Gameplay/BP_ActionsWidget.AddAction` _asbp_actions_widget (`self.ExitAction`) (`self.ExitLabel`)))

(fn `RefreshEditActions`
  ;[1 1 1 0.8] Refresh edit actions
  (bind _asbp_actions_widget (cast `/Game/GrandOpening/Blueprints/Widgets/Gameplay/BP_ActionsWidget` (`WidgetComponent.GetUserWidgetObject` (`/Game/GrandOpening/Blueprints/Environments/Build/BP_PlacementGhost.PromptWidget` (`self.GhostActor`)))))
  (`/Game/GrandOpening/Blueprints/Widgets/Gameplay/BP_ActionsWidget.ClearActions` _asbp_actions_widget)
  (`/Game/GrandOpening/Blueprints/Widgets/Gameplay/BP_ActionsWidget.AddAction` _asbp_actions_widget (`self.PickUpAction`) (`self.PickUpLabel`))
  (`/Game/GrandOpening/Blueprints/Widgets/Gameplay/BP_ActionsWidget.AddAction` _asbp_actions_widget (`self.ExitAction`) (`self.ExitLabel`)))

(fn `RotateGhost`
  ;[1 1 1 0.8] Rotate ghost
  (set `self.GhostRotation` (`KismetMathLibrary.ComposeRotators` (`self.GhostRotation`) (`/Game/GrandOpening/Blueprints/DataAssets/Structures/BP_StructureDataAsset.RotationStep` (`self.ArmedStructure`)))))

(fn `SnapToSurface`
  (params (WorldLocation :type "Vector Structure") (SurfaceNormal :type "Vector Structure") (Footprint :type "IntPoint Structure") (StepCm :type "Float (double-precision)"))
  (returns (Snapped :type "Vector Structure"))
  (bind (_x _y) (break `IntPoint` Footprint))
  (bind _returnvalue (* StepCm 0.5))
  (bind _returnvalue_2 (* _returnvalue (`KismetMathLibrary.Conv_IntToDouble` _x)))
  (bind _returnvalue_3 (* _returnvalue (`KismetMathLibrary.Conv_IntToDouble` _y)))
  ;[1 1 1 0.8] Snap to surface
  (bind _frame (`self.SurfaceFrame` SurfaceNormal))
  (bind _returnvalue_4 (`KismetMathLibrary.LessLess_VectorRotator` WorldLocation _frame))
  (return (`KismetMathLibrary.GreaterGreater_VectorRotator` (`KismetMathLibrary.MakeVector` (+ (* StepCm (`KismetMathLibrary.Round` (/ (- (.x _returnvalue_4) _returnvalue_2) StepCm))) _returnvalue_2) (+ (* StepCm (`KismetMathLibrary.Round` (/ (- (.y _returnvalue_4) _returnvalue_3) StepCm))) _returnvalue_3) (.z _returnvalue_4)) _frame)))

(fn `StartEditing`
  ;[1 1 1 0.8] Start editing
  (set `self.Editing` true)
  (`self.CloseBuildMenu`)
  (`self.RefreshEditActions`)
  (`/Game/GrandOpening/Blueprints/Widgets/Gameplay/BP_CrosshairWidget.ShowMode` (`/Game/GrandOpening/Blueprints/ActorComponents/BP_InteractionComponent.Crosshair` (`self.Interaction`)) (`self.EditModeLabel`) (`self.ExitAction`) (`self.ExitLabel`)))

(fn `StopBuilding`
  (bind _interaction (`self.Interaction`))
  ;[1 1 1 0.8] Stop building
  (`self.CloseBuildMenu`)
  (set `self.Building` false)
  (set `self.CanPlace` false)
  (set `self.Editing` false)
  (set `self.CanPickUp` false)
  (set `self.EditTarget` null)
  (`/Game/GrandOpening/Blueprints/ActorComponents/BP_InteractionComponent.SetSuspended` _interaction false)
  (`/Game/GrandOpening/Blueprints/Widgets/Gameplay/BP_CrosshairWidget.HideMode` (`/Game/GrandOpening/Blueprints/ActorComponents/BP_InteractionComponent.Crosshair` _interaction))
  (set `self.ArmedStructure` null)
  (`/Engine/EditorBlueprintResources/StandardMacros.IsValid` (`self.GhostActor`)
    (:`Is Valid`
      (`Actor.K2_DestroyActor` (`self.GhostActor`))
      (set `self.GhostActor` null))))

(fn `SurfaceFrame`
  (params (SurfaceNormal :type "Vector Structure"))
  (returns (Frame :type "Rotator Structure"))
  ;[1 1 1 0.8] Surface frame
  (return (`KismetMathLibrary.SelectRotator` (`KismetMathLibrary.MakeRotFromZX` SurfaceNormal (`KismetMathLibrary.Vector_Forward`)) (`KismetMathLibrary.MakeRotFromZY` SurfaceNormal (`KismetMathLibrary.Vector_Up`)) (>= (`KismetMathLibrary.Abs` (.z SurfaceNormal)) 0.7))))

(fn `ToggleBuild`
  ;[1 1 1 0.8] Toggle build
  (if (`self.Building`)
    (`self.StopBuilding`)
    (else
      (set `self.Building` true)
      (`/Game/GrandOpening/Blueprints/ActorComponents/BP_InteractionComponent.SetSuspended` (`self.Interaction`) true)
      (bind _returnvalue (`|SpawnActorFromClass` "/Game/GrandOpening/Blueprints/Environments/Build/BP_PlacementGhost.BP_PlacementGhost_C" (`KismetMathLibrary.MakeTransform` (0.0 0.0 0.0)) "AlwaysSpawn" "MultiplyWithRoot" null null))
      (set `self.GhostActor` _returnvalue)
      (`/Game/GrandOpening/Blueprints/Environments/Build/BP_PlacementGhost.SetShown` _returnvalue false)
      (`self.OpenBuildMenu`))))

(fn `TraceFoundation`
  (returns (SurfacePoint :type "Vector Structure") (SurfaceNormal :type "Vector Structure") (Hit :type Boolean) (SurfaceActor :type "Actor Object Reference"))
  ;[1 1 1 0.8] Trace foundation
  (bind (_outhit _returnvalue) (`KismetSystemLibrary.LineTraceSingle` (`SceneComponent.K2_GetComponentLocation` (`self.ViewCamera`)) (+ (`SceneComponent.K2_GetComponentLocation` (`self.ViewCamera`)) (* (`SceneComponent.GetForwardVector` (`self.ViewCamera`)) (`self.MaxPlaceDistanceCm`))) "TraceTypeQuery3" false (`|MakeArray` (`self.GetOwner`))))
  (bind (_bblockinghit _binitialoverlap _time _distance _location _impactpoint _normal _impactnormal _physmat _hitactor) (`GameplayStatics.BreakHitResult` _outhit))
  (return _impactpoint _impactnormal _returnvalue _hitactor))

(fn `TraceStructure`
  (returns (Target :type "Actor Object Reference"))
  (bind _viewcamera (`self.ViewCamera`))
  (bind _returnvalue (`SceneComponent.K2_GetComponentLocation` _viewcamera))
  ;[1 1 1 0.8] Trace structure
  (bind (_outhit _returnvalue_2) (`KismetSystemLibrary.LineTraceSingle` _returnvalue (+ _returnvalue (* (`SceneComponent.GetForwardVector` _viewcamera) (`self.MaxPlaceDistanceCm`))) "TraceTypeQuery1" false (`|MakeArray` (`self.GhostActor`) :!type "Actor Object Reference")))
  (if _returnvalue_2
    (bind (_bblockinghit _binitialoverlap _time _distance _location _impactpoint _normal _impactnormal _physmat _hitactor) (`GameplayStatics.BreakHitResult` _outhit))
    (bind _returnvalue_3 (`Actor.GetComponentByClass` _hitactor "/Game/GrandOpening/Blueprints/ActorComponents/BP_PlaceableComponent.BP_PlaceableComponent_C"))
    (`/Engine/EditorBlueprintResources/StandardMacros.IsValid` _returnvalue_3
      (:`Is Valid`
        (`/Engine/EditorBlueprintResources/StandardMacros.IsValid` (`/Game/GrandOpening/Blueprints/ActorComponents/BP_PlaceableComponent.Structure` _returnvalue_3)
          (:`Is Valid`
            (return _hitactor)))))))

(fn `UpdateEditGhost`
  (bind _ghostactor (`self.GhostActor`))
  ;[1 1 1 0.8] Update edit ghost
  (bind _target (`self.TraceStructure`))
  (`/Engine/EditorBlueprintResources/StandardMacros.IsValid` _target
    (:`Is Valid`
      (if (not (== _target (`self.EditTarget`)))
        (set `self.EditTarget` _target)
        (bind _structure (`/Game/GrandOpening/Blueprints/ActorComponents/BP_PlaceableComponent.Structure` (`Actor.GetComponentByClass` _target "/Game/GrandOpening/Blueprints/ActorComponents/BP_PlaceableComponent.BP_PlaceableComponent_C")))
        (`/Game/GrandOpening/Blueprints/Environments/Build/BP_PlacementGhost.SetPreviewMesh` _ghostactor (`/Game/GrandOpening/Blueprints/DataAssets/Structures/BP_StructureDataAsset.PreviewMesh` _structure))
        (`/Game/GrandOpening/Blueprints/Environments/Build/BP_PlacementGhost.SetCellLayout` _ghostactor (`/Game/GrandOpening/Blueprints/DataAssets/Structures/BP_StructureDataAsset.FootprintCells` _structure) (`/Game/GrandOpening/Blueprints/DataAssets/Structures/BP_StructureDataAsset.SnapStepCm` _structure)))
      (bind (_canpickup _reason) (`self.ValidatePickup` _target))
      (set `self.CanPickUp` _canpickup)
      (`Actor.K2_SetActorTransform` _ghostactor (`Actor.GetTransform` _target) false false)
      (bind _returnvalue (`Actor.GetActorUpVector` _target))
      (bind _frame (`self.SurfaceFrame` _returnvalue))
      (`/Game/GrandOpening/Blueprints/Environments/Build/BP_PlacementGhost.SetSurface` _ghostactor _returnvalue _frame)
      (`/Game/GrandOpening/Blueprints/Environments/Build/BP_PlacementGhost.SetDecalsShown` _ghostactor true)
      (`self.PresentGhostResult` _canpickup _reason)
      (`/Game/GrandOpening/Blueprints/Environments/Build/BP_PlacementGhost.SetShown` _ghostactor true))
    (:`Is Not Valid`
      (set `self.CanPickUp` false)
      (`/Game/GrandOpening/Blueprints/Environments/Build/BP_PlacementGhost.SetShown` _ghostactor false))))

(fn `UpdateGhost`
  (bind _ghostactor (`self.GhostActor`))
  (bind _armedstructure (`self.ArmedStructure`))
  ;[1 1 1 0.8] Update ghost
  (`/Engine/EditorBlueprintResources/StandardMacros.IsValid` (`self.ArmedStructure`)
    (:`Is Valid`
      (bind (_surfacepoint _surfacenormal _hit _surfaceactor) (`self.TraceFoundation`))
      (if _hit
        (bind _result (`self.ValidatePlacement` _armedstructure _surfacepoint _surfacenormal _surfaceactor (`self.GhostRotation`)))
        (bind (_valid _reason _snappedtransform) (break `/Game/GrandOpening/Blueprints/Structures/S_PlacementResult` _result))
        (set `self.CanPlace` _valid)
        (`Actor.K2_SetActorTransform` _ghostactor _snappedtransform false false)
        (bind (_normal _allowed) (`self.PlacementNormal` _armedstructure _surfacenormal))
        (bind _frame (`self.SurfaceFrame` _normal))
        (`/Game/GrandOpening/Blueprints/Environments/Build/BP_PlacementGhost.SetSurface` _ghostactor _normal _frame)
        (`/Game/GrandOpening/Blueprints/Environments/Build/BP_PlacementGhost.SetDecalsShown` _ghostactor _allowed)
        (`self.PresentGhostResult` _valid _reason)
        (`/Game/GrandOpening/Blueprints/Environments/Build/BP_PlacementGhost.SetShown` _ghostactor true)
        (else
          (set `self.CanPlace` false)
          (`/Game/GrandOpening/Blueprints/Environments/Build/BP_PlacementGhost.SetShown` _ghostactor false))))
    (:`Is Not Valid`
      (set `self.CanPlace` false)
      (`/Game/GrandOpening/Blueprints/Environments/Build/BP_PlacementGhost.SetShown` _ghostactor false))))

(fn `ValidatePickup`
  (params (Target :type "Actor Object Reference"))
  (returns (CanPickUp :type Boolean) (Reason :type Text))
  (locals (BlockReason :type Text))
  (bind _blockreason (`local.BlockReason`))
  ;[1 1 1 0.8] Validate pickup
  (bind _asbp_checkout_base (cast `/Game/GrandOpening/Blueprints/Environments/Checkout/BP_CheckoutBase` Target)
    (:`then`
      (bind _returnvalue (`/Game/GrandOpening/Blueprints/Environments/Checkout/BP_CheckoutBase.HasCustomers` _asbp_checkout_base))
      (if _returnvalue
        (set `local.BlockReason` (`self.ReasonCheckoutBusy`))
        (else
          (bind _manned (`/Game/GrandOpening/Blueprints/Environments/Checkout/BP_CheckoutBase.IsManned` _asbp_checkout_base))
          (if _manned
            (set `local.BlockReason` (`self.ReasonCheckoutManned`))))))
    (:`CastFailed`
      (bind _asbp_shelf_base (cast `/Game/GrandOpening/Blueprints/Environments/Shelves/BP_ShelfBase` Target)
        (:`then`
          (bind _products (`/Game/GrandOpening/Blueprints/Environments/Shelves/BP_ShelfBase.StockedProducts` _asbp_shelf_base))
          (if (not (`KismetArrayLibrary.Array_IsEmpty` _products))
            (set `local.BlockReason` (`self.ReasonShelfStocked`))))
        (:`CastFailed`
          _))))
  (return (`KismetTextLibrary.TextIsEmpty` _blockreason) _blockreason))

(fn `ValidatePlacement`
  (params (Structure :type "/Game/GrandOpening/Blueprints/DataAssets/Structures/BP_StructureDataAsset Object Reference") (Location :type "Vector Structure") (SurfaceNormal :type "Vector Structure") (SurfaceActor :type "Actor Object Reference") (Rotation :type "Rotator Structure"))
  (returns (Result :type "/Game/GrandOpening/Blueprints/Structures/S_PlacementResult Structure"))
  (locals (BlockedHere :type Boolean) (CustomerHere :type Boolean))
  (bind _snapstepcm (`/Game/GrandOpening/Blueprints/DataAssets/Structures/BP_StructureDataAsset.SnapStepCm` Structure))
  (bind (_x _y) (break `IntPoint` (`/Game/GrandOpening/Blueprints/DataAssets/Structures/BP_StructureDataAsset.FootprintCells` Structure)))
  (bind _returnvalue (* (`self.ProbeHeightCm`) 0.5))
  (bind _returnvalue_2 (> (mod (`KismetMathLibrary.Abs` (.yaw Rotation)) 180.0) 45.0))
  (bind _returnvalue_3 (select `bool` _returnvalue_2 :`false` _x :`true` _y))
  (bind _returnvalue_4 (select `bool` _returnvalue_2 :`false` _y :`true` _x))
  ;[1 1 1 0.8] Validate placement
  (`/Engine/EditorBlueprintResources/StandardMacros.IsValid` Structure
    (:`Is Valid`
      (bind (_normal _allowed) (`self.PlacementNormal` Structure SurfaceNormal))
      (bind _frame (`self.SurfaceFrame` _normal))
      (bind _snapped (`self.SnapToSurface` Location _normal (make `IntPoint` _returnvalue_3 _returnvalue_4) _snapstepcm))
      (if (not _allowed)
        (bind _returnvalue_5 (`KismetMathLibrary.MakeTransform` _snapped (`KismetMathLibrary.ComposeRotators` Rotation _frame)))
        (return (make `/Game/GrandOpening/Blueprints/Structures/S_PlacementResult` false (`self.ReasonWrongSurface`) _returnvalue_5))
        (else
          (bind _returnvalue_6 (+ _snapped (`KismetMathLibrary.GreaterGreater_VectorRotator` (`KismetMathLibrary.MakeVector` 0.0 0.0 _returnvalue) _frame)))
          (bind _allowed_2 (`self.IsLocationAllowedFor` Structure _returnvalue_6))
          (if (not _allowed_2)
            (return (make `/Game/GrandOpening/Blueprints/Structures/S_PlacementResult` false (`self.ReasonWrongZone`) _returnvalue_5))
            (else
              (bind _outactors (`KismetSystemLibrary.BoxOverlapActors` _returnvalue_6 (`KismetMathLibrary.Vector_GetAbs` (`KismetMathLibrary.GreaterGreater_VectorRotator` (`KismetMathLibrary.MakeVector` (* (* _returnvalue_3 _snapstepcm) 0.5) (* (* _returnvalue_4 _snapstepcm) 0.5) _returnvalue) _frame)) (`|MakeArray` "ObjectTypeQuery1" "ObjectTypeQuery2" "ObjectTypeQuery3" :!type "EObjectTypeQuery Enum")))
              (for _array_element _outactors
                (if (!= _array_element SurfaceActor)
                  (`/Engine/EditorBlueprintResources/StandardMacros.IsValid` (`Actor.GetComponentByClass` _array_element "/Game/GrandOpening/Blueprints/ActorComponents/BP_PlaceableComponent.BP_PlaceableComponent_C")
                    (:`Is Valid`
                      (set `local.BlockedHere` true))
                    (:`Is Not Valid`
                      (cast `/Game/GrandOpening/Blueprints/AI/Customer/BP_Customer` _array_element)
                      (set `local.CustomerHere` true)))))
              (if (`local.CustomerHere`)
                (return (make `/Game/GrandOpening/Blueprints/Structures/S_PlacementResult` false (`self.ReasonCustomerHere`) _returnvalue_5))
                (elif (`local.BlockedHere`)
                  (return (make `/Game/GrandOpening/Blueprints/Structures/S_PlacementResult` false (`self.ReasonBlocked`) _returnvalue_5))
                  (else
                    (return (make `/Game/GrandOpening/Blueprints/Structures/S_PlacementResult` true "" _returnvalue_5))))))))))
    (:`Is Not Valid`
      (return (make `/Game/GrandOpening/Blueprints/Structures/S_PlacementResult` false (`self.ReasonNoStructure`))))))
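; BP_QueueComponent manages an ordered queue of members with a configurable capacity and lays out their standing slots along a spline.
; Joining rejects duplicates and refuses entry when full, while leaving removes the member from the array, whose order gives each member's slot index.
; Slot transforms are world-space points at even spacing along the spline, clamped to its length so overflow slots collapse onto the end.
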(fn `Clear`
  ;[1 1 1 0.8] Clear
  (`KismetArrayLibrary.Array_Clear` (`self.Members`)))

(fn `ConfigureQueue`
  (params (NewCapacity :type Integer))
  ;[1 1 1 0.8] Configure queue
  (set `self.Capacity` NewCapacity))

(fn `GetSlotIndex`
  (params (Member :type "Actor Object Reference"))
  (returns (Index :type Integer))
  ;[1 1 1 0.8] Get slot index
  (return (`KismetArrayLibrary.Array_Find` (`self.Members`) Member)))

(fn `Leave`
  (params (Member :type "Actor Object Reference"))
  ;[1 1 1 0.8] Leave
  (`KismetArrayLibrary.Array_RemoveItem` (`self.Members`) Member))

(fn `SlotTransform`
  (params (Index :type Integer))
  (returns (Slot :type "Transform Structure"))
  ;[1 1 1 0.8] Slot transform
  (return (`self.GetTransformAtDistanceAlongSpline` self (`KismetMathLibrary.FMin` (* (`self.SlotSpacingCm`) (`KismetMathLibrary.Conv_IntToDouble` Index)) (`self.GetSplineLength` self)) "World" false)))

(fn `TryJoin`
  (params (Member :type "Actor Object Reference"))
  (returns (Joined :type Boolean))
  (locals (Accepted :type Boolean))
  (bind _members (`self.Members`))
  ;[1 1 1 0.8] Try join
  (set `local.Accepted` (and (not (`KismetArrayLibrary.Array_Contains` _members Member)) (< (`KismetArrayLibrary.Array_Length` _members) (`self.Capacity`))))
  (if (`local.Accepted`)
    (`KismetArrayLibrary.Array_Add` _members Member))
  (return (`local.Accepted`)))
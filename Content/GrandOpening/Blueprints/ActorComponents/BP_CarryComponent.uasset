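; Actor component that lets its owner grab, carry, throw or place physics actors using a PhysicsHandle.
; Each tick drives the handle target ahead of the camera, yaw-only, composed with the item's carry offset.
; Carried items ignore Pawn and Vehicle collision, show the prompt widget, and get notified on pickup and release.
; Lagging items turn ghosted, passing through world collision with a material fade, using two distance thresholds as hysteresis.
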(event `self.ReceiveBeginPlay`
  ;[1 1 1 0.8] Event begin play
  (bind _resolved (`self.ResolveCarry` self))
  (set `self.Ready` _resolved))

(event `self.ReceiveTick`
  (params (DeltaSeconds :type "Float (single-precision)"))
  ;[1 1 1 0.8] Event tick
  (`self.AdvanceCarryPose`))

(fn `AdvanceCarryPose`
  (bind _carriedactor (`self.CarriedActor`))
  (bind _viewcamera (`self.ViewCamera`))
  ;[1 1 1 0.8] Advance carry pose
  (`/Engine/EditorBlueprintResources/StandardMacros.IsValid` _carriedactor
    (:`Is Valid`
      (bind _transform (message `/Game/GrandOpening/Blueprints/Interfaces/BPI_Carryable.GetCarryOffset` _carriedactor))
      (`PhysicsHandleComponent.SetTargetLocationAndRotation` (`self.CarryHandle`) (.location (`KismetMathLibrary.ComposeTransforms` _transform (`KismetMathLibrary.MakeTransform` (+ (`SceneComponent.K2_GetComponentLocation` _viewcamera) (* (`SceneComponent.GetForwardVector` _viewcamera) (`self.HoldDistance`))) (`KismetMathLibrary.MakeRotator` 0.0 0.0 (.yaw (`SceneComponent.K2_GetComponentRotation` _viewcamera)))))) (.rotation (`KismetMathLibrary.ComposeTransforms` _transform (`KismetMathLibrary.MakeTransform` (+ (`SceneComponent.K2_GetComponentLocation` _viewcamera) (* (`SceneComponent.GetForwardVector` _viewcamera) (`self.HoldDistance`))) (`KismetMathLibrary.MakeRotator` 0.0 0.0 (.yaw (`SceneComponent.K2_GetComponentRotation` _viewcamera)))))))
      (`self.RefreshGhost`))))

(fn `GrabActor`
  (params (Target :type "Actor Object Reference"))
  (returns (Grabbed :type Boolean))
  (bind _prompt (`self.Prompt`))
  ;[1 1 1 0.8] Grab actor
  (bind _carrying (`self.IsCarrying` self))
  (`/Engine/EditorBlueprintResources/StandardMacros.IsValid` Target
    (:`Is Valid`
      (if (and (`self.Ready`) (not _carrying))
        (bind _body (message `/Game/GrandOpening/Blueprints/Interfaces/BPI_Carryable.GetCarryBody` Target))
        (`/Engine/EditorBlueprintResources/StandardMacros.IsValid` _body
          (:`Is Valid`
            (for _array_element (`Actor.K2_GetComponentsByClass` Target "/Script/Engine.PrimitiveComponent")
              (`PrimitiveComponent.SetCollisionResponseToChannel` _array_element "ECC_Pawn" "ECR_Ignore")
              (`PrimitiveComponent.SetCollisionResponseToChannel` _array_element "ECC_Vehicle" "ECR_Ignore"))
            (`PrimitiveComponent.SetSimulatePhysics` _body true)
            (set `self.CarriedBody` _body)
            (`PhysicsHandleComponent.GrabComponentAtLocationWithRotation` (`self.CarryHandle`) _body "None" (`SceneComponent.K2_GetComponentLocation` _body) (`SceneComponent.K2_GetComponentRotation` _body))
            (set `self.CarriedActor` Target)
            (`SceneComponent.K2_AttachToComponent` _prompt _body "None" "KeepRelative" "KeepRelative" "KeepRelative" false)
            (`SceneComponent.K2_SetRelativeLocation` _prompt (`KismetMathLibrary.MakeVector` 0.0 0.0 (+ (.z (`.Max` (`StaticMeshComponent.GetLocalBounds` _body))) (`self.ActionPromptOffset`))) false false)
            (`SceneComponent.SetVisibility` (`self.Prompt`) true false)
            (message `/Game/GrandOpening/Blueprints/Interfaces/BPI_Carryable.OnCarriedChanged` Target true)
            (`self.OnCarryChanged`)
            (return true))
          (:`Is Not Valid`
            (return false)))
        (else
          (return false))))))

(fn `IsCarrying`
  (returns (Carrying :type Boolean))
  ;[1 1 1 0.8] Is carrying
  (`/Engine/EditorBlueprintResources/StandardMacros.IsValid` (`self.CarriedActor`)
    (:`Is Valid`
      (return true))
    (:`Is Not Valid`
      (return false))))

(fn `PlaceActor`
  (params (Location :type "Vector Structure"))
  (returns (ReturnValue :type Boolean))
  (locals (PlacedBody :type "PrimitiveComponent Object Reference"))
  (bind _placedbody (`local.PlacedBody`))
  (bind (_origin _boxextent) (`Actor.GetActorBounds` (`self.GetOwner` _placedbody) true false))
  ;[1 1 1 0.8] Place actor
  (set `local.PlacedBody` (`self.CarriedBody`))
  (bind _released (`self.ReleaseActor` self))
  (if _released
    (`SceneComponent.K2_SetWorldLocation` _placedbody (+ Location (`KismetMathLibrary.MakeVector` 0.0 0.0 (- (.z (`SceneComponent.K2_GetComponentLocation` _placedbody)) (- (.z _origin) (.z _boxextent))))) false true)
    (`PrimitiveComponent.SetPhysicsLinearVelocity` _placedbody (0.0 0.0 0.0) false "None")
    (`PrimitiveComponent.SetPhysicsAngularVelocityInDegrees` _placedbody (0.0 0.0 0.0) false "None"))
  (return _released))

(fn `RefreshGhost`
  (bind _returnvalue (`KismetMathLibrary.Vector_Distance` (`SceneComponent.K2_GetComponentLocation` (`self.CarriedBody`)) (`PhysicsHandleComponent.GetTargetLocationAndRotation` (`self.CarryHandle`))))
  ;[1 1 1 0.8] Refresh ghost
  (if (`self.Ghosted`)
    (if (< _returnvalue (`self.SolidDistanceCm`))
      (`self.SetGhost` false))
    (elif (> _returnvalue (`self.GhostDistanceCm`))
      (`self.SetGhost` true))))

(fn `ReleaseActor`
  (returns (Released :type Boolean))
  (bind _carriedactor (`self.CarriedActor`))
  ;[1 1 1 0.8] Release actor
  (`/Engine/EditorBlueprintResources/StandardMacros.IsValid` _carriedactor
    (:`Is Valid`
      (message `/Game/GrandOpening/Blueprints/Interfaces/BPI_Carryable.OnCarriedChanged` _carriedactor false)
      (`PhysicsHandleComponent.ReleaseComponent` (`self.CarryHandle`))
      (set `self.CarriedBody` null)
      (`self.SetGhost` false)
      (for _array_element (`Actor.K2_GetComponentsByClass` _carriedactor "/Script/Engine.PrimitiveComponent")
        (`PrimitiveComponent.SetCollisionResponseToChannel` _array_element "ECC_Pawn" "ECR_Block")
        (`PrimitiveComponent.SetCollisionResponseToChannel` _array_element "ECC_Vehicle" "ECR_Block"))
      (`SceneComponent.K2_AttachToComponent` (`self.Prompt`) (`Actor.RootComponent` (`self.GetOwner`)) "None" "KeepRelative" "KeepRelative" "KeepRelative" false)
      (`SceneComponent.SetVisibility` (`self.Prompt`) false false)
      (set `self.CarriedActor` null)
      (`self.OnCarryChanged`)
      (return true))
    (:`Is Not Valid`
      (return false))))

(fn `ResolveCarry`
  (returns (Resolved :type Boolean))
  (bind _returnvalue (`self.GetOwner`))
  (bind _returnvalue_2 (`Actor.GetComponentByClass` _returnvalue "/Script/Engine.PhysicsHandleComponent"))
  ;[1 1 1 0.8] Resolve carry
  (set `self.CarryHandle` _returnvalue_2)
  (set `self.ViewCamera` (`Actor.GetComponentByClass` _returnvalue "/Script/Engine.CameraComponent"))
  (set `self.Prompt` (`Actor.GetComponentByClass` _returnvalue "/Script/UMG.WidgetComponent"))
  (`/Engine/EditorBlueprintResources/StandardMacros.IsValid` _returnvalue_2
    (:`Is Valid`
      (return true))
    (:`Is Not Valid`
      (return false))))

(fn `SetGhost`
  (params (Ghost :type Boolean))
  (bind _carriedactor (`self.CarriedActor`))
  ;[1 1 1 0.8] Set ghost
  (if (!= Ghost (`self.Ghosted`))
    (set `self.Ghosted` Ghost)
    (for _array_element (`Actor.K2_GetComponentsByClass` _carriedactor "/Script/Engine.StaticMeshComponent")
      (`MeshComponent.SetScalarParameterValueOnMaterials` _array_element "GhostAmount" (select `bool` Ghost :`true` 1.0)))
    (for _array_element_2 (`Actor.K2_GetComponentsByClass` _carriedactor "/Script/Engine.PrimitiveComponent")
      (if Ghost
        (`PrimitiveComponent.SetCollisionResponseToChannel` _array_element_2 "ECC_WorldStatic" "ECR_Ignore")
        (`PrimitiveComponent.SetCollisionResponseToChannel` _array_element_2 "ECC_WorldDynamic" "ECR_Ignore")
        (else
          (`PrimitiveComponent.SetCollisionResponseToChannel` _array_element_2 "ECC_WorldStatic" "ECR_Block")
          (`PrimitiveComponent.SetCollisionResponseToChannel` _array_element_2 "ECC_WorldDynamic" "ECR_Block"))))))

(fn `ThrowActor`
  (returns (ReturnValue :type Boolean))
  (locals (ThrownBody :type "PrimitiveComponent Object Reference"))
  ;[1 1 1 0.8] Throw actor
  (set `local.ThrownBody` (`self.CarriedBody`))
  (bind _released (`self.ReleaseActor` self))
  (if _released
    (`PrimitiveComponent.AddImpulse` (`local.ThrownBody`) (* (`SceneComponent.GetForwardVector` (`self.ViewCamera`)) (`self.ThrowSpeed`)) "None" true))
  (return _released))